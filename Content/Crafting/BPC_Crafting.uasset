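; Player crafting component that unlocks recipes from discovered items and crafts them from inventory ingredients.
; AddDiscoveredItem records new item classes, notifies listeners and briefly shows a HUD notice when the count of unlocked data-table recipes grows.
; CraftItem reports missing ingredients or consumes them, then spawns a physics pickup or grabbable actor in front of the player.
; Crafting a spear, axe or pickaxe completes the CraftTool quest.
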(event `self.ReceiveBeginPlay`
  (bind _asbp_player_character (cast `/Game/PlayerCharacter/BP_PlayerCharacter` (`GameplayStatics.GetPlayerCharacter` 0)))
  (set `self.PlayerRef` _asbp_player_character))

(event `ShowNewRecipeText`
  (bind _recipetext (`/Game/PlayerCharacter/GUI/WBP_InGameScreen.RecipeText` (`/Game/PlayerCharacter/BP_PlayerCharacter.InGameScreenWidget` (`self.PlayerRef`))))
  (`Widget.SetVisibility` _recipetext "Visible")
  (`KismetSystemLibrary.Delay` 5.0)
  (`Widget.SetVisibility` _recipetext "Hidden"))

(fn `AddDiscoveredItem`
  (params (ItemClass :type "/Game/Items/ItemObjects/BP_ItemObject Class Reference"))
  (if (`KismetSystemLibrary.IsValidClass` ItemClass)
    (if (not (`KismetArrayLibrary.Array_Contains` (`self.DiscoveredItems`) ItemClass))
      (`KismetArrayLibrary.Array_Add` (`self.DiscoveredItems`) ItemClass)
      (`self.OnRecipesUpdated`)
      (`self.CheckNewUnlockedRecipe`))))

(fn `AreAllRequirementsMet`
  (params (S_CraftingRecipe :type "/Game/Crafting/CraftingRecipes/S_CraftingRecipe Structure (by ref)"))
  (returns (AreAllReqMet :type Boolean))
  (for _array_element (`.UnlockRequirements_12_5A448D5F4F0D9604D84B6683E79F35ED` (break `/Game/Crafting/CraftingRecipes/S_CraftingRecipe` S_CraftingRecipe))
    (if (not (`KismetArrayLibrary.Array_Contains` (`self.DiscoveredItems`) _array_element))
      (return false)))
  (return true))

(fn `CanCraft`
  (params (Recipe :type "/Game/Crafting/CraftingRecipes/S_CraftingRecipe Structure"))
  (returns (CanCraft :type Boolean) (MissingIngredients :type "Array of /Game/Crafting/CraftingRecipes/S_MissingIngredient Structure"))
  (locals (OwnedAmount :type Integer) (LocalMissingIngredients :type "Array of /Game/Crafting/CraftingRecipes/S_MissingIngredient Structure"))
  (bind _localmissingingredients (`local.LocalMissingIngredients`))
  (for _array_element (`.Ingredients_13_CD827881482FD40157E82DB600499BA8` (break `/Game/Crafting/CraftingRecipes/S_CraftingRecipe` Recipe))
    (bind (_itemclass _amount) (break `/Game/Crafting/CraftingRecipes/S_CraftingIngredient` _array_element))
    (bind _itemcount (`/Game/Inventory/BPC_Inventory.GetItemCount` (`/Game/PlayerCharacter/BP_PlayerCharacter.BPC_Inventory` (`self.PlayerRef`)) _itemclass))
    (bind _output_get (set `local.OwnedAmount` _itemcount))
    (if (not (>= _output_get _amount))
      (`KismetArrayLibrary.Array_Add` (`local.LocalMissingIngredients`) (make `/Game/Crafting/CraftingRecipes/S_MissingIngredient` _itemclass _amount (`local.OwnedAmount`) (- _amount (`local.OwnedAmount`))))))
  (if (== (`KismetArrayLibrary.Array_Length` _localmissingingredients) 0)
    (return true)
    (else
      (return false _localmissingingredients))))

(fn `CheckNewUnlockedRecipe`
  (bind _unlockedrecipes (`self.GetUnlockedRecipes`))
  (bind _returnvalue (`KismetArrayLibrary.Array_Length` _unlockedrecipes))
  (if (> _returnvalue (`self.NumberOfUnlockedRecipes`))
    (`self.ShowNewRecipeText`))
  (set `self.NumberOfUnlockedRecipes` _returnvalue))

(fn `CraftItem`
  (params (Recipe :type "/Game/Crafting/CraftingRecipes/S_CraftingRecipe Structure"))
  (returns (Crafted :type Boolean) (MissingIngredients :type "Array of /Game/Crafting/CraftingRecipes/S_MissingIngredient Structure"))
  (bind (_id _resultitemtype _resultitemobjectclass _resultgrabbableobjectactor _ingredients) (break `/Game/Crafting/CraftingRecipes/S_CraftingRecipe` Recipe))
  (bind (_cancraft _missingingredients) (`self.CanCraft` Recipe))
  (if _cancraft
    (for _array_element _ingredients
      (bind (_itemclass _amount) (break `/Game/Crafting/CraftingRecipes/S_CraftingIngredient` _array_element))
      (`/Game/Inventory/BPC_Inventory.RemoveItemByClass` (`/Game/PlayerCharacter/BP_PlayerCharacter.BPC_Inventory` (`self.PlayerRef`)) _itemclass _amount))
    (switch `/Game/Crafting/CraftingRecipes/E_ResultCraftedItemType` _resultitemtype
      (:`NewEnumerator0`
        (`self.SpawnNewCraftedItem` _resultitemobjectclass)
        (if (or (== _resultitemobjectclass "/Game/Items/ItemObjects/Tool/BP_ToolObject_Spear.BP_ToolObject_Spear_C") (== _resultitemobjectclass "/Game/Items/ItemObjects/Tool/BP_ToolObject_Axe.BP_ToolObject_Axe_C") (== _resultitemobjectclass "/Game/Items/ItemObjects/Tool/BP_ToolObject_Pickaxe.BP_ToolObject_Pickaxe_C"))
          (`/Game/Quests/BP_QuestManager.CompleteQuest` (`/Game/PlayerCharacter/BP_PlayerCharacter.QuestManager` (`self.PlayerRef`)) "CraftTool"))
        (return true))
      (:`NewEnumerator1`
        (`self.SpawnNewCraftedObject` _resultgrabbableobjectactor)
        (return true)))
    (else
      (return false _missingingredients))))

(fn `GetUnlockedRecipes`
  (returns (UnlockedRecipes :type "Array of /Game/Crafting/CraftingRecipes/S_CraftingRecipe Structure"))
  (locals (Unlocked :type Boolean :default true) (OutputArray :type "Array of /Game/Crafting/CraftingRecipes/S_CraftingRecipe Structure"))
  (bind _outrownames (`DataTableFunctionLibrary.GetDataTableRowNames` (`self.CraftingRecipesTable`)))
  (for _array_element _outrownames
    (bind _returnvalue (`|GetDataTableRow` (`self.CraftingRecipesTable`) _array_element)
      (:`then`
        (bind _areallreqmet (`self.AreAllRequirementsMet` _returnvalue))
        (if _areallreqmet
          (`KismetArrayLibrary.Array_Add` (`local.OutputArray`) _returnvalue)))))
  (return (`local.OutputArray`)))

(fn `SpawnNewCraftedItem`
  (params (ItemObjectClass :type "/Game/Items/ItemObjects/BP_ItemObject Class Reference"))
  (bind (_id _displayname _description _itemtype _stackable _stacksize _staticmesh _staticmeshtransform) (defaults `Object` ItemObjectClass))
  (bind _playerref (`self.PlayerRef`))
  (bind _returnvalue (`|SpawnActorFromClass` "/Game/Items/BP_PickableItemActor.BP_PickableItemActor_C" (`KismetMathLibrary.MakeTransform` (+ (`Actor.K2_GetActorLocation` _playerref) (* (`KismetMathLibrary.GetForwardVector` (`Actor.K2_GetActorRotation` _playerref)) 120.0))) "Undefined" "MultiplyWithRoot" null null))
  (set `/Game/Items/BP_PickableItemActor.ItemObjectClass` ItemObjectClass _returnvalue)
  (bind _staticmesh_2 (`/Game/Items/BP_PickableItemActor.StaticMesh` _returnvalue))
  (`StaticMeshComponent.SetStaticMesh` _staticmesh_2 _staticmesh)
  (`SceneComponent.K2_SetRelativeTransform` _staticmesh_2 _staticmeshtransform false false)
  (`PrimitiveComponent.SetSimulatePhysics` _staticmesh_2 true))

(fn `SpawnNewCraftedObject`
  (params (GrabbableObjectClass :type "/Game/GrabbableObjects/BP_GrabbableObject Class Reference"))
  (bind _playerref (`self.PlayerRef`))
  (`|SpawnActorFromClass` GrabbableObjectClass (`KismetMathLibrary.MakeTransform` (+ (`Actor.K2_GetActorLocation` _playerref) (* (`KismetMathLibrary.GetForwardVector` (`Actor.K2_GetActorRotation` _playerref)) 120.0))) "Undefined" "MultiplyWithRoot" null null))