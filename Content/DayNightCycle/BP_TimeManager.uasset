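; Day-night clock manager that tracks time of day, total game hours and days survived since last death.
; Tick advances time unless paused or the player sleeps, rotating the sun and toggling sky sphere material glow and opacity by sun pitch.
; It gates sleeping by chase state, cooldown and hour, and provides HH:MM text.
; Time state restores from the GameInstance save on BeginPlay and exports as a save struct.
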(event `self.ReceiveBeginPlay`
  (bind _outactors (`GameplayStatics.GetAllActorsOfClass` "/Game/PlayerCharacter/BP_PlayerCharacter.BP_PlayerCharacter_C"))
  (set `self.PlayerRef` (`|GetArrayItem` _outactors))
  (bind _outactors_2 (`GameplayStatics.GetAllActorsOfClass` "/Script/Engine.StaticMeshActor"))
  (set `self.SkySphereMesh` (`|GetArrayItem` _outactors_2))
  (bind _asbp_game_instance (cast `/Game/Saving/BP_GameInstance` (`GameplayStatics.GetGameInstance`)))
  (bind _currentsave (`/Game/Saving/BP_GameInstance.CurrentSave` _asbp_game_instance))
  (`/Engine/EditorBlueprintResources/StandardMacros.IsValid` _currentsave
    (:`Is Valid`
      (`self.ApplySaveData` (`/Game/Saving/BP_SaveGame.TimeData` _currentsave)))))

(event `self.ReceiveTick`
  (params (DeltaSeconds :type "Float (single-precision)"))
  (if (and (`self.TimeProgresses`) (not (`/Game/PlayerCharacter/BP_PlayerCharacter.IsSleeping` (`self.PlayerRef`))))
    (`self.Update Time` DeltaSeconds)))

(fn `AddGameHours`
  (params (HoursToAdd :type "Float (double-precision)"))
  (bind _returnvalue (+ HoursToAdd (`self.CurrentHourOfDay`)))
  (bind _hourin24 (`self.WrapHourTo24` _returnvalue))
  (set `self.CurrentHourOfDay` _hourin24)
  (set `self.TotalGameHours` (+ _returnvalue (`self.TotalGameHours`)))
  (`self.UpdateSunRotationFromTime`))

(fn `ApplySaveData`
  (params (SaveData :type "/Game/Saving/SavingStructures/S_TimeData Structure"))
  (bind (_currenthourofday _totalgamehours _lastdeathtotalgamehours _lastsleeptotalgamehours _sunangle _timeprograsses) (break `/Game/Saving/SavingStructures/S_TimeData` SaveData))
  (set `self.CurrentHourOfDay` _currenthourofday)
  (set `self.TotalGameHours` _totalgamehours)
  (set `self.LastDeathTotalGameHours` _lastdeathtotalgamehours)
  (set `self.LastSleepTotalGameHours` _lastsleeptotalgamehours)
  (`self.K2_SetActorRotation` (`self.SunActor`) (`KismetMathLibrary.MakeRotator` 0.0 _sunangle) false)
  (set `self.TimeProgresses` _timeprograsses))

(fn `CanSleep`
  (returns (CanSleep :type Boolean) (ReturnMessage :type Text))
  (bind _playerref (`self.PlayerRef`))
  (if (`/Game/PlayerCharacter/BP_PlayerCharacter.IsSleeping` _playerref)
    (return false "You are already sleeping")
    (elif (`/Game/PlayerCharacter/BP_PlayerCharacter.IsBeingChased` _playerref)
      (return false "Can't sleep while being chased by a predator")
      (elif (< (- (`self.TotalGameHours`) (`self.LastSleepTotalGameHours`)) (`self.SleepCooldownGameHours`))
        (return false (`|FormatText` "Wait {RemHours} hours to sleep again" (+ (`self.GetRemainingSleepCooldownHours`) 1)))
        (elif (`KismetMathLibrary.InRange_FloatFloat` (`self.CurrentHourOfDay`) 6.0 (`self.MinDayHourToSleep`))
          (return false "Too early to sleep")
          (else
            (return true "")))))))

(fn `GetCurrentHourAndMinute`
  (returns (Hours :type Integer) (Minutes :type Integer))
  (bind _currenthourofday (`self.CurrentHourOfDay`))
  (bind _returnvalue (`KismetMathLibrary.FFloor` _currenthourofday))
  (return _returnvalue (`KismetMathLibrary.FFloor` (* (- _currenthourofday _returnvalue) 60.0))))

(fn `GetFormattedTimeText`
  (returns (TimeText :type Text))
  (locals (HourString :type String) (MinuteString :type String))
  (bind (_hours _minutes) (`self.GetCurrentHourAndMinute`))
  (if (< _hours 10)
    (set `local.HourString` (`KismetStringLibrary.Concat_StrStr` "0" (`KismetStringLibrary.Conv_IntToString` _hours)))
    (else
      (set `local.HourString` (`KismetStringLibrary.Conv_IntToString` _hours))))
  (if (< _minutes 10)
    (set `local.MinuteString` (`KismetStringLibrary.Concat_StrStr` "0" (`KismetStringLibrary.Conv_IntToString` _minutes)))
    (else
      (set `local.MinuteString` (`KismetStringLibrary.Conv_IntToString` _minutes))))
  (return (`KismetTextLibrary.Conv_StringToText` (`KismetStringLibrary.Concat_StrStr` (`local.HourString`) ":" (`local.MinuteString`)))))

(fn `GetRemainingSleepCooldownHours`
  (returns (RemainingHours :type Integer))
  (return (`KismetMathLibrary.FFloor` (- (`self.SleepCooldownGameHours`) (- (`self.TotalGameHours`) (`self.LastSleepTotalGameHours`))))))

(fn `GetSaveData`
  (returns (SaveData :type "/Game/Saving/SavingStructures/S_TimeData Structure"))
  (return (make `/Game/Saving/SavingStructures/S_TimeData` (`self.CurrentHourOfDay`) (`self.TotalGameHours`) (`self.LastDeathTotalGameHours`) (`self.LastSleepTotalGameHours`) (.pitch (`self.K2_GetActorRotation` (`self.SunActor`))) (`self.TimeProgresses`))))

(fn `GetTotalDaysSurvived`
  (returns (DaysSurvived :type Integer))
  (return (`KismetMathLibrary.FFloor` (/ (`self.LastDeathTotalGameHours`) 24.0))))

(fn `Update Time`
  (params (DeltaSeconds :type "Float (double-precision)"))
  (bind _returnvalue (/ DeltaSeconds (`self.RealSecondsPerGameHour`)))
  (bind _hourin24 (`self.WrapHourTo24` (+ (`self.CurrentHourOfDay`) _returnvalue)))
  (set `self.CurrentHourOfDay` _hourin24)
  (set `self.TotalGameHours` (+ _returnvalue (`self.TotalGameHours`)))
  (set `self.LastDeathTotalGameHours` (+ _returnvalue (`self.LastDeathTotalGameHours`)))
  (`self.UpdateSunRotationFromTime`))

(fn `UpdateSunRotationFromTime`
  (bind _sunactor (`self.SunActor`))
  (bind _staticmeshcomponent (`StaticMeshActor.StaticMeshComponent` (`self.SkySphereMesh`)))
  (`self.K2_SetActorRotation` _sunactor (`KismetMathLibrary.MakeRotator` 0.0 (- (* (`self.CurrentHourOfDay`) (`self.DegreesPerHour`)) (`self.SunPitchOffset`))) false)
  (if (`KismetMathLibrary.InRange_FloatFloat` (.pitch (`self.K2_GetActorRotation` _sunactor)) 0.0 180.0)
    (`MeshComponent.SetScalarParameterValueOnMaterials` _staticmeshcomponent "Glow Crank" 1.0)
    (`MeshComponent.SetScalarParameterValueOnMaterials` _staticmeshcomponent "Opacity Multi" 1.0)
    (else
      (`MeshComponent.SetScalarParameterValueOnMaterials` _staticmeshcomponent "Glow Crank" 0.0)
      (`MeshComponent.SetScalarParameterValueOnMaterials` _staticmeshcomponent "Opacity Multi" 0.0))))

(fn `UserConstructionScript`)

(fn `WrapHourTo24`
  (params (InputHour :type "Float (double-precision)"))
  (returns (HourIn24 :type "Float (double-precision)"))
  (if (>= InputHour 24.0)
    (return (- InputHour 24.0))
    (elif (< InputHour 0.0)
      (return (+ InputHour 24.0))
      (else
        (return InputHour)))))