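; BP_Bed is a bed object that lets time skip forward by rotating the sun when slept in.
; On BeginPlay it caches the first DirectionalLight in the level as SunLight.
; Sleep checks CanInteractWithObject, then pitches that light locally by SleepHours at 15 degrees per hour, treating a full rotation as a 24-hour day.
; The rotation is applied in a single step, with no fade or interpolation.
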(event `self.ReceiveBeginPlay`
  (`parent.ReceiveBeginPlay`)
  (bind _outactors (`GameplayStatics.GetAllActorsOfClass` "/Script/Engine.DirectionalLight"))
  (set `self.SunLight` (`|GetArrayItem` _outactors)))

(fn `Sleep`
  (if (`self.CanInteractWithObject`)
    (`self.K2_AddActorLocalRotation` (`self.SunLight`) (`KismetMathLibrary.MakeRotator` 0.0 (* (`self.SleepHours`) 15.0)) false false)))

(fn `UserConstructionScript`
  (`parent.UserConstructionScript`))