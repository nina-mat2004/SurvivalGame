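; Time manager component that runs the day/night clock and the player's sleep mechanic.
; Tick advances the wrapped hour and a total-hours counter, then pitches the first DirectionalLight to match and toggles sky mesh material glow and opacity by sun pitch.
; Sleep freezes time, input and camera for a delay, then skips hours ahead.
; CanSleep gates it on sleep state, chases, hour and cooldown; several time helper functions are stubs.
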(event `self.ReceiveBeginPlay`
  (bind _outactors (`GameplayStatics.GetAllActorsOfClass` "/Script/Engine.DirectionalLight"))
  (set `self.SunActor` (`|GetArrayItem` _outactors))
  (bind _outactors_2 (`GameplayStatics.GetAllActorsOfClass` "/Game/PlayerCharacter/BP_PlayerCharacter.BP_PlayerCharacter_C"))
  (set `self.PlayerRef` (`|GetArrayItem` _outactors_2))
  (bind _outactors_3 (`GameplayStatics.GetAllActorsOfClass` "/Script/Engine.StaticMeshActor"))
  (set `self.SkySphereMesh` (`|GetArrayItem` _outactors_3)))

(event `self.ReceiveTick`
  (params (DeltaSeconds :type "Float (single-precision)"))
  (if (and (`self.TimeProgresses`) (not (`/Game/PlayerCharacter/BP_PlayerCharacter.IsSleeping` (`self.PlayerRef`))))
    (`self.UpdateTime` DeltaSeconds)))

(event `StartSleep`
  (bind _playerref (`self.PlayerRef`))
  (bind _camera (`/Game/PlayerCharacter/BP_PlayerCharacter.Camera` _playerref))
  (set `/Game/PlayerCharacter/BP_PlayerCharacter.IsSleeping` true _playerref)
  (set `self.TimeProgresses` false)
  (`Actor.DisableInput` (`Pawn.GetController` _playerref) null)
  (set `self.CameraLastRotation` (`SceneComponent.K2_GetComponentRotation` _camera))
  (`SceneComponent.K2_SetWorldRotation` _camera (struct :`Pitch` 90.0) false false)
  (`KismetSystemLibrary.Delay` (`self.SleepSequenceDuration`))
  (`self.FinishSleep`))

(event `FinishSleep`
  (bind _playerref (`self.PlayerRef`))
  (`self.AddGameHours` (`self.SleepHours`))
  (set `self.LastSleepTotalGameHours` (`self.TotalGameHours`))
  (set `/Game/PlayerCharacter/BP_PlayerCharacter.IsSleeping` false _playerref)
  (set `self.TimeProgresses` true)
  (`Actor.EnableInput` (`Pawn.GetController` _playerref) null)
  (`SceneComponent.K2_SetWorldRotation` (`/Game/PlayerCharacter/BP_PlayerCharacter.Camera` _playerref) (`self.CameraLastRotation`) false false))

(fn `AddGameHours`
  (params (HoursToAdd :type "Float (double-precision)"))
  (bind _returnvalue (+ HoursToAdd (`self.CurrentHourOfDay`)))
  (bind _hourin24 (`self.WrapHourTo24` _returnvalue))
  (set `self.CurrentHourOfDay` _hourin24)
  (set `self.TotalGameHours` (+ _returnvalue (`self.TotalGameHours`)))
  (`self.UpdateSunRotationFromTime`))

(fn `CanSleep`
  (returns (CanSleep :type Boolean) (ReturnMessage :type Text))
  (bind _playerref (`self.PlayerRef`))
  (if (`/Game/PlayerCharacter/BP_PlayerCharacter.IsSleeping` _playerref)
    (return false "Your are already sleeping")
    (elif (`/Game/PlayerCharacter/BP_PlayerCharacter.IsBeingChased` _playerref)
      (return false "Can't sleep while being chased by a predator")
      (elif (< (`self.CurrentHourOfDay`) (`self.MinDayHourToSleep`))
        (return false "Too early to sleep")
        (elif (< (- (`self.TotalGameHours`) (`self.LastSleepTotalGameHours`)) (`self.SleepCooldownGameHours`))
          (return false (`|FormatText` "Wait {RemHours} hours to sleep again" (`self.GetRemainingSleepCooldownHours`)))
          (else
            (return true "")))))))

(fn `GetCurrentHourAndMinute`
  (returns (Hours :type Integer) (Minutes :type Integer))
  (bind _currenthourofday (`self.CurrentHourOfDay`))
  (bind _returnvalue (`KismetMathLibrary.FFloor` _currenthourofday))
  (return _returnvalue (`KismetMathLibrary.FFloor` (* (- _currenthourofday _returnvalue) 60.0))))

(fn `GetFormattedTimeText`
  (returns (TimeText :type Text))
  (return ""))

(fn `GetRemainingSleepCooldownHours`
  (returns (RemainingHours :type Integer))
  (return (`KismetMathLibrary.FFloor` (- (`self.SleepCooldownGameHours`) (- (`self.TotalGameHours`) (`self.LastSleepTotalGameHours`))))))

(fn `GetSunPitchFromTime`
  (params (Hour :type "Float (double-precision)")))

(fn `GetTimeFromSunRotation`
  (params (SunPitch :type "Float (double-precision)"))
  (returns (Hour :type "Float (double-precision)") (Minute :type "Float (double-precision)"))
  (return 0.0 0.0))

(fn `SetCurrentHourOfDay`
  (params (NewHour :type "Float (double-precision)")))

(fn `UpdateSunRotationFromTime`
  (bind _sunactor (`self.SunActor`))
  (bind _staticmeshcomponent (`StaticMeshActor.StaticMeshComponent` (`self.SkySphereMesh`)))
  (`Actor.K2_SetActorRotation` _sunactor (`KismetMathLibrary.MakeRotator` 0.0 (- (* (`self.CurrentHourOfDay`) (`self.DegreesPerHour`)) (`self.SunPitchOffset`))) false)
  (if (`KismetMathLibrary.InRange_FloatFloat` (.pitch (`Actor.K2_GetActorRotation` _sunactor)) 0.0 180.0)
    (`MeshComponent.SetScalarParameterValueOnMaterials` _staticmeshcomponent "Glow Crank" 1.0)
    (`MeshComponent.SetScalarParameterValueOnMaterials` _staticmeshcomponent "Opacity Multi" 1.0)
    (else
      (`MeshComponent.SetScalarParameterValueOnMaterials` _staticmeshcomponent "Glow Crank" 0.0)
      (`MeshComponent.SetScalarParameterValueOnMaterials` _staticmeshcomponent "Opacity Multi" 0.0))))

(fn `UpdateTime`
  (params (DeltaSeconds :type "Float (double-precision)"))
  (bind _returnvalue (/ DeltaSeconds (`self.RealSecondsPerGameHour`)))
  (bind _hourin24 (`self.WrapHourTo24` (+ (`self.CurrentHourOfDay`) _returnvalue)))
  (set `self.CurrentHourOfDay` _hourin24)
  (set `self.TotalGameHours` (+ _returnvalue (`self.TotalGameHours`)))
  (`self.UpdateSunRotationFromTime`))

(fn `WrapHourTo24`
  (params (InHour :type "Float (double-precision)"))
  (returns (HourIn24 :type "Float (double-precision)"))
  (if (>= InHour 24.0)
    (return (- InHour 24.0))
    (elif (< InHour 0.0)
      (return (+ InHour 24.0))
      (else
        (return InHour)))))