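; BP_Bed is an interactable bed that lets the player sleep to skip in-game hours.
; UseObject checks the time manager, found at BeginPlay, and shows a warning if sleep is not allowed.
; Sleeping pauses time, hides the HUD, disables input and rotates the camera for a timed delay.
; Waking advances the clock, restores the player, completes the "SleepInBed" quest and updates attributes.
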(event `self.ReceiveBeginPlay`
  (`parent.ReceiveBeginPlay`)
  (bind _outactors (`GameplayStatics.GetAllActorsOfClass` "/Script/Engine.Actor"))
  (for _array_element _outactors
    (bind _asbp_time_manager (cast `/Game/DayNightCycle/BP_TimeManager` _array_element))
    (set `self.TimeManager` _asbp_time_manager)
    (break)))

(event `StartSleep`
  (bind _playerref (`self.PlayerRef`))
  (bind _camera (`/Game/PlayerCharacter/BP_PlayerCharacter.Camera` _playerref))
  (set `/Game/DayNightCycle/BP_TimeManager.TimeProgresses` false (`self.TimeManager`))
  (set `Widget.Visibility` "Hidden" (`/Game/PlayerCharacter/BP_PlayerCharacter.InGameScreenWidget` _playerref))
  (set `/Game/PlayerCharacter/BP_PlayerCharacter.IsSleeping` true _playerref)
  (`self.DisableInput` (`Pawn.GetController` _playerref) null)
  (set `self.LastCameraRotation` (`SceneComponent.K2_GetComponentRotation` _camera))
  (`SceneComponent.K2_SetWorldRotation` _camera (struct :`Pitch` 90.0) false false)
  (`KismetSystemLibrary.Delay` (`self.SleepSequenceDuration`))
  (`self.FinishSleeping`))

(event `FinishSleeping`
  (bind _playerref (`self.PlayerRef`))
  (bind _timemanager (`self.TimeManager`))
  (`/Game/DayNightCycle/BP_TimeManager.AddGameHours` _timemanager (`self.SleepHours`))
  (set `/Game/DayNightCycle/BP_TimeManager.LastSleepTotalGameHours` (`/Game/DayNightCycle/BP_TimeManager.TotalGameHours` _timemanager) _timemanager)
  (set `/Game/DayNightCycle/BP_TimeManager.TimeProgresses` true _timemanager)
  (set `/Game/PlayerCharacter/BP_PlayerCharacter.IsSleeping` false _playerref)
  (set `Widget.Visibility` "Visible" (`/Game/PlayerCharacter/BP_PlayerCharacter.InGameScreenWidget` _playerref))
  (`self.EnableInput` (`Pawn.GetController` _playerref) null)
  (`SceneComponent.K2_SetWorldRotation` (`/Game/PlayerCharacter/BP_PlayerCharacter.Camera` _playerref) (`self.LastCameraRotation`) false false)
  (`/Game/Quests/BP_QuestManager.OnQuestCompleted` (`/Game/PlayerCharacter/BP_PlayerCharacter.QuestManager` _playerref) "SleepInBed")
  (`/Game/Attributes/BPC_Attributes.SetAttributesAfterSleeping` (`/Game/PlayerCharacter/BP_PlayerCharacter.BPC_Attributes` _playerref)))

(fn `UseObject`
  (if (`self.CanInteractWithObject`)
    (bind (_cansleep _returnmessage) (`/Game/DayNightCycle/BP_TimeManager.CanSleep` (`self.TimeManager`)))
    (if _cansleep
      (`self.StartSleep`)
      (else
        (`/Game/PlayerCharacter/UI/WBP_WarningInfo.SetText` (`self.WarningInfoWidget`) _returnmessage)
        (`self.ShowWarning`)))))

(fn `UserConstructionScript`
  (`parent.UserConstructionScript`))