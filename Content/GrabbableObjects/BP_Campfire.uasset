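; Grabbable campfire that the player lights with sticks and dry grass from the inventory to cook raw meat.
; Lighting toggles light and particles and starts a self-repeating delayed fuel drain that extinguishes the fire when empty.
; Interaction follows the cooking state: cooking blocks grabbing, completes only if still lit, restarts on relighting, and yields cooked meat when collected.
; A state text widget yaws toward the player camera each tick.
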(event `self.ReceiveBeginPlay`
  (`parent.ReceiveBeginPlay`)
  (`self.UpdateStateText`))

(event `self.ReceiveTick`
  (params (DeltaSeconds :type "Float (single-precision)"))
  (`parent.ReceiveTick` DeltaSeconds)
  (`SceneComponent.K2_SetWorldRotation` (`self.WidgetComponent`) (`KismetMathLibrary.MakeRotator` 0.0 0.0 (.yaw (`KismetMathLibrary.FindLookAtRotation` (`SceneComponent.K2_GetComponentLocation` (`self.WidgetComponent`)) (`SceneComponent.K2_GetComponentLocation` (`/Game/Characters/PlayerCharacter/BP_PlayerCharacter.Camera` (`self.PlayerRef`)))))) false false))

(event `DrainFuel`
  (if (> (`self.Fuel`) 0.0)
    (set `self.Fuel` (- (`self.Fuel`) (`self.FuelDrainRate`)))
    (`KismetSystemLibrary.Delay` 1.0)
    (`self.DrainFuel`)
    (else
      (`self.SetCampFireLitState` false))))

(event `StartCooking`
  (`self.SpawnMeatMesh`)
  (set `self.CookingState` "NewEnumerator1")
  (set `self.CanBeGrabbed` false)
  (`self.UpdateStateText`)
  (`KismetSystemLibrary.Delay` (`self.CookTime`))
  (if (`self.IsLit`)
    (`self.FinishCooking`)))

(fn `DespawnMeatMesh`
  (`SceneComponent.SetVisibility` (`self.MeatMesh`) false false))

(fn `FinishCooking`
  (set `self.CookingState` "NewEnumerator0")
  (`self.UpdateStateText`))

(fn `GivePlayerMeat`
  (bind _returnvalue (`|GenericCreateObject` "/Game/Items/ItemObjects/Food/BP_FoodObject_CookedMeat.BP_FoodObject_CookedMeat_C"))
  (bind _itemaddedsuccessfully (`/Game/NewInventory/BPC_Inventory.AddItemToInventory` (`/Game/Characters/PlayerCharacter/BP_PlayerCharacter.BPC_Inventory` (`self.PlayerRef`)) (make `/Game/NewInventory/S_ItemData` _returnvalue (struct) 1)))
  (if _itemaddedsuccessfully
    (set `self.CookingState` "NewEnumerator5")
    (set `self.CanBeGrabbed` true)
    (`self.DespawnMeatMesh`)
    (`self.UpdateStateText`)
    (else
      (`KismetSystemLibrary.PrintString` "Count add meat to inv"))))

(fn `LightUpCampfire`
  (locals (OwnedStickAmount :type Integer :default 0) (OwnedDryGrassAmount :type Integer :default 0) (RequiredStickAmount :type Integer :default 2) (RequiredDryGrassAmount :type Integer :default 1) (NotEnoughMaterialText :type Text :default "NSLOCTEXT(\"[4CEF8167105D2E92E35C5F314175C78E]\", \"46BD8E6043D7C1A63D652D81233FE6B9\", \"You need 2x Stick and 1x Dry Grass to light up the Campfire\")") (RequiredStickClass :type "/Game/Items/ItemObjects/BP_ItemObject Class Reference" :default "/Script/Engine.BlueprintGeneratedClass'/Game/Items/ItemObjects/Material/BP_MaterialObject_Stick.BP_MaterialObject_Stick_C'") (RequiredDryGrassClass :type "/Game/Items/ItemObjects/BP_ItemObject Class Reference" :default "/Script/Engine.BlueprintGeneratedClass'/Game/Items/ItemObjects/Material/BP_MaterialObject_DryGrass.BP_MaterialObject_DryGrass_C'"))
  (bind _itemcount (`/Game/NewInventory/BPC_Inventory.GetItemCount` (`/Game/Characters/PlayerCharacter/BP_PlayerCharacter.BPC_Inventory` (`self.PlayerRef`)) (`local.RequiredStickClass`)))
  (set `local.OwnedStickAmount` _itemcount)
  (bind _itemcount_2 (`/Game/NewInventory/BPC_Inventory.GetItemCount` (`/Game/Characters/PlayerCharacter/BP_PlayerCharacter.BPC_Inventory` (`self.PlayerRef`)) (`local.RequiredDryGrassClass`)))
  (set `local.OwnedDryGrassAmount` _itemcount_2)
  (if (and (>= (`local.OwnedStickAmount`) (`local.RequiredStickAmount`)) (>= (`local.OwnedDryGrassAmount`) (`local.RequiredDryGrassAmount`)))
    (`/Game/NewInventory/BPC_Inventory.RemoveItemByClass` (`/Game/Characters/PlayerCharacter/BP_PlayerCharacter.BPC_Inventory` (`self.PlayerRef`)) (`local.RequiredStickClass`) (`local.RequiredStickAmount`))
    (`/Game/NewInventory/BPC_Inventory.RemoveItemByClass` (`/Game/Characters/PlayerCharacter/BP_PlayerCharacter.BPC_Inventory` (`self.PlayerRef`)) (`local.RequiredDryGrassClass`) (`local.RequiredDryGrassAmount`))
    (`self.SetCampFireLitState` true)
    (if (`|EnumEquality` (`self.CookingState`) "NewEnumerator1")
      (`self.StartCooking`))
    (else
      (`/Game/Characters/PlayerCharacter/HUD/WBP_WarningInfo.SetText` (`self.WarningInfoWidget`) (`local.NotEnoughMaterialText`))
      (`self.ShowWarning`))))

(fn `ResetObjectOnGrabbed`
  (set `self.Fuel` 0.0)
  (`self.SetCampFireLitState` false))

(fn `SetCampFireLitState`
  (params (NewLit :type Boolean))
  (if NewLit
    (set `self.IsLit` true)
    (`LightComponent.SetIntensity` (`self.PointLightComponent`) 5000.0)
    (`ActorComponent.Activate` (`self.ParticleSystem`) false)
    (set `self.Fuel` (`self.MaxFuel`))
    (`self.DrainFuel`)
    (else
      (set `self.IsLit` false)
      (`LightComponent.SetIntensity` (`self.PointLightComponent`) 0.0)
      (`ActorComponent.Deactivate` (`self.ParticleSystem`))))
  (`self.UpdateStateText`))

(fn `SpawnMeatMesh`
  (`SceneComponent.SetVisibility` (`self.MeatMesh`) true false))

(fn `Try Ignite Campfire`
  (locals (RequiredSticksAmount :type Integer :default 2) (RequiredDryGrassAmount :type Integer :default 1) (RequiredStickClass :type "/Game/Items/ItemObjects/BP_ItemObject Class Reference" :default "/Script/Engine.BlueprintGeneratedClass'/Game/Items/ItemObjects/Material/BP_MaterialObject_Stick.BP_MaterialObject_Stick_C'") (RequiredDryGrassClass :type "/Game/Items/ItemObjects/BP_ItemObject Class Reference" :default "/Script/Engine.BlueprintGeneratedClass'/Game/Items/ItemObjects/Material/BP_MaterialObject_DryGrass.BP_MaterialObject_DryGrass_C'") (OwnedStickAmount :type Integer) (OwnedDryGrassAmount :type Integer) (NotEnoughMaterialText :type Text :default "NSLOCTEXT(\"[4CEF8167105D2E92E35C5F314175C78E]\", \"837887134B88F3A6E171A289C3C29E14\", \"You need 2x Stick and 1x Dry Grass to light the Campfire\")"))
  (if (`self.CanInteractWithObject`)
    (if (`self.IsLit`)
      (switch `/Game/GrabbableObjects/E_CookingState` (`self.CookingState`)
        (:`NewEnumerator0`
          (`self.GivePlayerMeat`))
        (:`NewEnumerator1`
          (`/Game/Characters/PlayerCharacter/HUD/WBP_WarningInfo.SetText` (`self.WarningInfoWidget`) "In process of cooking")
          (`self.ShowWarning`))
        (:`NewEnumerator5`
          (`self.TryCookMeat`)))
      (else
        (switch `/Game/GrabbableObjects/E_CookingState` (`self.CookingState`)
          (:`NewEnumerator0`
            (`self.GivePlayerMeat`))
          (:`NewEnumerator1`
            (`self.LightUpCampfire`)
            (`self.StartCooking`))
          (:`NewEnumerator5`
            (`self.LightUpCampfire`)))))))

(fn `TryCookMeat`
  (bind _itemcount (`/Game/NewInventory/BPC_Inventory.GetItemCount` (`/Game/Characters/PlayerCharacter/BP_PlayerCharacter.BPC_Inventory` (`self.PlayerRef`)) "/Game/Items/ItemObjects/Food/BP_FoodObject_RawMeat.BP_FoodObject_RawMeat_C"))
  (if (> _itemcount 0)
    (`/Game/NewInventory/BPC_Inventory.RemoveItemByClass` (`/Game/Characters/PlayerCharacter/BP_PlayerCharacter.BPC_Inventory` (`self.PlayerRef`)) "/Game/Items/ItemObjects/Food/BP_FoodObject_RawMeat.BP_FoodObject_RawMeat_C" 1)
    (`self.StartCooking`)
    (else
      (`/Game/Characters/PlayerCharacter/HUD/WBP_WarningInfo.SetText` (`self.WarningInfoWidget`) "No Raw Meat in your inventory")
      (`self.ShowWarning`))))

(fn `UpdateStateText`
  (locals (StateText :type Text))
  (bind _aswbp_campfire_state (cast `/Game/GrabbableObjects/WBP_CampfireState` (`WidgetComponent.GetUserWidgetObject` (`self.WidgetComponent`))))
  (if (`self.IsLit`)
    (switch `/Game/GrabbableObjects/E_CookingState` (`self.CookingState`)
      (:`NewEnumerator0`
        (bind _textblock (`/Game/GrabbableObjects/WBP_CampfireState.TextBlock` _aswbp_campfire_state))
        (set `TextBlock.Text` "Cooked meat ready" _textblock))
      (:`NewEnumerator1`
        (set `TextBlock.Text` "Cooking..." _textblock))
      (:`NewEnumerator5`
        (set `TextBlock.Text` "Ready to cook" _textblock)))
    (elif (`|EnumEquality` (`self.CookingState`) "NewEnumerator0")
      (set `TextBlock.Text` "Cooked meat ready" _textblock)
      (else
        (set `TextBlock.Text` "" _textblock)))))

(fn `UserConstructionScript`
  (`parent.UserConstructionScript`))