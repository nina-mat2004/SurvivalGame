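; Grabbable campfire that the player lights with sticks and dry grass from the inventory, then uses to cook raw food.
; Lighting toggles light and particles and starts a self-repeating delayed fuel drain that extinguishes it when empty.
; A Not Cooking/Cooking/Ready state drives interaction, menu, food mesh and grabbability; cooking only finishes if still lit after the delay.
; A world widget shows state, yawing toward the player camera each tick.
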(event `self.ReceiveBeginPlay`
  (`parent.ReceiveBeginPlay`)
  (`self.UpdateStateText`))

(event `self.ReceiveTick`
  (params (DeltaSeconds :type "Float (single-precision)"))
  (`parent.ReceiveTick` DeltaSeconds)
  (`SceneComponent.K2_SetWorldRotation` (`self.WidgetComponent`) (`KismetMathLibrary.MakeRotator` 0.0 0.0 (.yaw (`KismetMathLibrary.FindLookAtRotation` (`SceneComponent.K2_GetComponentLocation` (`self.WidgetComponent`)) (`SceneComponent.K2_GetComponentLocation` (`/Game/PlayerCharacter/BP_PlayerCharacter.Camera` (`self.PlayerRef`)))))) false false))

(event `DrainFuel`
  (if (> (`self.Fuel`) 0.0)
    (set `self.Fuel` (- (`self.Fuel`) (`self.FuelDrainRate`)))
    (`KismetSystemLibrary.Delay` 1.0)
    (`self.DrainFuel`)
    (else
      (`self.SetCampFireLitState` false))))

(event `StartCooking`
  (params (RawFood :type "/Game/Items/ItemObjects/BP_ItemObject Class Reference") (CookedFood :type "/Game/Items/ItemObjects/BP_ItemObject Class Reference"))
  (`self.SpawnFoodMesh` RawFood)
  (set `self.CookingState` "NewEnumerator1")
  (set `self.CanBeGrabbed` false)
  (`self.UpdateStateText`)
  (`KismetSystemLibrary.Delay` (`self.CookTime`))
  (if (`self.IsLit`)
    (`self.FinishCooking` CookedFood)))

(fn `DespawnFoodMesh`
  (`StaticMeshComponent.SetStaticMesh` (`self.FoodMesh`) null))

(fn `FinishCooking`
  (params (CookedFood :type "/Game/Items/ItemObjects/BP_ItemObject Class Reference"))
  (`self.SpawnFoodMesh` CookedFood)
  (set `self.CookingState` "NewEnumerator0")
  (`self.UpdateStateText`)
  (set `self.CurrentCookedFood` CookedFood))

(fn `GivePlayerFood`
  (bind _currentcookedfood (`self.CurrentCookedFood`))
  (if (`KismetSystemLibrary.IsValidClass` _currentcookedfood)
    (bind _returnvalue (`|GenericCreateObject` _currentcookedfood))
    (bind _itemaddedsuccessfully (`/Game/Inventory/BPC_Inventory.AddItemToInventory` (`/Game/PlayerCharacter/BP_PlayerCharacter.BPC_Inventory` (`self.PlayerRef`)) (make `/Game/Inventory/S_ItemData` _returnvalue (struct) 1)))
    (if _itemaddedsuccessfully
      (set `self.CookingState` "NewEnumerator5")
      (set `self.CanBeGrabbed` true)
      (`self.DespawnFoodMesh`)
      (`self.UpdateStateText`)
      (else
        (`/Game/PlayerCharacter/GUI/WBP_WarningInfo.SetText` (`self.WarningInfoWidget`) "Your inventory is full")
        (`self.ShowWarning`)))))

(fn `HideCookingMenuWidget`
  (bind _returnvalue (`GameplayStatics.GetPlayerController` 0))
  (bind _playerref (`self.PlayerRef`))
  (set `self.CanBeGrabbed` true)
  (set `Widget.Visibility` "Hidden" (`/Game/PlayerCharacter/BP_PlayerCharacter.CookingMenuWidget` _playerref))
  (`CharacterMovementComponent.SetMovementMode` (`Character.CharacterMovement` _playerref) "MOVE_Walking" 0)
  (set `/Game/PlayerCharacter/BP_PlayerCharacter.IsCookingMenuOpened` false _playerref)
  (`WidgetBlueprintLibrary.SetInputMode_GameOnly` _returnvalue)
  (set `PlayerController.bShowMouseCursor` false _returnvalue))

(fn `LightUpCampfire`
  (locals (OwnedStickAmount :type Integer :default 0) (OwnedDryGrassAmount :type Integer :default 0) (RequiredStickAmount :type Integer :default 2) (RequiredDryGrassAmount :type Integer :default 1) (NotEnoughMaterialText :type Text :default "NSLOCTEXT(\"[4CEF8167105D2E92E35C5F314175C78E]\", \"46BD8E6043D7C1A63D652D81233FE6B9\", \"You need 2x Stick and 1x Dry Grass to light up the Campfire\")") (RequiredStickClass :type "/Game/Items/ItemObjects/BP_ItemObject Class Reference" :default "/Script/Engine.BlueprintGeneratedClass'/Game/Items/ItemObjects/Material/BP_MaterialObject_Stick.BP_MaterialObject_Stick_C'") (RequiredDryGrassClass :type "/Game/Items/ItemObjects/BP_ItemObject Class Reference" :default "/Script/Engine.BlueprintGeneratedClass'/Game/Items/ItemObjects/Material/BP_MaterialObject_DryGrass.BP_MaterialObject_DryGrass_C'"))
  (bind _itemcount (`/Game/Inventory/BPC_Inventory.GetItemCount` (`/Game/PlayerCharacter/BP_PlayerCharacter.BPC_Inventory` (`self.PlayerRef`)) (`local.RequiredStickClass`)))
  (set `local.OwnedStickAmount` _itemcount)
  (bind _itemcount_2 (`/Game/Inventory/BPC_Inventory.GetItemCount` (`/Game/PlayerCharacter/BP_PlayerCharacter.BPC_Inventory` (`self.PlayerRef`)) (`local.RequiredDryGrassClass`)))
  (set `local.OwnedDryGrassAmount` _itemcount_2)
  (if (and (>= (`local.OwnedStickAmount`) (`local.RequiredStickAmount`)) (>= (`local.OwnedDryGrassAmount`) (`local.RequiredDryGrassAmount`)))
    (`/Game/Inventory/BPC_Inventory.RemoveItemByClass` (`/Game/PlayerCharacter/BP_PlayerCharacter.BPC_Inventory` (`self.PlayerRef`)) (`local.RequiredStickClass`) (`local.RequiredStickAmount`))
    (`/Game/Inventory/BPC_Inventory.RemoveItemByClass` (`/Game/PlayerCharacter/BP_PlayerCharacter.BPC_Inventory` (`self.PlayerRef`)) (`local.RequiredDryGrassClass`) (`local.RequiredDryGrassAmount`))
    (`self.SetCampFireLitState` true)
    (if (`|EnumEquality` (`self.CookingState`) "NewEnumerator1")
      (`self.StartCooking` null))
    (else
      (`/Game/PlayerCharacter/GUI/WBP_WarningInfo.SetText` (`self.WarningInfoWidget`) (`local.NotEnoughMaterialText`))
      (`self.ShowWarning`))))

(fn `ResetObjectOnGrabbed`
  (set `self.Fuel` 0.0)
  (`self.SetCampFireLitState` false))

(fn `SetCampFireLitState`
  (params (NewLit :type Boolean))
  (if NewLit
    (set `self.IsLit` true)
    (`LightComponent.SetIntensity` (`self.PointLightComponent`) 5000.0)
    (`ActorComponent.Activate` (`self.ParticleSystem`) false)
    (set `self.Fuel` (`self.MaxFuel`))
    (`self.DrainFuel`)
    (else
      (set `self.IsLit` false)
      (`LightComponent.SetIntensity` (`self.PointLightComponent`) 0.0)
      (`ActorComponent.Deactivate` (`self.ParticleSystem`))))
  (`self.UpdateStateText`))

(fn `ShowCookingMenuWidget`
  (bind _returnvalue (`GameplayStatics.GetPlayerController` 0))
  (bind _playerref (`self.PlayerRef`))
  (bind _cookingmenuwidget (`/Game/PlayerCharacter/BP_PlayerCharacter.CookingMenuWidget` _playerref))
  (set `self.CanBeGrabbed` false)
  (`/Game/GrabbableObjects/Campfire/WBP_CookingMenu.UpdateCookingMenu` _cookingmenuwidget)
  (set `Widget.Visibility` "Visible" _cookingmenuwidget)
  (`CharacterMovementComponent.DisableMovement` (`Character.CharacterMovement` _playerref))
  (set `/Game/PlayerCharacter/BP_PlayerCharacter.IsCookingMenuOpened` true _playerref)
  (`WidgetBlueprintLibrary.SetInputMode_GameAndUIEx` _returnvalue null)
  (set `PlayerController.bShowMouseCursor` true _returnvalue))

(fn `SpawnFoodMesh`
  (params (Food :type "/Game/Items/ItemObjects/BP_ItemObject Class Reference"))
  (bind _returnvalue (`StaticMeshComponent.SetStaticMesh` (`self.FoodMesh`) (`.StaticMesh` (defaults `Object` Food))))
  (`KismetSystemLibrary.PrintString` (`KismetStringLibrary.Conv_BoolToString` _returnvalue)))

(fn `Try Cook Food`
  (params (RawFood :type "/Game/Items/ItemObjects/BP_ItemObject Class Reference") (CookedFood :type "/Game/Items/ItemObjects/BP_ItemObject Class Reference"))
  (`self.HideCookingMenuWidget`)
  (bind _itemcount (`/Game/Inventory/BPC_Inventory.GetItemCount` (`/Game/PlayerCharacter/BP_PlayerCharacter.BPC_Inventory` (`self.PlayerRef`)) RawFood))
  (if (> _itemcount 0)
    (`/Game/Inventory/BPC_Inventory.RemoveItemByClass` (`/Game/PlayerCharacter/BP_PlayerCharacter.BPC_Inventory` (`self.PlayerRef`)) RawFood 1)
    (`self.StartCooking` RawFood CookedFood)
    (else
      (`/Game/PlayerCharacter/GUI/WBP_WarningInfo.SetText` (`self.WarningInfoWidget`) "No Raw Meat in your inventory")
      (`self.ShowWarning`))))

(fn `TryInteractWithCampfire`
  (locals (RequiredSticksAmount :type Integer :default 2) (RequiredDryGrassAmount :type Integer :default 1) (RequiredStickClass :type "/Game/Items/ItemObjects/BP_ItemObject Class Reference" :default "/Script/Engine.BlueprintGeneratedClass'/Game/Items/ItemObjects/Material/BP_MaterialObject_Stick.BP_MaterialObject_Stick_C'") (RequiredDryGrassClass :type "/Game/Items/ItemObjects/BP_ItemObject Class Reference" :default "/Script/Engine.BlueprintGeneratedClass'/Game/Items/ItemObjects/Material/BP_MaterialObject_DryGrass.BP_MaterialObject_DryGrass_C'") (OwnedStickAmount :type Integer) (OwnedDryGrassAmount :type Integer) (NotEnoughMaterialText :type Text :default "NSLOCTEXT(\"[4CEF8167105D2E92E35C5F314175C78E]\", \"837887134B88F3A6E171A289C3C29E14\", \"You need 2x Stick and 1x Dry Grass to light the Campfire\")"))
  (if (`self.CanInteractWithObject`)
    (if (`self.IsLit`)
      (switch `/Game/GrabbableObjects/Campfire/E_CookingState` (`self.CookingState`)
        (:`NewEnumerator0`
          (`self.GivePlayerFood`))
        (:`NewEnumerator1`
          (`/Game/PlayerCharacter/GUI/WBP_WarningInfo.SetText` (`self.WarningInfoWidget`) "In process of cooking")
          (`self.ShowWarning`))
        (:`NewEnumerator5`
          (`self.ShowCookingMenuWidget`)))
      (else
        (switch `/Game/GrabbableObjects/Campfire/E_CookingState` (`self.CookingState`)
          (:`NewEnumerator0`
            (`self.GivePlayerFood`))
          (:`NewEnumerator1`
            (`self.LightUpCampfire`)
            (`self.StartCooking` null))
          (:`NewEnumerator5`
            (`self.LightUpCampfire`)))))))

(fn `UpdateStateText`
  (locals (StateText :type Text))
  (bind _aswbp_campfire_state (cast `/Game/GrabbableObjects/Campfire/WBP_CampfireState` (`WidgetComponent.GetUserWidgetObject` (`self.WidgetComponent`))))
  (if (`self.IsLit`)
    (switch `/Game/GrabbableObjects/Campfire/E_CookingState` (`self.CookingState`)
      (:`NewEnumerator0`
        (bind _textblock (`/Game/GrabbableObjects/Campfire/WBP_CampfireState.TextBlock` _aswbp_campfire_state))
        (set `TextBlock.Text` "Cooked meat ready" _textblock))
      (:`NewEnumerator1`
        (set `TextBlock.Text` "Cooking..." _textblock))
      (:`NewEnumerator5`
        (set `TextBlock.Text` "Ready to cook" _textblock)))
    (elif (`|EnumEquality` (`self.CookingState`) "NewEnumerator0")
      (set `TextBlock.Text` "Cooked meat ready" _textblock)
      (else
        (set `TextBlock.Text` "" _textblock)))))

(fn `UserConstructionScript`
  (`parent.UserConstructionScript`))