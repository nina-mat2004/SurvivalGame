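; BP_GrabbableObject is a grabbable object that turns solid once it reaches Landscape ground and refuses interaction until then.
; While not solid, Tick traces along the mesh's local Z by GroundOffset; a Landscape hit disables physics, blocks Pawns and sets IsSolid.
; CanInteractWithObject returns that state, briefly showing a warning widget when false.
; SetObjectIsNotSolid clears the flag, and ResetObjectOnGrabbed is an empty stub.
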(event `self.ReceiveBeginPlay`
  (bind _returnvalue (`|CreateWidget` "/Game/Characters/PlayerCharacter/HUD/WBP_WarningInfo.WBP_WarningInfo_C"))
  (bind _output_get (set `self.WarningInfoWidget` _returnvalue))
  (`UserWidget.AddToViewport` _output_get 0)
  (set `Widget.Visibility` "Hidden" _output_get)
  (bind _asbp_player_character (cast `/Game/Characters/PlayerCharacter/BP_PlayerCharacter` (`GameplayStatics.GetPlayerCharacter` 0)))
  (set `self.PlayerRef` _asbp_player_character))

(event `ShowWarning`
  (bind _warninginfowidget (`self.WarningInfoWidget`))
  (set `Widget.Visibility` "Visible" _warninginfowidget)
  (`KismetSystemLibrary.Delay` 3.0)
  (set `Widget.Visibility` "Hidden" _warninginfowidget)
  (`/Game/Characters/PlayerCharacter/HUD/WBP_WarningInfo.SetText` _warninginfowidget ""))

(event `self.ReceiveTick`
  (params (DeltaSeconds :type "Float (single-precision)"))
  (`self.TryToBeSolidObject`))

(fn `CanInteractWithObject`
  (returns (CanInteractWithObject :type Boolean))
  (locals (NotSolidText :type Text :default "NSLOCTEXT(\"[E6FDB42F814A30FE5C8773698A10ED2C]\", \"2844094C4514111854CEF9890991DE1D\", \"You can\\'t interact with this object because it is not solid\")"))
  (if (`self.IsSolid`)
    (return true)
    (else
      (`/Game/Characters/PlayerCharacter/HUD/WBP_WarningInfo.SetText` (`self.WarningInfoWidget`) (`local.NotSolidText`))
      (`self.ShowWarning`)
      (return false))))

(fn `ResetObjectOnGrabbed`)

(fn `SetObjectIsNotSolid`
  (set `self.IsSolid` false))

(fn `TryToBeSolidObject`
  (bind _staticmesh (`self.StaticMesh`))
  (bind _staticmesh_2 (`self.StaticMesh`))
  (if (not (`self.IsSolid`))
    (bind _outhit (`KismetSystemLibrary.LineTraceSingle` (`SceneComponent.K2_GetComponentLocation` _staticmesh) (`KismetMathLibrary.TransformLocation` (`SceneComponent.K2_GetComponentToWorld` _staticmesh) (`KismetMathLibrary.MakeVector` 0.0 0.0 (`self.Ground Offset`))) "TraceTypeQuery1"))
    (cast `Landscape` (`.HitActor` (`GameplayStatics.BreakHitResult` _outhit)))
    (`PrimitiveComponent.SetCollisionResponseToChannel` _staticmesh_2 "ECC_Pawn" "ECR_Block")
    (`PrimitiveComponent.SetSimulatePhysics` _staticmesh_2 false)
    (set `self.IsSolid` true)))

(fn `UserConstructionScript`)