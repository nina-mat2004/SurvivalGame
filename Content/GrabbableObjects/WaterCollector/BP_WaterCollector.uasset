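; Grabbable water collector that gains water on a repeating delay up to a cap and refills a water bottle from the player's inventory.
; UseWaterCollector tops up the first water object found, deducts the supply and completes a quest, or warns if water or a bottle is missing.
; A widget shows the supply and yaws toward the player camera.
; TryToBeSolidObject traces for landscape to disable physics and block pawns.
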(event `self.ReceiveBeginPlay`
  (`parent.ReceiveBeginPlay`)
  (`self.Refil`))

(event `self.ReceiveTick`
  (params (DeltaSeconds :type "Float (single-precision)"))
  (`parent.ReceiveTick` DeltaSeconds)
  (`SceneComponent.K2_SetWorldRotation` (`self.WidgetComponent`) (`KismetMathLibrary.MakeRotator` 0.0 0.0 (.yaw (`KismetMathLibrary.FindLookAtRotation` (`SceneComponent.K2_GetComponentLocation` (`self.WidgetComponent`)) (`SceneComponent.K2_GetComponentLocation` (`/Game/PlayerCharacter/BP_PlayerCharacter.Camera` (`self.PlayerRef`)))))) false false))

(event `Refil`
  (set `self.CollectorWaterSupply` (`KismetMathLibrary.FClamp` (+ (`self.CollectorWaterSupply`) 1.0) 0.0 (`self.MaxWaterSupply`)))
  (`self.UpdateStateText`)
  (`KismetSystemLibrary.Delay` (`self.RefilDelay`))
  (`self.Refil`))

(fn `TryToBeSolidObject`
  (bind _staticmesh (`self.StaticMesh`))
  (bind _staticmesh_2 (`self.StaticMesh`))
  (if (not (`self.IsSolid`))
    (bind _outhit (`KismetSystemLibrary.LineTraceSingle` (`SceneComponent.K2_GetComponentLocation` _staticmesh) (`KismetMathLibrary.TransformLocation` (`SceneComponent.K2_GetComponentToWorld` _staticmesh) (`KismetMathLibrary.MakeVector` 0.0 0.0 (`self.GroundOffset`))) "TraceTypeQuery1"))
    (cast `Landscape` (`.HitActor` (`GameplayStatics.BreakHitResult` _outhit)))
    (`PrimitiveComponent.SetCollisionResponseToChannel` _staticmesh_2 "ECC_Pawn" "ECR_Block")
    (`PrimitiveComponent.SetSimulatePhysics` _staticmesh_2 false)
    (set `self.IsSolid` true)))

(fn `UpdateStateText`
  (locals (CapacityText :type String :default "Capacity: "))
  (bind _aswbp_water_collector_state (cast `/Game/GrabbableObjects/WaterCollector/WBP_WaterCollectorState` (`WidgetComponent.GetUserWidgetObject` (`self.WidgetComponent`))))
  (`/Game/GrabbableObjects/WaterCollector/WBP_WaterCollectorState.UpdateStateText` _aswbp_water_collector_state (`self.CollectorWaterSupply`)))

(fn `UserConstructionScript`
  (`parent.UserConstructionScript`))

(fn `UseWaterCollector`
  (params (PlayerRef :type "/Game/PlayerCharacter/BP_PlayerCharacter Object Reference"))
  (locals (LocalIndex :type Integer))
  (bind _player_ref (`self.Player Ref`))
  (if (`self.CanInteractWithObject`)
    (bind _output_get (set `self.Player Ref` PlayerRef))
    (for (_array_element _array_index) (`/Game/Inventory/BPC_Inventory.Items` (`/Game/PlayerCharacter/BP_PlayerCharacter.BPC_Inventory` _output_get))
      (set `local.LocalIndex` _array_index)
      (bind (_itemobject _quantity) (break `/Game/Inventory/S_ItemData` _array_element))
      (`/Engine/EditorBlueprintResources/StandardMacros.IsValid` _itemobject
        (:`Is Valid`
          (bind _asbp_water_object (cast `/Game/Items/ItemObjects/Water/BP_WaterObject` _itemobject))
          (bind _waterpointstoadd (`/Game/Items/ItemObjects/Water/BP_WaterObject.WaterPointsToAdd` _asbp_water_object))
          (if (>= (`self.CollectorWaterSupply`) _waterpointstoadd)
            (set `/Game/Items/ItemObjects/Water/BP_WaterObject.WaterBottleSupply` (`KismetMathLibrary.FClamp` (+ _waterpointstoadd (`/Game/Items/ItemObjects/Water/BP_WaterObject.WaterBottleSupply` _asbp_water_object)) 0.0 100.0) _asbp_water_object)
            (`KismetArrayLibrary.Array_Set` (`/Game/Inventory/BPC_Inventory.Items` (`/Game/PlayerCharacter/BP_PlayerCharacter.BPC_Inventory` (`self.Player Ref`))) (`local.LocalIndex`) (make `/Game/Inventory/S_ItemData` _asbp_water_object _quantity))
            (set `self.CollectorWaterSupply` (- (`self.CollectorWaterSupply`) (`/Game/Items/ItemObjects/Water/BP_WaterObject.WaterPointsToAdd` _asbp_water_object)))
            (`self.UpdateStateText`)
            (`/Game/Quests/BP_QuestManager.CompleteQuest` (`/Game/PlayerCharacter/BP_PlayerCharacter.QuestManager` _player_ref) "UseWaterCollector")
            (`/Game/Inventory/BPC_Inventory.OnInventoryChanged` (`/Game/PlayerCharacter/BP_PlayerCharacter.BPC_Inventory` _player_ref))
            (return)
            (else
              (`/Game/PlayerCharacter/GUI/WBP_WarningInfo.SetText` (`self.WarningInfoWidget`) (`KismetTextLibrary.Conv_StringToText` (`self.NotEnoughWaterString`)))
              (`self.ShowWarning`)
              (return))))))
    (`/Game/PlayerCharacter/GUI/WBP_WarningInfo.SetText` (`self.WarningInfoWidget`) "You need to have Water Bottle in your Inventory")
    (`self.ShowWarning`)))