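; BP_WaterCollector is an interactable water source that passively gathers water and fills a water item in the player's inventory.
; A self-recalling Refil event with a delay raises its supply up to a maximum.
; UseWaterCollector scans inventory for a water definition, transfers its WaterPoints from the supply into that slot's runtime state and broadcasts the inventory change.
; It shows a warning when supply is insufficient or no bottle is found.
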(event `self.ReceiveBeginPlay`
  (`parent.ReceiveBeginPlay`)
  (`self.Refil`))

(event `Refil`
  (set `self.WaterSupply` (`KismetMathLibrary.Clamp` (+ (`self.WaterSupply`) 1) 0 (`self.MaxWaterSupply`)))
  (`KismetSystemLibrary.Delay` 3.0)
  (`self.Refil`))

(fn `UserConstructionScript`
  (`parent.UserConstructionScript`))

(fn `UseWaterCollector`
  (params (PlayerRef :type "/Game/Characters/PlayerCharacter/BP_PlayerCharacter Object Reference"))
  (locals (LocalIndex :type Integer))
  (if (`self.CanInteractWithObject`)
    (bind _output_get (set `self.Player Ref` PlayerRef))
    (for (_array_element _array_index) (`/Game/NewInventory/BPC_Inventory.Items` (`/Game/Characters/PlayerCharacter/BP_PlayerCharacter.BPC_Inventory` _output_get))
      (set `local.LocalIndex` _array_index)
      (bind (_itemdefinition _runtimestate _quantity) (break `/Game/NewInventory/S_InventorySlot` _array_element))
      (`/Engine/EditorBlueprintResources/StandardMacros.IsValid` _itemdefinition
        (:`Is Valid`
          (bind _asda_water_definition (cast `/Game/Items/ItemData/Water/DA_WaterDefinition` _itemdefinition))
          (bind _waterpoints (`/Game/Items/ItemData/Water/DA_WaterDefinition.WaterPoints` _asda_water_definition))
          (if (>= (`self.WaterSupply`) _waterpoints)
            (`KismetArrayLibrary.Array_Set` (`/Game/NewInventory/BPC_Inventory.Items` (`/Game/Characters/PlayerCharacter/BP_PlayerCharacter.BPC_Inventory` (`self.Player Ref`))) (`local.LocalIndex`) (make `/Game/NewInventory/S_InventorySlot` _asda_water_definition (make `/Game/NewInventory/S_RuntimeState` (`KismetMathLibrary.Clamp` (+ _waterpoints (`.WaterSupply_5_AFD39A71424FFA51BE4C578A92CD3F18` (break `/Game/NewInventory/S_RuntimeState` _runtimestate))) 0 100)) _quantity))
            (set `self.WaterSupply` (- (`self.WaterSupply`) (`/Game/Items/ItemData/Water/DA_WaterDefinition.WaterPoints` _asda_water_definition)))
            (`/Game/NewInventory/BPC_Inventory.OnInventoryChanged` (`/Game/Characters/PlayerCharacter/BP_PlayerCharacter.BPC_Inventory` (`self.Player Ref`)))
            (return)
            (else
              (`/Game/Characters/PlayerCharacter/HUD/WBP_WarningInfo.SetText` (`self.WarningInfoWidget`) (`KismetTextLibrary.Conv_StringToText` (`KismetStringLibrary.Concat_StrStr` (`self.NotEnoughWaterString`) (`KismetStringLibrary.Concat_StrStr` "(" (`KismetStringLibrary.Conv_IntToString` (`self.WaterSupply`)) "/" (`KismetStringLibrary.Conv_IntToString` (`self.MaxWaterSupply`)) ")"))))
              (`self.ShowWarning`)
              (return))))))
    (`/Game/Characters/PlayerCharacter/HUD/WBP_WarningInfo.SetText` (`self.WarningInfoWidget`) "You need to have Water Bottle in your Inventory")
    (`self.ShowWarning`)))