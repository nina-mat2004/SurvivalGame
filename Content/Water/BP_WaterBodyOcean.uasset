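; Ocean water body actor that detects when the player's camera goes underwater.
; Overlap events with BP_PlayerCharacter toggle a flag, and BeginPlay caches the player reference.
; While the flag is set, Tick compares camera height to the actor's Z, updates IsUnderWater on the player and calls ShowBreathWidget every submerged frame.
; Ending the overlap stops these checks without resetting IsUnderWater.
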(event `self.ReceiveActorBeginOverlap`
  (params (OtherActor :type "Actor Object Reference"))
  (cast `/Game/PlayerCharacter/BP_PlayerCharacter` OtherActor)
  (set `self.IsPlayerOverlapping` true))

(event `self.ReceiveActorEndOverlap`
  (params (OtherActor :type "Actor Object Reference"))
  (cast `/Game/PlayerCharacter/BP_PlayerCharacter` OtherActor)
  (set `self.IsPlayerOverlapping` false))

(event `self.ReceiveBeginPlay`
  (bind _asbp_player_character (cast `/Game/PlayerCharacter/BP_PlayerCharacter` (`GameplayStatics.GetPlayerCharacter` 0)))
  (set `self.PlayerRef` _asbp_player_character))

(event `self.ReceiveTick`
  (params (DeltaSeconds :type "Float (single-precision)"))
  (bind (_returnvalue_x _returnvalue_y _returnvalue_z) (`KismetMathLibrary.BreakVector` (`self.K2_GetActorLocation`)))
  (bind _playerref (`self.PlayerRef`))
  (bind (_returnvalue_x_2 _returnvalue_y_2 _returnvalue_z_2) (`KismetMathLibrary.BreakVector` (`SceneComponent.K2_GetComponentLocation` (`/Game/PlayerCharacter/BP_PlayerCharacter.Camera` (`self.PlayerRef`)))))
  (if (`self.IsPlayerOverlapping`)
    (if (< _returnvalue_z_2 _returnvalue_z)
      (set `/Game/PlayerCharacter/BP_PlayerCharacter.IsUnderWater` true _playerref)
      (`/Game/PlayerCharacter/BP_PlayerCharacter.ShowBreathWidget` _playerref)
      (else
        (set `/Game/PlayerCharacter/BP_PlayerCharacter.IsUnderWater` false (`self.PlayerRef`))))))

(fn `UserConstructionScript`)