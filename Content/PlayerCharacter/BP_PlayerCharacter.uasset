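; Player character for a survival game, handling interaction, physics grabbing, tool and hand attacks, sprinting, swimming, and death with respawn at the start point.
; Camera line traces drive pickup prompts, use, hit and grab actions, with a PhysicsHandle carrying and rotating objects on Tick.
; Inventory, crafting and attribute components track items and energy, alongside quest and time managers.
; It creates all HUD and menu widgets at BeginPlay, switching input and movement as menus toggle.
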(event `self.ReceiveTick`
  (params (DeltaSeconds :type "Float (single-precision)"))
  (`self.TryToFindObjectToInteractWith`)
  (`self.EventTickGrabbingObject`)
  (`self.RotateObjectVertically` DeltaSeconds)
  (`self.RotateObjectHorizontally` DeltaSeconds))

(event `self.ReceiveBeginPlay`
  (set `self.RespawnPoint` (`self.K2_GetActorLocation`))
  (`self.CreateInGameScreen`)
  (`self.CreateInteractionWidget`)
  (`self.Create Inventory Widget`)
  (`self.CreateCraftingMenuWidget`)
  (`self.CreateCookingMenuWidget`)
  (`self.CreateDialogLineWidget`)
  (`self.CreateStatsWidget`)
  (`self.CreateDeathScreenWidget`)
  (bind _returnvalue (`GameplayStatics.GetActorOfClass` "/Game/Quests/BP_QuestManager.BP_QuestManager_C"))
  (set `self.QuestManager` _returnvalue)
  (bind _returnvalue_2 (`GameplayStatics.GetActorOfClass` "/Game/DayNightCycle/BP_TimeManager.BP_TimeManager_C"))
  (set `self.TimeManager` _returnvalue_2))

(event `self.Buoyancy.OnEnteredWaterDelegate`
  (params (Pontoon :type "SphericalPontoon Structure (by ref)"))
  (bind _bpc_attributes (`self.BPC_Attributes`))
  ;[1 1 1] Swimming Movement
  (`CharacterMovementComponent.SetMovementMode` (`self.CharacterMovement`) "MOVE_Flying" 0)
  (set `self.IsSwimming` true)
  (`/Game/Attributes/BPC_Attributes.CleaningInWater` _bpc_attributes)
  (`/Game/Attributes/BPC_Attributes.DecreaseEnergy` _bpc_attributes))

(event `self.Buoyancy.OnExitedWaterDelegate`
  (params (Pontoon :type "SphericalPontoon Structure (by ref)"))
  ;[1 1 1] Swimming Movement
  (`CharacterMovementComponent.SetMovementMode` (`self.CharacterMovement`) "MOVE_Walking" 0)
  (set `self.IsSwimming` false))

(event `EndGameEvent`
  (set `Widget.Visibility` "Hidden" (`self.InGameScreenWidget`))
  (`KismetSystemLibrary.Delay` 2.0)
  (`GameplayStatics.OpenLevel` "EndScreenLevel"))

(event `PlayerDiedEvent`
  (`GameplayStatics.SetGamePaused` true)
  (`self.CloseAllMenus`)
  (`self.OpenMenu` (`self.DeathScreenWidget`)))

(event `PlayerRespawnEvent`
  (`GameplayStatics.SetGamePaused` false)
  (`self.CloseMenu` (`self.DeathScreenWidget`))
  (`/Game/Attributes/BPC_Attributes.SetAttributesAfterRespawn` (`self.BPC_Attributes`))
  (`/Game/Inventory/BPC_Inventory.DropItemsAfterDeath` (`self.BPC_Inventory`))
  (set `/Game/DayNightCycle/BP_TimeManager.LastDeathTotalGameHours` 0.0 (`self.TimeManager`))
  (`self.TeleportToRespawnPoint`))

(fn `CloseAllMenus`
  (set `Widget.Visibility` "Hidden" (`self.InventoryWidget`))
  (set `Widget.Visibility` "Hidden" (`self.CraftingMenuWidget`))
  (set `Widget.Visibility` "Hidden" (`self.StatsWidget`)))

(fn `CloseMenu`
  (params (UserWidget :type "UserWidget Object Reference"))
  (bind _returnvalue (`GameplayStatics.GetPlayerController` 0))
  (bind _charactermovement (`self.CharacterMovement`))
  (`Widget.SetVisibility` UserWidget "Hidden")
  (`WidgetBlueprintLibrary.SetInputMode_GameOnly` _returnvalue)
  (set `PlayerController.bShowMouseCursor` false _returnvalue)
  (if (`self.IsSwimming`)
    (`CharacterMovementComponent.SetMovementMode` _charactermovement "MOVE_Flying" 0)
    (else
      (`CharacterMovementComponent.SetMovementMode` _charactermovement "MOVE_Walking" 0)))
  (set `self.IsAnyMenuOpen` false))

(fn `Create Inventory Widget`
  (bind _returnvalue (`|CreateWidget` "/Game/Inventory/WBP_Inventory.WBP_Inventory_C"))
  (set `/Game/Inventory/WBP_Inventory.InventoryComponentRef` (`self.BPC_Inventory`) _returnvalue)
  (bind _output_get (set `self.InventoryWidget` _returnvalue))
  (`UserWidget.AddToViewport` _output_get 0)
  (`Widget.SetVisibility` _output_get "Hidden"))

(fn `CreateCookingMenuWidget`
  (bind _returnvalue (`|CreateWidget` "/Game/GrabbableObjects/Campfire/WBP_CookingMenu.WBP_CookingMenu_C"))
  (bind _output_get (set `self.CookingMenuWidget` _returnvalue))
  (`UserWidget.AddToViewport` _output_get 0)
  (set `Widget.Visibility` "Hidden" _output_get))

(fn `CreateCraftingMenuWidget`
  (bind _returnvalue (`|CreateWidget` "/Game/Crafting/UI/WBP_CraftingMenu.WBP_CraftingMenu_C"))
  (bind _output_get (set `self.CraftingMenuWidget` _returnvalue))
  (`UserWidget.AddToViewport` _output_get 0)
  (`Widget.SetVisibility` _output_get "Hidden"))

(fn `CreateDeathScreenWidget`
  (bind _returnvalue (`|CreateWidget` "/Game/MainMenu/Widgets/WBP_DeathScreen.WBP_DeathScreen_C"))
  (bind _output_get (set `self.DeathScreenWidget` _returnvalue))
  (`UserWidget.AddToViewport` _output_get 0)
  (set `Widget.Visibility` "Hidden" _output_get))

(fn `CreateDialogLineWidget`
  (bind _returnvalue (`|CreateWidget` "/Game/EndGameDialog/WBP_Subtitles.WBP_Subtitles_C"))
  (bind _output_get (set `self.DialogLineWidget` _returnvalue))
  (`UserWidget.AddToViewport` _output_get 0)
  (set `Widget.Visibility` "Hidden" _returnvalue))

(fn `CreateInGameScreen`
  (bind _returnvalue (`|CreateWidget` "/Game/PlayerCharacter/GUI/WBP_InGameScreen.WBP_InGameScreen_C"))
  (bind _output_get (set `self.InGameScreenWidget` _returnvalue))
  (`UserWidget.AddToViewport` _output_get 0)
  (bind _returnvalue_2 (`|CreateWidget` "/Game/PlayerCharacter/GUI/WBP_Breath.WBP_Breath_C"))
  (bind _output_get_2 (set `self.BreathUnderWaterWidget` _returnvalue_2))
  (`UserWidget.AddToViewport` _output_get_2 0)
  (set `Widget.Visibility` "Hidden" _output_get_2))

(fn `CreateInteractionWidget`
  ;[1 1 1] Interaction
  (bind _returnvalue (`|CreateWidget` "/Game/PlayerCharacter/GUI/WBP_PickUpText.WBP_PickUpText_C"))
  (bind _output_get (set `self.InteractionWidget` _returnvalue))
  (`UserWidget.AddToViewport` _output_get 0)
  (`Widget.SetVisibility` _output_get "Hidden")
  (bind _returnvalue_2 (`|CreateWidget` "/Game/PlayerCharacter/GUI/WBP_RotationInfo.WBP_RotationInfo_C"))
  (bind _output_get_2 (set `self.RotationWidget` _returnvalue_2))
  (`UserWidget.AddToViewport` _output_get_2 0)
  (`Widget.SetVisibility` _output_get_2 "Hidden"))

(fn `CreateStatsWidget`
  (bind _returnvalue (`|CreateWidget` "/Game/PlayerCharacter/GUI/WBP_PlayerStats.WBP_PlayerStats_C"))
  (bind _output_get (set `self.StatsWidget` _returnvalue))
  (`UserWidget.AddToViewport` _output_get 0)
  (set `Widget.Visibility` "Hidden" _output_get))

(fn `DestroyEquippedItem`
  (`self.K2_DestroyActor` (`self.CurrentEquipedItem`))
  (set `self.CurrentHotbarIndex` -1))

(fn `EventTickGrabbingObject`
  (bind _camera (`self.Camera`))
  (if (`self.IsGrabbingObject`)
    (`PhysicsHandleComponent.SetTargetLocation` (`self.PhysicsHandle`) (+ (`SceneComponent.K2_GetComponentLocation` _camera) (* (`KismetMathLibrary.GetForwardVector` (`SceneComponent.K2_GetComponentRotation` _camera)) (`self.TraceLength`))))))

(fn `HideBreathWidget`
  (set `Widget.Visibility` "Hidden" (`self.BreathUnderWaterWidget`)))

(fn `OpenMenu`
  (params (Menu :type "UserWidget Object Reference"))
  (bind _returnvalue (`GameplayStatics.GetPlayerController` 0))
  (if (not (`self.IsAnyMenuOpen`))
    (set `Widget.Visibility` "Visible" Menu)
    (`WidgetBlueprintLibrary.SetInputMode_GameAndUIEx` _returnvalue null)
    (set `PlayerController.bShowMouseCursor` true _returnvalue)
    (`CharacterMovementComponent.DisableMovement` (`self.CharacterMovement`))
    (set `self.IsAnyMenuOpen` true)))

(fn `ReleaseGrabbedObject`
  (if (`self.IsGrabbingObject`)
    (`PhysicsHandleComponent.ReleaseComponent` (`self.PhysicsHandle`))
    (set `self.IsGrabbingObject` false)
    (`/Game/GrabbableObjects/BP_GrabbableObject.SetObjectIsNotSolid` (`self.CurrentGrabbedObject`))
    (`Widget.SetVisibility` (`self.RotationWidget`) "Hidden")))

(fn `ResetGrabbedObject`
  (bind _currentgrabbedobject (`self.CurrentGrabbedObject`))
  (if (`self.IsGrabbingObject`)
    (`/Engine/EditorBlueprintResources/StandardMacros.IsValid` _currentgrabbedobject
      (:`Is Valid`
        (`self.ReleaseGrabbedObject`)
        (`SceneComponent.K2_SetWorldRotation` :`self` (`/Game/GrabbableObjects/BP_GrabbableObject.StaticMesh` _currentgrabbedobject))))))

(fn `RotateObjectHorizontally`
  (params (DeltaSeconds :type "Float (double-precision)"))
  (locals (RotationSpeedYaw :type "Float (double-precision)" :default 100.0))
  (bind _physicshandle (`self.PhysicsHandle`))
  (if (`self.IsRotatingObjectH`)
    (if (`self.IsGrabbingObject`)
      (`/Engine/EditorBlueprintResources/StandardMacros.IsValid` (`self.CurrentGrabbedObject`)
        (:`Is Valid`
          (`PhysicsHandleComponent.SetTargetRotation` _physicshandle (`KismetMathLibrary.MakeRotator` (.roll (`.TargetRotation` (`PhysicsHandleComponent.GetTargetLocationAndRotation` _physicshandle))) (.pitch (`.TargetRotation` (`PhysicsHandleComponent.GetTargetLocationAndRotation` _physicshandle))) (+ (.yaw (`.TargetRotation` (`PhysicsHandleComponent.GetTargetLocationAndRotation` _physicshandle))) (* DeltaSeconds (`local.RotationSpeedYaw`))))))))))

(fn `RotateObjectVertically`
  (params (DeltaSeconds :type "Float (double-precision)"))
  (locals (RotationSpeedPitch :type "Float (double-precision)" :default 100.0))
  (bind _physicshandle (`self.PhysicsHandle`))
  (if (`self.IsRotatingObjectV`)
    (if (`self.IsGrabbingObject`)
      (`/Engine/EditorBlueprintResources/StandardMacros.IsValid` (`self.CurrentGrabbedObject`)
        (:`Is Valid`
          (`PhysicsHandleComponent.SetTargetRotation` _physicshandle (`KismetMathLibrary.ComposeRotators` (`KismetMathLibrary.MakeRotator` 0.0 (* DeltaSeconds (`local.RotationSpeedPitch`))) (`.TargetRotation` (`PhysicsHandleComponent.GetTargetLocationAndRotation` _physicshandle)))))))))

(fn `ShowBreathWidget`
  (set `Widget.Visibility` "Visible" (`self.BreathUnderWaterWidget`)))

(fn `Spawn and Attach Equipped Item`
  (params (ItemToEquip :type "/Game/Items/ItemObjects/BP_ItemObject Object Reference"))
  (bind _currentequipeditem (`self.CurrentEquipedItem`))
  (bind _asbp_tool_object (cast `/Game/Items/ItemObjects/Tool/BP_ToolObject` ItemToEquip))
  (`/Engine/EditorBlueprintResources/StandardMacros.IsValid` _currentequipeditem
    (:`Is Valid`
      (`self.K2_DestroyActor` _currentequipeditem))
    (:`Is Not Valid`
      _))
  (bind _returnvalue (`|SpawnActorFromClass` (`/Game/Items/ItemObjects/Tool/BP_ToolObject.AttachActor` _asbp_tool_object) (`SceneComponent.K2_GetComponentToWorld` (`self.Mesh`)) "Undefined" "MultiplyWithRoot" null null))
  (`PrimitiveComponent.SetSimulatePhysics` (`/Game/Items/ToolActors/BP_ToolActor.StaticMesh` _returnvalue) false)
  (bind _output_get (set `self.CurrentEquipedItem` _returnvalue))
  (`self.K2_AttachToComponent` _output_get (`self.Mesh`) (`/Game/Items/ToolActors/BP_ToolActor.SocketName` _returnvalue) "SnapToTarget" "SnapToTarget" "KeepRelative" true))

(fn `StartSprinting`
  (if (`/Game/Attributes/BPC_Attributes.CanSprint` (`self.BPC_Attributes`))
    (set `CharacterMovementComponent.MaxWalkSpeed` 600.0 (`self.CharacterMovement`))
    (set `self.IsSprinting` true)
    (`/Game/Attributes/BPC_Attributes.DecreaseEnergy` (`self.BPC_Attributes`))))

(fn `StopSprinting`
  (set `CharacterMovementComponent.MaxWalkSpeed` 300.0 (`self.CharacterMovement`))
  (set `self.IsSprinting` false)
  (`/Game/Attributes/BPC_Attributes.IncreaseEnergy` (`self.BPC_Attributes`)))

(fn `TeleportToRespawnPoint`
  (`self.K2_SetActorLocation` (`self.RespawnPoint`)))

(fn `TryGrabObject`
  (bind _camera (`self.Camera`))
  (bind _returnvalue (`SceneComponent.K2_GetComponentLocation` _camera))
  (bind (_outhit _returnvalue_2) (`KismetSystemLibrary.LineTraceSingle` _returnvalue (+ _returnvalue (* (`KismetMathLibrary.GetForwardVector` (`SceneComponent.K2_GetComponentRotation` _camera)) (`self.TraceLength`))) "TraceTypeQuery1"))
  (if _returnvalue_2
    (bind (_bblockinghit _binitialoverlap _time _distance _location _impactpoint _normal _impactnormal _physmat _hitactor _hitcomponent) (`GameplayStatics.BreakHitResult` _outhit))
    (bind _asbp_grabbable_object (cast `/Game/GrabbableObjects/BP_GrabbableObject` _hitactor))
    (if (`/Game/GrabbableObjects/BP_GrabbableObject.CanBeGrabbed` _asbp_grabbable_object)
      (bind _output_get (set `self.CurrentGrabbedObject` _asbp_grabbable_object))
      (`PhysicsHandleComponent.GrabComponentAtLocationWithRotation` :`self` (`self.PhysicsHandle`) :`Component` _hitcomponent :`InBoneName` "GrabSocket" :`Location` (`SceneComponent.K2_GetComponentLocation` _hitcomponent))
      (`/Game/GrabbableObjects/BP_GrabbableObject.ResetObjectOnGrabbed` _output_get)
      (set `self.IsGrabbingObject` true)
      (bind _staticmesh (`/Game/GrabbableObjects/BP_GrabbableObject.StaticMesh` _output_get))
      (`PrimitiveComponent.SetCollisionResponseToChannel` _staticmesh "ECC_Pawn" "ECR_Ignore")
      (`PrimitiveComponent.SetSimulatePhysics` _staticmesh true)
      (`Widget.SetVisibility` (`self.RotationWidget`) "Visible"))))

(fn `TryHitObject`
  (bind _currentequipeditem (`self.CurrentEquipedItem`))
  (bind _camera (`self.Camera`))
  (bind _currentequipeditem_2 (`self.CurrentEquipedItem`))
  (bind _returnvalue (`SceneComponent.K2_GetComponentLocation` _camera))
  (bind _outhit (`KismetSystemLibrary.LineTraceSingle` _returnvalue (+ _returnvalue (* (`KismetMathLibrary.GetForwardVector` (`SceneComponent.K2_GetComponentRotation` _camera)) (`self.TraceLength`))) "TraceTypeQuery1"))
  (bind _asbp_harvestable_resource (cast `/Game/Resources/BP_HarvestableResource` (`.HitActor` (`GameplayStatics.BreakHitResult` _outhit)))
    (:`then`
      (if (`KismetSystemLibrary.IsValid` _currentequipeditem)
        (`/Game/Resources/BP_HarvestableResource.ApplyHitDamage` _asbp_harvestable_resource _currentequipeditem)
        (`/Game/Attributes/BPC_Attributes.AddDirtinessPoints` (`self.BPC_Attributes`) 5.0)))
    (:`CastFailed`
      (bind _asbp_animal_base (cast `/Game/AnimalAI/Base/BP_AnimalBase` (`.HitActor` (`GameplayStatics.BreakHitResult` _outhit))))
      (if (`KismetSystemLibrary.IsValid` _currentequipeditem_2)
        (bind _asbp_tool_object (castclass `/Game/Items/ItemObjects/Tool/BP_ToolObject` (`/Game/Items/ToolActors/BP_ToolActor.ObjectClass` _currentequipeditem_2)))
        (`TimelineComponent.PlayFromStart` (`/Game/Items/ToolActors/BP_ToolActor.TL_ToolSwing` _currentequipeditem_2))
        (`/Game/AnimalAI/Base/BP_AnimalBase.ReceiveDamage` _asbp_animal_base (`.Damage` (defaults `Object` _asbp_tool_object)) self)
        (else
          (`/Game/AnimalAI/Base/BP_AnimalBase.ReceiveDamage` _asbp_animal_base (`self.HandDamage`) self))))))

(fn `TryInteractWithObject`
  (bind _camera (`self.Camera`))
  (bind _returnvalue (`SceneComponent.K2_GetComponentLocation` _camera))
  (if (not (`self.IsGrabbingObject`))
    (bind _outhit (`KismetSystemLibrary.LineTraceSingle` _returnvalue (+ _returnvalue (* (`KismetMathLibrary.GetForwardVector` (`SceneComponent.K2_GetComponentRotation` _camera)) (`self.TraceLength`))) "TraceTypeQuery1"))
    (bind _asbp_grabbable_object (cast `/Game/GrabbableObjects/BP_GrabbableObject` (`.HitActor` (`GameplayStatics.BreakHitResult` _outhit))))
    (bind _output_get (set `self.CurrentGrabbableObjectInteraction` _asbp_grabbable_object))
    (bind _asbp_water_collector (cast `/Game/GrabbableObjects/WaterCollector/BP_WaterCollector` _output_get)
      (:`then`
        (`/Game/GrabbableObjects/WaterCollector/BP_WaterCollector.UseWaterCollector` _asbp_water_collector self))
      (:`CastFailed`
        (bind _asbp_bed (cast `/Game/GrabbableObjects/Bed/BP_Bed` _output_get)
          (:`then`
            (`/Game/GrabbableObjects/Bed/BP_Bed.TryToSleep` _asbp_bed))
          (:`CastFailed`
            (bind _asbp_campfire (cast `/Game/GrabbableObjects/Campfire/BP_Campfire` _output_get))
            (`/Game/GrabbableObjects/Campfire/BP_Campfire.TryInteractWithCampfire` _asbp_campfire)))))))

(fn `TryPickUpObject`
  (bind _currentinractable (`self.CurrentInractable`))
  (if (and (`KismetSystemLibrary.IsValid` _currentinractable) (not (`self.IsAnyMenuOpen`)))
    (bind _returnvalue (`|GenericCreateObject` (`/Game/Items/BP_PickableItemActor.ItemObjectClass` _currentinractable)))
    (bind _itemaddedsuccessfully (`/Game/Inventory/BPC_Inventory.AddItemToInventory` (`self.BPC_Inventory`) (make `/Game/Inventory/S_ItemData` _returnvalue (`/Game/Items/BP_PickableItemActor.RuntimeState` _currentinractable) 1)))
    (if _itemaddedsuccessfully
      (`self.K2_DestroyActor` (`self.CurrentInractable`))
      (bind _returnvalue_2 (`GameplayStatics.GetObjectClass` _returnvalue))
      (if (== _returnvalue_2 "/Game/Items/ItemObjects/Material/BP_MaterialObject_Stick.BP_MaterialObject_Stick_C")
        (`/Game/Quests/BP_QuestManager.CompleteQuest` (`self.QuestManager`) "GatherSticks"))
      (`/Game/Crafting/BPC_Crafting.AddDiscoveredItem` (`self.BPC_Crafting`) _returnvalue_2))))

(fn `TryToFindObjectToInteractWith`
  (locals (PickUpText :type Text :default "NSLOCTEXT(\"[D90F6FE00E9A5CB4518B163AAAE71BC7]\", \"87688B7D40145618D1635CA4A19CC162\", \"Press E to pick up\")") (InteractText :type Text :default "NSLOCTEXT(\"[D90F6FE00E9A5CB4518B163AAAE71BC7]\", \"FB07028C47E9F40B35939BA3C989AAF2\", \"Press E to interact or use RMB to grab\")"))
  (bind _interactionwidget (`self.InteractionWidget`))
  (bind _interactionwidget_2 (`self.InteractionWidget`))
  (bind _interactionwidget_3 (`self.InteractionWidget`))
  (bind _camera (`self.Camera`))
  (bind _interactionwidget_4 (`self.InteractionWidget`))
  (bind _interactionwidget_5 (`self.InteractionWidget`))
  (bind _returnvalue (`SceneComponent.K2_GetComponentLocation` _camera))
  (set `self.CurrentInractable` null)
  (`/Game/PlayerCharacter/GUI/WBP_PickUpText.SetText` _interactionwidget_5 "")
  (`Widget.SetVisibility` _interactionwidget_5 "Hidden")
  (if (not (`self.IsGrabbingObject`))
    (bind _outhit (`KismetSystemLibrary.LineTraceSingle` _returnvalue (+ _returnvalue (* (`KismetMathLibrary.GetForwardVector` (`SceneComponent.K2_GetComponentRotation` _camera)) (`self.TraceLength`))) "TraceTypeQuery1"))
    (bind _asbp_pickable_item_actor (cast `/Game/Items/BP_PickableItemActor` (`.HitActor` (`GameplayStatics.BreakHitResult` _outhit)))
      (:`then`
        (set `self.CurrentInractable` _asbp_pickable_item_actor)
        (`/Game/PlayerCharacter/GUI/WBP_PickUpText.SetText` _interactionwidget (`local.PickUpText`))
        (`Widget.SetVisibility` _interactionwidget "Visible"))
      (:`CastFailed`
        (`/Game/PlayerCharacter/GUI/WBP_PickUpText.SetText` _interactionwidget_4 "")
        (`Widget.SetVisibility` _interactionwidget_4 "Hidden")
        (cast `/Game/GrabbableObjects/BP_GrabbableObject` (`.HitActor` (`GameplayStatics.BreakHitResult` _outhit))
          (:`then`
            (`/Game/PlayerCharacter/GUI/WBP_PickUpText.SetText` _interactionwidget_2 (`local.InteractText`))
            (`Widget.SetVisibility` _interactionwidget_2 "Visible"))
          (:`CastFailed`
            (`/Game/PlayerCharacter/GUI/WBP_PickUpText.SetText` _interactionwidget_3 "")
            (`Widget.SetVisibility` _interactionwidget_3 "Hidden")))))))

(fn `UpdateEquippedItem`
  (params (Index :type Integer))
  (bind _itemobject (break `/Game/Inventory/S_ItemData` (`|GetArrayItem` (`/Game/Inventory/BPC_Inventory.HotbarItems` (`self.BPC_Inventory`)) Index)))
  (if (!= Index (`self.CurrentHotbarIndex`))
    (`/Engine/EditorBlueprintResources/StandardMacros.IsValid` _itemobject
      (:`Is Valid`
        (`self.Spawn and Attach Equipped Item` _itemobject)
        (set `self.CurrentHotbarIndex` Index))
      (:`Is Not Valid`
        (set `self.CurrentHotbarIndex` -1)))))

(fn `UserConstructionScript`)