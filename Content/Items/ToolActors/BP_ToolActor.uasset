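; BP_ToolActor is a tool actor set up to animate its StaticMesh with swing and attack motions.
; BeginPlay caches the mesh's relative idle rotation and location, deriving a rolled swing rotation and a Z-raised attack location.
; The TL_ToolSwing and TL_ToolAttack timelines lerp the mesh between those poses on update.
; Nothing in this graph plays either timeline.
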(event `self.ReceiveBeginPlay`
  (bind _output_get (set `self.ToolIdleRotation` (`SceneComponent.RelativeRotation` (`self.StaticMesh`))))
  (set `self.ToolSwingRotation` (`KismetMathLibrary.MakeRotator` (+ (.roll _output_get) 90.0) (.pitch _output_get) (.yaw _output_get)))
  (bind _output_get_2 (set `self.ToolIdleLocation` (`SceneComponent.RelativeLocation` (`self.StaticMesh`))))
  (set `self.ToolAttackLocation` (+ _output_get_2 (0.0 0.0 90.0))))

(fn `UserConstructionScript`)