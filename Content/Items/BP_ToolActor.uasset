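; BP_ToolActor is a tool item actor set up for a rotational swing of its static mesh.
; On BeginPlay it caches the mesh's relative rotation as the idle pose and derives a swing pose rolled 90 degrees from it.
; The TL_ToolSwing timeline would lerp the mesh between the two poses, but nothing in this graph plays it.
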(event `self.ReceiveBeginPlay`
  (bind _output_get (set `self.TooldIdleRotation` (`SceneComponent.RelativeRotation` (`self.StaticMesh`))))
  (set `self.ToolSwingRotation` (`KismetMathLibrary.MakeRotator` (+ (.roll _output_get) 90.0) (.pitch _output_get) (.yaw _output_get))))

(fn `UserConstructionScript`)