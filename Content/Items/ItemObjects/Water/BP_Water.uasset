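; BP_Water is a water bottle item that the player drinks from to gain water points.
; UseItem adds a fixed amount through the player's BPCAttributes and subtracts it from the bottle's supply, failing when too little remains.
; The item is never flagged for deletion, even when it runs low.
; GetItemInfo builds rich-text info showing the drink amount and remaining supply.
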(fn `GetItemInfo`
  (returns (ItemInfo :type Text))
  (locals (DrinkAmount :type String :default "Drink amount: ") (WaterSupply :type String :default "Water supply: "))
  (return (`KismetTextLibrary.Conv_StringToText` (`KismetStringLibrary.Concat_StrStr` "<DefaultSmall>" (`KismetStringLibrary.Concat_StrStr` (`local.DrinkAmount`) (`KismetStringLibrary.Conv_Int64ToString` (`KismetMathLibrary.Conv_DoubleToInt64` (`self.WaterPointsToAdd`))) "</> \n<DefaultSmall>" (`local.WaterSupply`) (`KismetStringLibrary.Conv_Int64ToString` (`KismetMathLibrary.Conv_DoubleToInt64` (`self.WaterBottleSupply`)))) "</>"))))

(fn `UseItem`
  (params (PlayerRef :type "/Game/PlayerCharacter/BP_PlayerCharacter Object Reference"))
  (returns (DeleteItem :type Boolean) (UsedSuccessfuly :type Boolean))
  (if (>= (`self.WaterBottleSupply`) (`self.WaterPointsToAdd`))
    (`/Game/Attributes/BPC_Attributes.AddWaterPoints` (`/Game/PlayerCharacter/BP_PlayerCharacter.BPC_Attributes` PlayerRef) (`self.WaterPointsToAdd`))
    (set `self.WaterBottleSupply` (- (`self.WaterBottleSupply`) (`self.WaterPointsToAdd`)))
    (return false true)
    (else
      (return false false))))