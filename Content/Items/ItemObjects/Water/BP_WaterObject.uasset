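; BP_WaterObject is a water item object whose use restores the player's water points from a limited supply.
; UseItem checks that the item's runtime WaterSupply covers one use of WaterPoints, otherwise nothing happens.
; On success it adds those points to the player and swaps the inventory entry for rebuilt item data with a reduced supply and unchanged quantity.
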(fn `UseItem`
  (params (ItemToUse :type "/Game/NewInventory/S_ItemData Structure") (PlayerRef :type "/Game/Characters/PlayerCharacter/BP_PlayerCharacter Object Reference") (InventoryComponent :type "/Game/NewInventory/BPC_Inventory Object Reference"))
  (bind (_itemobject _runtimestate _quantity) (break `/Game/NewInventory/S_ItemData` ItemToUse))
  (bind _watersupply (break `/Game/NewInventory/S_RuntimeState` _runtimestate))
  (bind _asbp_water_object (cast `/Game/Items/ItemObjects/Water/BP_WaterObject` _itemobject))
  (bind _waterpoints (`/Game/Items/ItemObjects/Water/BP_WaterObject.WaterPoints` _asbp_water_object))
  (if (>= _watersupply _waterpoints)
    (`/Game/Characters/PlayerCharacter/BP_PlayerCharacter.Add Water Points` PlayerRef _waterpoints)
    (`/Game/NewInventory/BPC_Inventory.SetInventoryItem` InventoryComponent ItemToUse (make `/Game/NewInventory/S_ItemData` _asbp_water_object (make `/Game/NewInventory/S_RuntimeState` (- _watersupply (`/Game/Items/ItemObjects/Water/BP_WaterObject.WaterPoints` _asbp_water_object))) _quantity))))