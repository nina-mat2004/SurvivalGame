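; BP_Heal is a healing item object that restores health to the player who uses it.
; UseItem adds HealthPoints through the player's BPCAttributes component, then always reports success and flags the item for deletion, making it single-use.
; GetItemInfo builds a small-styled rich text description from the HealAmount label and the HealthPoints value as a whole number.
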(fn `GetItemInfo`
  (returns (ItemInfo :type Text))
  (locals (HealAmount :type String :default "Heal amount: "))
  (return (`KismetTextLibrary.Conv_StringToText` (`KismetStringLibrary.Concat_StrStr` "<DefaultSmall>" (`local.HealAmount`) (`KismetStringLibrary.Conv_Int64ToString` (`KismetMathLibrary.Conv_DoubleToInt64` (`self.HealthPoints`))) "</>"))))

(fn `UseItem`
  (params (PlayerRef :type "/Game/PlayerCharacter/BP_PlayerCharacter Object Reference"))
  (returns (DeleteItem :type Boolean) (UsedSuccessfuly :type Boolean))
  (`/Game/Attributes/BPC_Attributes.AddHealthPoints` (`/Game/PlayerCharacter/BP_PlayerCharacter.BPC_Attributes` PlayerRef) (`self.HealthPoints`))
  (return true true))