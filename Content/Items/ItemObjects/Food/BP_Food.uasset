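; BP_Food is a food item object that restores the player's hunger when used.
; UseItem adds its HungerPoints through the player's BPCAttributes component, then reports success and flags the item for deletion.
; GetItemInfo builds tagged rich text showing the hunger restore amount, plus a "Can be cooked" note when CanBeCooked is set.
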(fn `GetItemInfo`
  (returns (ItemInfo :type Text))
  (locals (HungerRestore :type String :default "Hunger restore: ") (CanBeCookedString :type String))
  (if (`self.CanBeCooked`)
    (set `local.CanBeCookedString` "Can be cooked"))
  (return (`KismetTextLibrary.Conv_StringToText` (`KismetStringLibrary.Concat_StrStr` "<DefaultSmall>" (`local.HungerRestore`) (`KismetStringLibrary.Conv_Int64ToString` (`KismetMathLibrary.Conv_DoubleToInt64` (`self.HungerPoints`))) "</> \n<DefaultSmall>" (`local.CanBeCookedString`) "</>"))))

(fn `UseItem`
  (params (PlayerRef :type "/Game/PlayerCharacter/BP_PlayerCharacter Object Reference"))
  (returns (DeleteItem :type Boolean) (UsedSuccessfuly :type Boolean))
  (`/Game/Attributes/BPC_Attributes.AddHungerPoints` (`/Game/PlayerCharacter/BP_PlayerCharacter.BPC_Attributes` PlayerRef) (`self.HungerPoints`))
  (return true true))