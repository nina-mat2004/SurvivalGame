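; Item spawn point that scatters physics-simulated pickups of one item class at random reachable points within a radius.
; A self-rescheduling timed loop spawns a new batch once every tracked item is gone.
; On BeginPlay it restores items from the current save by spawn point ID, which defaults to the object name.
; GetSaveData packs the surviving items under that ID for saving.
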(event `self.ReceiveBeginPlay`
  (set `self.HomeLocation` (`self.K2_GetActorLocation`))
  (bind _asbp_game_instance (cast `/Game/Saving/BP_GameInstance` (`GameplayStatics.GetGameInstance`)))
  (bind _currentsave (`/Game/Saving/BP_GameInstance.CurrentSave` _asbp_game_instance))
  (`/Engine/EditorBlueprintResources/StandardMacros.IsValid` _currentsave
    (:`Is Valid`
      (for _array_element (`/Game/Saving/BP_SaveGame.ItemSpawnpoints` _currentsave)
        (if (`KismetStringLibrary.EqualEqual_StrStr` (`.ID_2_5F35A35B41550D29A4AF9DAD7CE8C67E` (break `/Game/Saving/SavingStructures/S_ItemSpawnpointData` _array_element)) (`self.ID`))
          (`self.ApplySaveData` _array_element))))
    (:`Is Not Valid`
      (`self.SpawnItems`)))
  (`self.RespawnItems`))

(event `RespawnItems`
  (if (`self.AreAllItemsPickedUp`)
    (`self.SpawnItems`))
  (`KismetSystemLibrary.Delay` (`self.RespawnDelay`))
  (`self.RespawnItems`))

(fn `ApplySaveData`
  (params (SaveData :type "/Game/Saving/SavingStructures/S_ItemSpawnpointData Structure"))
  (for _array_element (`.Items_7_6954492F46E3D133E802D9B968C8D4ED` (break `/Game/Saving/SavingStructures/S_ItemSpawnpointData` SaveData))
    (bind _returnvalue (`|SpawnActorFromClass` "/Game/Items/BP_PickableItemActor.BP_PickableItemActor_C" (`KismetMathLibrary.MakeTransform` (`.Location_35_226C467546458D7A7EE345AF41E46190` (break `/Game/Saving/SavingStructures/S_ItemPickUpData` _array_element))) "Undefined" "MultiplyWithRoot" null true null))
    (`/Game/Items/BP_PickableItemActor.ApplySaveData` _returnvalue _array_element)
    (`KismetArrayLibrary.Array_Add` (`self.SpawnedItems`) _returnvalue)))

(fn `AreAllItemsPickedUp`
  (returns (AllItemsPickedUp :type Boolean))
  (for _array_element (`self.SpawnedItems`)
    (`/Engine/EditorBlueprintResources/StandardMacros.IsValid` _array_element
      (:`Is Valid`
        (return false))))
  (return true))

(fn `GetSaveData`
  (returns (SaveData :type "/Game/Saving/SavingStructures/S_ItemSpawnpointData Structure"))
  (locals (ItemSaveData :type "Array of /Game/Saving/SavingStructures/S_ItemPickUpData Structure"))
  (for _array_element (`self.SpawnedItems`)
    (`/Engine/EditorBlueprintResources/StandardMacros.IsValid` _array_element
      (:`Is Valid`
        (`KismetArrayLibrary.Array_Add` (`local.ItemSaveData`) (`/Game/Items/BP_PickableItemActor.GetSaveData` _array_element)))))
  (return (make `/Game/Saving/SavingStructures/S_ItemSpawnpointData` (`self.ID`) (`local.ItemSaveData`))))

(fn `SpawnItems`
  (bind _actorclass (`self.ActorClass`))
  (bind (_id _displayname _description _itemtype _stackable _stacksize _staticmesh _staticmeshtransform) (defaults `Object` _actorclass))
  (for _ (range (`self.MinSpawnAmount`) (+ (`self.MaxSpawnAmount`) 1))
    (bind _returnvalue (`|SpawnActorFromClass` "/Game/Items/BP_PickableItemActor.BP_PickableItemActor_C" (`KismetMathLibrary.MakeTransform` (`NavigationSystemV1.K2_GetRandomReachablePointInRadius` (`self.HomeLocation`) (`self.SpawnRadius`) null null) (`KismetMathLibrary.MakeRotator` 0.0 0.0 (`KismetMathLibrary.RandomFloatInRange` 0.0 90.0))) "Undefined" "MultiplyWithRoot" null true null))
    (`KismetArrayLibrary.Array_Add` (`self.SpawnedItems`) _returnvalue)
    (set `/Game/Items/BP_PickableItemActor.ItemObjectClass` _actorclass _returnvalue)
    (bind _staticmesh_2 (`/Game/Items/BP_PickableItemActor.StaticMesh` _returnvalue))
    (`StaticMeshComponent.SetStaticMesh` _staticmesh_2 _staticmesh)
    (`SceneComponent.K2_SetRelativeTransform` _staticmesh_2 _staticmeshtransform false false)
    (`PrimitiveComponent.SetSimulatePhysics` _staticmesh_2 true)))

(fn `UserConstructionScript`
  (if (`KismetStringLibrary.IsEmpty` (`self.ID`))
    (set `self.ID` (`KismetSystemLibrary.GetObjectName` self))))