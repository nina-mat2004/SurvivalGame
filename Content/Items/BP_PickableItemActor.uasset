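; BP_PickableItemActor is a pickup item actor that can save and restore its state.
; Construction script defaults an empty ID to the object's name.
; GetSaveData packs ID, location, water supply, item class, mesh and that class's default mesh transform into a struct.
; ApplySaveData restores water supply, item class, mesh and relative transform, then enables physics, without applying the saved ID or location.
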(fn `ApplySaveData`
  (params (SaveData :type "/Game/Saving/SavingStructures/S_ItemPickUpData Structure"))
  (bind (_id _location _watersupply _itemclass _staticmesh _meshtransform) (break `/Game/Saving/SavingStructures/S_ItemPickUpData` SaveData))
  (bind _staticmesh_2 (`self.StaticMesh`))
  (set `self.WaterSupply` _watersupply)
  (set `self.ItemObjectClass` _itemclass)
  (`StaticMeshComponent.SetStaticMesh` _staticmesh_2 _staticmesh)
  (`SceneComponent.K2_SetRelativeTransform` _staticmesh_2 _meshtransform false false)
  (`PrimitiveComponent.SetSimulatePhysics` _staticmesh_2 true))

(fn `GetSaveData`
  (returns (SaveData :type "/Game/Saving/SavingStructures/S_ItemPickUpData Structure"))
  (return (make `/Game/Saving/SavingStructures/S_ItemPickUpData` (`self.ID`) (`self.K2_GetActorLocation`) (`self.WaterSupply`) (`self.ItemObjectClass`) (`StaticMeshComponent.StaticMesh` (`self.StaticMesh`)) (`.StaticMeshTransform` (defaults `Object` (`self.ItemObjectClass`))))))

(fn `UserConstructionScript`
  (if (`KismetStringLibrary.IsEmpty` (`self.ID`))
    (set `self.ID` (`KismetSystemLibrary.GetObjectName` self))))