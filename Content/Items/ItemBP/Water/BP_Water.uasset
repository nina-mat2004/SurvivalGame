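; BP_Water is a usable water bottle item that lets the player drink from a limited water supply.
; UseItem casts the selected item's ItemClass to BP_Water and checks that its supply covers one drink.
; If so, it adds water points to the player and lowers its own WaterSupply within a clamped range; otherwise it prints a warning.
; The event graph and construction script add no logic of their own.
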(fn `UseItem`
  (params (BPC_Inventory :type "/Game/NewInventory/BPC_Inventory Object Reference") (SelectedItem :type "/Game/NewInventory/S_ItemData Structure"))
  (locals (OneDrinkOfWater :type Integer :default 25))
  (bind _asbp_water (cast `/Game/Items/ItemBP/Water/BP_Water` (`.ItemClass_37_5E96F30A488B4287D92F9A9E36D555D4` (break `/Game/NewInventory/S_ItemData` SelectedItem))))
  (if (>= (`/Game/Items/ItemBP/Water/BP_Water.WaterSupply` _asbp_water) (`local.OneDrinkOfWater`))
    (`/Game/Characters/PlayerCharacter/BP_PlayerCharacter.Add Water Points` (`self.PlayerRef`) (`local.OneDrinkOfWater`))
    (set `self.WaterSupply` (`KismetMathLibrary.Clamp` (- (`self.WaterSupply`) (`local.OneDrinkOfWater`)) 0 100))
    (else
      (`KismetSystemLibrary.PrintString` "Not enough water in water bottle"))))

(fn `UserConstructionScript`
  (`parent.UserConstructionScript`))