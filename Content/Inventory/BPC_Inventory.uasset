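; Inventory component for the player character, managing fixed-size item and hotbar slot arrays with stacking, per-type duplicate limits, and timed on-screen warnings.
; Adding, deleting and hotbar equipping update both arrays and fire change events, with tools tracking their own hotbar flag.
; Using items plays type-specific sounds and may consume them.
; Dropping spawns physics pickup actors, and death randomly drops or destroys each stack.
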(event `self.ReceiveBeginPlay`
  (`KismetArrayLibrary.Array_Resize` (`self.Items`) (`self.InventorySize`))
  (`KismetArrayLibrary.Array_Resize` (`self.HotbarItems`) (`self.HotbarSize`))
  (bind _returnvalue (`GameplayStatics.GetActorOfClass` "/Game/PlayerCharacter/BP_PlayerCharacter.BP_PlayerCharacter_C"))
  (set `self.PlayerRef` _returnvalue)
  (bind _returnvalue_2 (`|CreateWidget` "/Game/PlayerCharacter/UI/WBP_InventoryWarningText.WBP_InventoryWarningText_C"))
  (bind _output_get (set `self.InvWarningWidget` _returnvalue_2))
  (`UserWidget.AddToViewport` _output_get 0)
  (`Widget.SetVisibility` _output_get "Hidden"))

(event `ShowWarning`
  (bind _invwarningwidget (`self.InvWarningWidget`))
  (set `Widget.Visibility` "Visible" _invwarningwidget)
  (`KismetSystemLibrary.Delay` 3.0)
  (set `Widget.Visibility` "Hidden" _invwarningwidget)
  (`/Game/PlayerCharacter/UI/WBP_InventoryWarningText.SetText` _invwarningwidget ""))

(fn `Add Item To Hotbar`
  (params (SelectedItem :type "/Game/Inventory/S_ItemData Structure"))
  (locals (LocalIndex :type Integer))
  (bind (_itemobject _quantity) (break `/Game/Inventory/S_ItemData` SelectedItem))
  (bind _returnvalue (`KismetArrayLibrary.Array_Find` (`self.Items`) SelectedItem))
  (if (> _returnvalue -1)
    (set `local.LocalIndex` _returnvalue)
    (bind _asbp_tool_object (cast `/Game/Items/ItemObjects/Tool/BP_Tool` _itemobject))
    (if (not (`/Game/Items/ItemObjects/Tool/BP_Tool.IsInHotbar` _asbp_tool_object))
      (bind (_canadditem _freeindex) (`self.Can Add Item to Hotbar`))
      (if _canadditem
        (set `/Game/Items/ItemObjects/Tool/BP_Tool.IsInHotbar` true _asbp_tool_object)
        (`KismetArrayLibrary.Array_Set` (`self.HotbarItems`) _freeindex (make `/Game/Inventory/S_ItemData` _asbp_tool_object _quantity))
        (`self.OnHotbarChanged`)
        (`KismetArrayLibrary.Array_Set` (`self.Items`) (`local.LocalIndex`) (make `/Game/Inventory/S_ItemData` _asbp_tool_object _quantity))
        (`GameplayStatics.PlaySound2D` "/Game/3rdPartyAssets/Sounds/Sounds/item_equip.item_equip" 1.0 1.0 0.0 null null)
        (`self.OnInventoryChanged`)
        (return)
        (else
          (`self.SetWarningText` (`self.HotbarFullText`))
          (return))))))

(fn `AddItemToInventory`
  (params (NewItem :type "/Game/Inventory/S_ItemData Structure"))
  (returns (ItemAddedSuccessfully :type Boolean))
  (locals (LocalNewItem :type "/Game/Inventory/S_ItemData Structure") (LocalIndex :type Integer))
  (bind (_itemobject _quantity) (break `/Game/Inventory/S_ItemData` (`local.LocalNewItem`)))
  (bind _itemtype (`/Game/Items/ItemObjects/BP_Item.ItemType` (`.ItemObject_49_5E96F30A488B4287D92F9A9E36D555D4` (break `/Game/Inventory/S_ItemData` NewItem))))
  (set `local.LocalNewItem` NewItem)
  (if (or (`|EnumEquality` _itemtype "NewEnumerator1") (`|EnumEquality` _itemtype "NewEnumerator3") (`|EnumEquality` _itemtype "NewEnumerator5"))
    (bind _containsitem (`self.ContainsItem` (`local.LocalNewItem`)))
    (if _containsitem
      (`self.SetWarningText` (`self.CantHoldMoreText`))
      (return false)
      (else
        _)))
  (for (_array_element _array_index) (`self.Items`)
    (set `local.LocalIndex` _array_index)
    (bind (_itemobject_2 _quantity_2) (break `/Game/Inventory/S_ItemData` _array_element))
    (if (`KismetSystemLibrary.IsValid` _itemobject_2)
      (if (and (`/Game/Items/ItemObjects/BP_Item.Stackable` _itemobject_2) (== (`/Game/Items/ItemObjects/BP_Item.ID` _itemobject_2) (`/Game/Items/ItemObjects/BP_Item.ID` _itemobject)))
        (bind _returnvalue (+ _quantity_2 _quantity))
        (if (<= _returnvalue (`/Game/Items/ItemObjects/BP_Item.StackSize` _itemobject_2))
          (`KismetArrayLibrary.Array_Set` (`self.Items`) (`local.LocalIndex`) (make `/Game/Inventory/S_ItemData` _itemobject_2 _returnvalue))
          (`self.OnInventoryChanged`)
          (return true)
          (else
            (`self.SetWarningText` (`self.CantHoldMoreText`))
            (return false))))))
  (if (`self.IsInventoryFull`)
    (`self.SetWarningText` (`self.InventoryFullText`))
    (return false)
    (else
      (bind _emptyindex (`self.FindFirstEmptyIndex`))
      (if (> _emptyindex -1)
        (`KismetArrayLibrary.Array_Set` (`self.Items`) _emptyindex (`local.LocalNewItem`))
        (`self.OnInventoryChanged`)
        (return true)))))

(fn `Can Add Item to Hotbar`
  (returns (CanAddItem :type Boolean) (FreeIndex :type Integer))
  (for (_array_element _array_index) (`self.HotbarItems`)
    (`/Engine/EditorBlueprintResources/StandardMacros.IsValid` (`.ItemObject_49_5E96F30A488B4287D92F9A9E36D555D4` (break `/Game/Inventory/S_ItemData` _array_element))
      (:`Is Not Valid`
        (return true _array_index))))
  (return false -1))

(fn `ContainsItem`
  (params (NewItem :type "/Game/Inventory/S_ItemData Structure"))
  (returns (ContainsItem :type Boolean))
  (for _array_element (`self.Items`)
    (bind _itemobject (break `/Game/Inventory/S_ItemData` _array_element))
    (`/Engine/EditorBlueprintResources/StandardMacros.IsValid` _itemobject
      (:`Is Valid`
        (if (== (`/Game/Items/ItemObjects/BP_Item.ID` _itemobject) (`/Game/Items/ItemObjects/BP_Item.ID` (`.ItemObject_49_5E96F30A488B4287D92F9A9E36D555D4` (break `/Game/Inventory/S_ItemData` NewItem))))
          (return true)))))
  (return false))

(fn `DeleteItemFromHotbar`
  (params (SelectedItem :type "/Game/Inventory/S_ItemData Structure"))
  (locals (CachedIndex :type Integer :default 0))
  (bind (_itemobject _quantity) (break `/Game/Inventory/S_ItemData` SelectedItem))
  (bind _hotbaritems (`self.HotbarItems`))
  (bind _playerref (`self.PlayerRef`))
  (bind _returnvalue (`KismetArrayLibrary.Array_Find` _hotbaritems SelectedItem))
  (bind _returnvalue_2 (`KismetArrayLibrary.Array_Find` (`self.Items`) SelectedItem))
  (bind _asbp_tool_object (cast `/Game/Items/ItemObjects/Tool/BP_Tool` _itemobject))
  (if (`/Game/Items/ItemObjects/Tool/BP_Tool.IsInHotbar` _asbp_tool_object)
    (`GameplayStatics.PlaySound2D` "/Game/3rdPartyAssets/Sounds/Sounds/item_equip.item_equip" 1.0 1.0 0.0 null null)
    (if (and (>= _returnvalue 0) (>= _returnvalue_2 0))
      (set `local.CachedIndex` _returnvalue)
      (set `/Game/Items/ItemObjects/Tool/BP_Tool.IsInHotbar` false _asbp_tool_object)
      (`KismetArrayLibrary.Array_Set` _hotbaritems _returnvalue)
      (`self.OnHotbarChanged`)
      (`KismetArrayLibrary.Array_Set` (`self.Items`) _returnvalue_2 (make `/Game/Inventory/S_ItemData` _asbp_tool_object _quantity))
      (`self.OnInventoryChanged`)
      (if (== (`local.CachedIndex`) (`/Game/PlayerCharacter/BP_PlayerCharacter.CurrentHotbarIndex` _playerref))
        (`/Game/PlayerCharacter/BP_PlayerCharacter.DestroyEquippedItem` _playerref)))))

(fn `DeleteItemFromInventory`
  (params (ItemToDelete :type "/Game/Inventory/S_ItemData Structure"))
  (locals (LocalIndex :type Integer :default 0))
  (for (_array_element _array_index) (`self.Items`)
    (bind _itemobject (break `/Game/Inventory/S_ItemData` _array_element))
    (`/Engine/EditorBlueprintResources/StandardMacros.IsValid` _itemobject
      (:`Is Valid`
        (if (== (`/Game/Items/ItemObjects/BP_Item.ID` _itemobject) (`/Game/Items/ItemObjects/BP_Item.ID` (`.ItemObject_49_5E96F30A488B4287D92F9A9E36D555D4` (break `/Game/Inventory/S_ItemData` ItemToDelete))))
          (bind _output_get (set `local.LocalIndex` _array_index))
          (bind _output (`|GetArrayItem` (`self.Items`) _output_get))
          (`self.DeleteItemFromHotbar` _output)
          (bind (_itemobject_2 _quantity) (break `/Game/Inventory/S_ItemData` _output))
          (if (> _quantity 1)
            (`KismetArrayLibrary.Array_Set` (`self.Items`) (`local.LocalIndex`) (make `/Game/Inventory/S_ItemData` _itemobject_2 (- _quantity 1)))
            (else
              (`KismetArrayLibrary.Array_Set` (`self.Items`) (`local.LocalIndex`))
              (set `/Game/Inventory/UI/WBP_Inventory.SelectedItem` (struct) (`/Game/PlayerCharacter/BP_PlayerCharacter.InventoryWidget` (`self.PlayerRef`)))))
          (`self.OnInventoryChanged`)
          (return))))))

(fn `DropItem`
  (params (SelectedItem :type "/Game/Inventory/S_ItemData Structure"))
  (locals (CachedIndex :type Integer :default 0))
  (bind _itemobject (break `/Game/Inventory/S_ItemData` SelectedItem))
  (bind _playerref (`self.PlayerRef`))
  (bind _returnvalue (`|SpawnActorFromClass` "/Game/Items/BP_PickableItemActor.BP_PickableItemActor_C" (`KismetMathLibrary.MakeTransform` (+ (`Actor.K2_GetActorLocation` _playerref) (* (`KismetMathLibrary.GetForwardVector` (`Actor.K2_GetActorRotation` _playerref)) (`KismetMathLibrary.RandomFloatInRange` 100.0 150.0)) (* (`KismetMathLibrary.GetRightVector` (`Pawn.GetControlRotation` _playerref)) (`KismetMathLibrary.RandomFloatInRange` -50.0 50.0)))) "Undefined" "MultiplyWithRoot" null false null))
  (bind _asbp_water_object (cast `/Game/Items/ItemObjects/Water/BP_Water` _itemobject)
    (:`then`
      (set `/Game/Items/BP_PickableItemActor.WaterSupply` (`/Game/Items/ItemObjects/Water/BP_Water.WaterBottleSupply` _asbp_water_object) _returnvalue))
    (:`CastFailed`
      _))
  (set `/Game/Items/BP_PickableItemActor.ItemObjectClass` (`GameplayStatics.GetObjectClass` _itemobject) _returnvalue)
  (bind _staticmesh (`/Game/Items/BP_PickableItemActor.StaticMesh` _returnvalue))
  (`StaticMeshComponent.SetStaticMesh` _staticmesh (`/Game/Items/ItemObjects/BP_Item.StaticMesh` _itemobject))
  (`SceneComponent.K2_SetRelativeTransform` _staticmesh (`/Game/Items/ItemObjects/BP_Item.StaticMeshTransform` _itemobject) false false)
  (`PrimitiveComponent.SetSimulatePhysics` _staticmesh true)
  (`self.DeleteItemFromInventory` SelectedItem))

(fn `DropItemsAfterDeath`
  (locals (SpawnChance :type Integer :default 75) (ItemOriginalQuantity :type Integer))
  (for _array_element (`self.Items`)
    (bind (_itemobject _quantity) (break `/Game/Inventory/S_ItemData` _array_element))
    (`/Engine/EditorBlueprintResources/StandardMacros.IsValid` _itemobject
      (:`Is Valid`
        (set `local.ItemOriginalQuantity` _quantity)
        (if (< (`KismetMathLibrary.RandomInteger` 100) (`local.SpawnChance`))
          (for _ (range (`local.ItemOriginalQuantity`))
            (`self.DropItem` _array_element)
            (`self.OnInventoryChanged` :!label _label)
            (`self.OnHotbarChanged`))
          (else
            (for _ (range (`local.ItemOriginalQuantity`))
              (`self.DeleteItemFromInventory` _array_element)
              (goto _label))))))))

(fn `FindFirstEmptyIndex`
  (returns (EmptyIndex :type Integer))
  (for (_array_element _array_index) (`self.Items`)
    (if (not (`KismetSystemLibrary.IsValid` (`.ItemObject_49_5E96F30A488B4287D92F9A9E36D555D4` (break `/Game/Inventory/S_ItemData` _array_element))))
      (return _array_index)))
  (return -1))

(fn `GetItemCount`
  (params (ItemClass :type "/Game/Items/ItemObjects/BP_Item Class Reference"))
  (returns (ItemCount :type Integer))
  (for _array_element (`self.Items`)
    (bind (_itemobject _quantity) (break `/Game/Inventory/S_ItemData` _array_element))
    (if (== ItemClass (`GameplayStatics.GetObjectClass` _itemobject))
      (return _quantity)))
  (return 0))

(fn `IsInventoryEmpty`
  (returns (IsEmpty :type Boolean))
  (for _array_element (`self.Items`)
    (`/Engine/EditorBlueprintResources/StandardMacros.IsValid` (`.ItemObject_49_5E96F30A488B4287D92F9A9E36D555D4` (break `/Game/Inventory/S_ItemData` _array_element))
      (:`Is Valid`
        (return false))))
  (return true))

(fn `IsInventoryFull`
  (returns (IsInenvotryFull :type Boolean))
  (for _array_element (`self.Items`)
    (if (not (`KismetSystemLibrary.IsValid` (`.ItemObject_49_5E96F30A488B4287D92F9A9E36D555D4` (break `/Game/Inventory/S_ItemData` _array_element))))
      (return false)))
  (return true))

(fn `RemoveItemByClass`
  (params (ItemClass :type "/Game/Items/ItemObjects/BP_Item Class Reference") (Amount :type Integer))
  (for (_array_element _array_index) (`self.Items`)
    (bind (_itemobject _quantity) (break `/Game/Inventory/S_ItemData` _array_element))
    (if (== ItemClass (`GameplayStatics.GetObjectClass` _itemobject))
      (bind _returnvalue (- _quantity Amount))
      (if (> _returnvalue 0)
        (`KismetArrayLibrary.Array_Set` (`self.Items`) _array_index (make `/Game/Inventory/S_ItemData` _itemobject _returnvalue))
        (else
          (`KismetArrayLibrary.Array_Set` (`self.Items`) _array_index)
          (set `/Game/Inventory/UI/WBP_Inventory.SelectedItem` (struct) (`/Game/PlayerCharacter/BP_PlayerCharacter.InventoryWidget` (`self.PlayerRef`)))))
      (`self.OnInventoryChanged`))))

(fn `SetWarningText`
  (params (Text :type Text))
  (`/Game/PlayerCharacter/UI/WBP_InventoryWarningText.SetText` (`self.InvWarningWidget`) Text)
  (`self.ShowWarning`))

(fn `UseItem`
  (params (SelectedItem :type "/Game/Inventory/S_ItemData Structure"))
  (locals (CachedIndex :type Integer :default 0))
  (bind _itemobject (break `/Game/Inventory/S_ItemData` SelectedItem))
  (bind (_deleteitem _usedsuccessfuly) (`/Game/Items/ItemObjects/BP_Item.UseItem` _itemobject (`self.PlayerRef`)))
  (if _usedsuccessfuly
    (switch `/Game/Items/E_ItemType` (`/Game/Items/ItemObjects/BP_Item.ItemType` _itemobject)
      (:`NewEnumerator0`
        (`GameplayStatics.PlaySound2D` "/Game/3rdPartyAssets/Sounds/Sounds/food_eat.food_eat" 1.0 1.0 0.0 null null))
      (:`NewEnumerator3`
        (`GameplayStatics.PlaySound2D` "/Game/3rdPartyAssets/Sounds/Sounds/water_drink.water_drink" 1.0 1.0 0.0 null null))
      (:`NewEnumerator4`
        (`GameplayStatics.PlaySound2D` "/Game/3rdPartyAssets/Sounds/Sounds/bandage_use.bandage_use" 1.0 1.0 0.0 null null)))
    (if _deleteitem
      (`self.DeleteItemFromInventory` SelectedItem))))