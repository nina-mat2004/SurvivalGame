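; Inventory component that manages the player's fixed-size item slots and hotbar, with changes announced through inventory and hotbar change calls.
; Adding blocks duplicates of two item types and merges stacks without splitting overflow, showing failures in a timed warning widget.
; Hotbar tools stay in the inventory, flagged on their tool object.
; Use delegates to the item object, while drop spawns its world actor ahead of the player, preserving water runtime state.
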(event `self.ReceiveBeginPlay`
  (`KismetArrayLibrary.Array_Resize` (`self.Items`) (`self.InventorySize`))
  (`KismetArrayLibrary.Array_Resize` (`self.HotbarItems`) (`self.HotbarSize`))
  (bind _returnvalue (`GameplayStatics.GetActorOfClass` "/Game/Characters/PlayerCharacter/BP_PlayerCharacter.BP_PlayerCharacter_C"))
  (set `self.PlayerRef` _returnvalue)
  (bind _returnvalue_2 (`|CreateWidget` "/Game/Characters/PlayerCharacter/HUD/WBP_InventoryWarningText.WBP_InventoryWarningText_C"))
  (bind _output_get (set `self.InvWarningWidget` _returnvalue_2))
  (`UserWidget.AddToViewport` _output_get 0)
  (`Widget.SetVisibility` _output_get "Hidden"))

(event `ShowWarning`
  (bind _invwarningwidget (`self.InvWarningWidget`))
  (set `Widget.Visibility` "Visible" _invwarningwidget)
  (`KismetSystemLibrary.Delay` 3.0)
  (set `Widget.Visibility` "Hidden" _invwarningwidget)
  (`/Game/Characters/PlayerCharacter/HUD/WBP_InventoryWarningText.SetText` _invwarningwidget ""))

(fn `Add Item To Hotbar`
  (params (SelectedItem :type "/Game/NewInventory/S_ItemData Structure"))
  (locals (LocalIndex :type Integer))
  (bind (_itemobject _runtimestate _quantity) (break `/Game/NewInventory/S_ItemData` SelectedItem))
  (bind _returnvalue (`KismetArrayLibrary.Array_Find` (`self.Items`) SelectedItem))
  (if (> _returnvalue -1)
    (set `local.LocalIndex` _returnvalue)
    (bind _asbp_tool_object (cast `/Game/Items/ItemObjects/Tool/BP_ToolObject` _itemobject))
    (if (not (`/Game/Items/ItemObjects/Tool/BP_ToolObject.IsInHotbar` _asbp_tool_object))
      (bind (_canadditem _freeindex) (`self.Can Add Item to Hotbar`))
      (if _canadditem
        (set `/Game/Items/ItemObjects/Tool/BP_ToolObject.IsInHotbar` true _asbp_tool_object)
        (`KismetArrayLibrary.Array_Set` (`self.HotbarItems`) _freeindex (make `/Game/NewInventory/S_ItemData` _asbp_tool_object (struct) _quantity))
        (`self.OnHotbarChanged`)
        (`KismetArrayLibrary.Array_Set` (`self.Items`) (`local.LocalIndex`) (make `/Game/NewInventory/S_ItemData` _asbp_tool_object (struct) _quantity))
        (`self.OnInventoryChanged`)
        (return)
        (else
          (`self.SetWarningText` (`self.HotbarFullText`))
          (return))))))

(fn `AddItemToInventory`
  (params (NewItem :type "/Game/NewInventory/S_ItemData Structure"))
  (returns (ItemAddedSuccessfully :type Boolean))
  (locals (LocalNewItem :type "/Game/NewInventory/S_ItemData Structure") (LocalIndex :type Integer))
  (bind (_itemobject _runtimestate _quantity) (break `/Game/NewInventory/S_ItemData` (`local.LocalNewItem`)))
  (bind _itemtype (`/Game/Items/ItemObjects/BP_ItemObject.ItemType` (`.ItemObject_49_5E96F30A488B4287D92F9A9E36D555D4` (break `/Game/NewInventory/S_ItemData` NewItem))))
  ;[1 1 1] Player can carry only one tool of the same type.
  (set `local.LocalNewItem` NewItem)
  (if (or (`|EnumEquality` _itemtype "NewEnumerator1") (`|EnumEquality` _itemtype "NewEnumerator3"))
    (bind _containsitem (`self.ContainsItem` (`local.LocalNewItem`)))
    (if _containsitem
      (`self.SetWarningText` (`self.CantHoldMoreText`))
      (return false)
      (else
        _)))
  (for (_array_element _array_index) (`self.Items`)
    (set `local.LocalIndex` _array_index)
    (bind (_itemobject_2 _runtimestate_2 _quantity_2) (break `/Game/NewInventory/S_ItemData` _array_element))
    (if (`KismetSystemLibrary.IsValid` _itemobject_2)
      (if (and (`/Game/Items/ItemObjects/BP_ItemObject.Stackable` _itemobject_2) (== (`/Game/Items/ItemObjects/BP_ItemObject.ID` _itemobject_2) (`/Game/Items/ItemObjects/BP_ItemObject.ID` _itemobject)))
        (bind _returnvalue (+ _quantity_2 _quantity))
        (if (<= _returnvalue (`/Game/Items/ItemObjects/BP_ItemObject.StackSize` _itemobject_2))
          (`KismetArrayLibrary.Array_Set` (`self.Items`) (`local.LocalIndex`) (make `/Game/NewInventory/S_ItemData` _itemobject_2 (struct) _returnvalue))
          (`self.OnInventoryChanged`)
          (return true)
          (else
            (`self.SetWarningText` (`self.CantHoldMoreText`))
            (return false))))))
  (if (`self.IsInventoryFull`)
    (`self.SetWarningText` (`self.InventoryFullText`))
    (return false)
    (else
      (bind _emptyindex (`self.FindFirstEmptyIndex`))
      (if (> _emptyindex -1)
        (`KismetArrayLibrary.Array_Set` (`self.Items`) _emptyindex (`local.LocalNewItem`))
        (`self.OnInventoryChanged`)
        (return true)))))

(fn `Can Add Item to Hotbar`
  (returns (CanAddItem :type Boolean) (FreeIndex :type Integer))
  (for (_array_element _array_index) (`self.HotbarItems`)
    (`/Engine/EditorBlueprintResources/StandardMacros.IsValid` (`.ItemObject_49_5E96F30A488B4287D92F9A9E36D555D4` (break `/Game/NewInventory/S_ItemData` _array_element))
      (:`Is Not Valid`
        (return true _array_index))))
  (return false -1))

(fn `ContainsItem`
  (params (NewItem :type "/Game/NewInventory/S_ItemData Structure"))
  (returns (ContainsItem :type Boolean))
  (for _array_element (`self.Items`)
    (bind _itemobject (break `/Game/NewInventory/S_ItemData` _array_element))
    (`/Engine/EditorBlueprintResources/StandardMacros.IsValid` _itemobject
      (:`Is Valid`
        (if (== (`/Game/Items/ItemObjects/BP_ItemObject.ID` _itemobject) (`/Game/Items/ItemObjects/BP_ItemObject.ID` (`.ItemObject_49_5E96F30A488B4287D92F9A9E36D555D4` (break `/Game/NewInventory/S_ItemData` NewItem))))
          (return true)))))
  (return false))

(fn `ContainsItemWithAtLeastQuantity`
  (params (Item :type "/Game/NewInventory/S_ItemData Structure") (Quantity :type Integer))
  (returns (ContainsItem :type Boolean))
  (for _array_element (`self.Items`)
    (bind (_itemobject _runtimestate _quantity) (break `/Game/NewInventory/S_ItemData` _array_element))
    (`/Engine/EditorBlueprintResources/StandardMacros.IsValid` _itemobject
      (:`Is Valid`
        (if (== (`/Game/Items/ItemObjects/BP_ItemObject.ID` _itemobject) (`/Game/Items/ItemObjects/BP_ItemObject.ID` (`.ItemObject_49_5E96F30A488B4287D92F9A9E36D555D4` (break `/Game/NewInventory/S_ItemData` Item))))
          (if (>= _quantity Quantity)
            (return true)
            (else
              (return false)))))))
  (return false))

(fn `DeleteItemFromHotbar`
  (params (SelectedItem :type "/Game/NewInventory/S_ItemData Structure"))
  (locals (CachedIndex :type Integer :default 0))
  (bind (_itemobject _runtimestate _quantity) (break `/Game/NewInventory/S_ItemData` SelectedItem))
  (bind _hotbaritems (`self.HotbarItems`))
  (bind _playerref (`self.PlayerRef`))
  (bind _returnvalue (`KismetArrayLibrary.Array_Find` _hotbaritems SelectedItem))
  (bind _returnvalue_2 (`KismetArrayLibrary.Array_Find` (`self.Items`) SelectedItem))
  (bind _asbp_tool_object (cast `/Game/Items/ItemObjects/Tool/BP_ToolObject` _itemobject))
  (if (`/Game/Items/ItemObjects/Tool/BP_ToolObject.IsInHotbar` _asbp_tool_object)
    (if (and (>= _returnvalue 0) (>= _returnvalue_2 0))
      (set `local.CachedIndex` _returnvalue)
      (set `/Game/Items/ItemObjects/Tool/BP_ToolObject.IsInHotbar` false _asbp_tool_object)
      (`KismetArrayLibrary.Array_Set` _hotbaritems _returnvalue)
      (`self.OnHotbarChanged`)
      (`KismetArrayLibrary.Array_Set` (`self.Items`) _returnvalue_2 (make `/Game/NewInventory/S_ItemData` _asbp_tool_object (struct) _quantity))
      (`self.OnInventoryChanged`)
      (if (== (`local.CachedIndex`) (`/Game/Characters/PlayerCharacter/BP_PlayerCharacter.CurrentHotbarIndex` _playerref))
        (`/Game/Characters/PlayerCharacter/BP_PlayerCharacter.DestroyEquippedItem` _playerref)))))

(fn `DeleteItemFromInventory`
  (params (ItemToDelete :type "/Game/NewInventory/S_ItemData Structure"))
  (locals (LocalIndex :type Integer :default 0))
  (for (_array_element _array_index) (`self.Items`)
    (if (== (`/Game/Items/ItemObjects/BP_ItemObject.ID` (`.ItemObject_49_5E96F30A488B4287D92F9A9E36D555D4` (break `/Game/NewInventory/S_ItemData` _array_element))) (`/Game/Items/ItemObjects/BP_ItemObject.ID` (`.ItemObject_49_5E96F30A488B4287D92F9A9E36D555D4` (break `/Game/NewInventory/S_ItemData` ItemToDelete))))
      (bind _output_get (set `local.LocalIndex` _array_index))
      (bind _output (`|GetArrayItem` (`self.Items`) _output_get))
      (if (`|EnumEquality` (`/Game/Items/ItemObjects/BP_ItemObject.ItemType` (`.ItemObject_49_5E96F30A488B4287D92F9A9E36D555D4` (break `/Game/NewInventory/S_ItemData` _output))) "NewEnumerator1")
        (`self.DeleteItemFromHotbar` _output))
      (bind (_itemobject _runtimestate _quantity) (break `/Game/NewInventory/S_ItemData` _output))
      (if (> _quantity 1)
        (`KismetArrayLibrary.Array_Set` (`self.Items`) (`local.LocalIndex`) (make `/Game/NewInventory/S_ItemData` _itemobject _runtimestate (- _quantity 1)))
        (else
          (`KismetArrayLibrary.Array_Set` (`self.Items`) (`local.LocalIndex`))
          (set `/Game/NewInventory/WBP_Inventory.SelectedItem` (struct) (`/Game/Characters/PlayerCharacter/BP_PlayerCharacter.InventoryWidget` (`self.PlayerRef`)))))
      (`self.OnInventoryChanged`)
      (return))))

(fn `DropItem`
  (params (SelectedItem :type "/Game/NewInventory/S_ItemData Structure"))
  (locals (CachedIndex :type Integer :default 0))
  (bind (_itemobject _runtimestate) (break `/Game/NewInventory/S_ItemData` SelectedItem))
  (bind _playerref (`self.PlayerRef`))
  (bind _returnvalue (`|SpawnActorFromClass` (`/Game/Items/ItemObjects/BP_ItemObject.WorldActor` _itemobject) (`KismetMathLibrary.MakeTransform` (+ (`Actor.K2_GetActorLocation` _playerref) (* (`KismetMathLibrary.GetForwardVector` (`Actor.K2_GetActorRotation` _playerref)) 120.0))) "Undefined" "MultiplyWithRoot" null null))
  (bind _asbp_water_actor (cast `/Game/Items/ItemActors/Water/BP_WaterActor` _returnvalue)
    (:`then`
      (set `/Game/Items/ItemActors/Water/BP_WaterActor_WaterBottle.RuntimeState` _runtimestate _asbp_water_actor))
    (:`CastFailed`
      _))
  (set `/Game/Items/ItemActors/BP_ItemActor.ClassRef` (`GameplayStatics.GetObjectClass` _itemobject) _returnvalue)
  (`self.DeleteItemFromInventory` SelectedItem))

(fn `FindFirstEmptyIndex`
  (returns (EmptyIndex :type Integer))
  (for (_array_element _array_index) (`self.Items`)
    (if (not (`KismetSystemLibrary.IsValid` (`.ItemObject_49_5E96F30A488B4287D92F9A9E36D555D4` (break `/Game/NewInventory/S_ItemData` _array_element))))
      (return _array_index)))
  (return -1))

(fn `GetItemCount`
  (params (ItemClass :type "/Game/Items/ItemObjects/BP_ItemObject Class Reference"))
  (returns (ItemCount :type Integer))
  (for _array_element (`self.Items`)
    (bind (_itemobject _runtimestate _quantity) (break `/Game/NewInventory/S_ItemData` _array_element))
    (if (== ItemClass (`GameplayStatics.GetObjectClass` _itemobject))
      (return _quantity)))
  (return 0))

(fn `IsInventoryEmpty`
  (returns (IsEmpty :type Boolean))
  (for _array_element (`self.Items`)
    (`/Engine/EditorBlueprintResources/StandardMacros.IsValid` (`.ItemObject_49_5E96F30A488B4287D92F9A9E36D555D4` (break `/Game/NewInventory/S_ItemData` _array_element))
      (:`Is Valid`
        (return false))))
  (return true))

(fn `IsInventoryFull`
  (returns (IsInenvotryFull :type Boolean))
  (for _array_element (`self.Items`)
    (if (not (`KismetSystemLibrary.IsValid` (`.ItemObject_49_5E96F30A488B4287D92F9A9E36D555D4` (break `/Game/NewInventory/S_ItemData` _array_element))))
      (return false)))
  (return true))

(fn `RemoveItemByClass`
  (params (ItemClass :type "/Game/Items/ItemObjects/BP_ItemObject Class Reference") (Amount :type Integer))
  (for (_array_element _array_index) (`self.Items`)
    (bind (_itemobject _runtimestate _quantity) (break `/Game/NewInventory/S_ItemData` _array_element))
    (if (== ItemClass (`GameplayStatics.GetObjectClass` _itemobject))
      (bind _returnvalue (- _quantity Amount))
      (if (> _returnvalue 0)
        (`KismetArrayLibrary.Array_Set` (`self.Items`) _array_index (make `/Game/NewInventory/S_ItemData` _itemobject _runtimestate _returnvalue))
        (else
          (`KismetArrayLibrary.Array_Set` (`self.Items`) _array_index)
          (set `/Game/NewInventory/WBP_Inventory.SelectedItem` (struct) (`/Game/Characters/PlayerCharacter/BP_PlayerCharacter.InventoryWidget` (`self.PlayerRef`)))))
      (`self.OnInventoryChanged`))))

(fn `SetInventoryItem`
  (params (OldItem :type "/Game/NewInventory/S_ItemData Structure") (NewItem :type "/Game/NewInventory/S_ItemData Structure"))
  (bind _items (`self.Items`))
  (`KismetArrayLibrary.Array_Set` _items (`KismetArrayLibrary.Array_Find` _items OldItem) NewItem)
  (`self.OnInventoryChanged`))

(fn `SetWarningText`
  (params (Text :type Text))
  (`/Game/Characters/PlayerCharacter/HUD/WBP_InventoryWarningText.SetText` (`self.InvWarningWidget`) Text)
  (`self.ShowWarning`))

(fn `UseItem`
  (params (SelectedItem :type "/Game/NewInventory/S_ItemData Structure"))
  (locals (CachedIndex :type Integer :default 0))
  (`/Game/Items/ItemObjects/BP_ItemObject.UseItem` (`.ItemObject_49_5E96F30A488B4287D92F9A9E36D555D4` (break `/Game/NewInventory/S_ItemData` SelectedItem)) SelectedItem (`self.PlayerRef`) self))