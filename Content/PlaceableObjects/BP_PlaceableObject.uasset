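; BP_PlaceableObject is a placeable object that can briefly show an on-screen info widget.
; On BeginPlay it prints a debug greeting, creates its own WBP_ObjectInfo, adds it to the viewport and hides it.
; ShowMessage reveals the widget for a few seconds, then hides it and clears its text; nothing in this Blueprint sets the message content.
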(event `self.ReceiveBeginPlay`
  (`KismetSystemLibrary.PrintString` "Hello")
  (bind _returnvalue (`|CreateWidget` "/Game/Characters/PlayerCharacter/HUD/WBP_ObjectInfo.WBP_ObjectInfo_C"))
  (bind _output_get (set `self.ObjectInfoWidget` _returnvalue))
  (`UserWidget.AddToViewport` _output_get 0)
  (set `Widget.Visibility` "Hidden" _output_get))

(event `ShowMessage`
  (bind _objectinfowidget (`self.ObjectInfoWidget`))
  (set `Widget.Visibility` "Visible" _objectinfowidget)
  (`KismetSystemLibrary.Delay` 3.0)
  (set `Widget.Visibility` "Hidden" _objectinfowidget)
  (`/Game/Characters/PlayerCharacter/HUD/WBP_ObjectInfo.SetText` _objectinfowidget ""))

(fn `UserConstructionScript`)