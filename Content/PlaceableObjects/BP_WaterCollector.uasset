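; Placeable water collector that slowly accumulates water for players to top up their water bottles.
; A self-retriggering Refil event, started at BeginPlay, adds a unit on a fixed delay up to the maximum supply.
; UseWaterCollector finds a BP_Water inventory item, moves the inventory's UsedWater amount into it and broadcasts the inventory change.
; An info widget message reports insufficient supply or a missing bottle.
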(event `self.ReceiveBeginPlay`
  (`parent.ReceiveBeginPlay`)
  (`self.Refil`))

(event `Refil`
  (set `self.WaterSupply` (`KismetMathLibrary.Clamp` (+ (`self.WaterSupply`) 1) 0 (`self.MaxWaterSupply`)))
  (`KismetSystemLibrary.Delay` 3.0)
  (`self.Refil`))

(fn `UserConstructionScript`
  (`parent.UserConstructionScript`))

(fn `UseWaterCollector`
  (params (PlayerRef :type "/Game/Characters/PlayerCharacter/BP_PlayerCharacter Object Reference"))
  (locals (CachedIndex :type Integer))
  (bind _output_get (set `self.Player Ref` PlayerRef))
  (bind _bpc_inventory (`/Game/Characters/PlayerCharacter/BP_PlayerCharacter.BPC_Inventory` _output_get))
  (for (_array_element _array_index) (`/Game/NewInventory/BPC_Inventory.Items` _bpc_inventory)
    (set `local.CachedIndex` _array_index)
    (bind (_itemclass _quantity) (break `/Game/NewInventory/S_ItemData` _array_element))
    (`/Engine/EditorBlueprintResources/StandardMacros.IsValid` _itemclass
      (:`Is Valid`
        (bind _asbp_water (cast `/Game/Items/ItemBP/Water/BP_Water` _itemclass))
        (if (> (`self.WaterSupply`) (`/Game/NewInventory/BPC_Inventory.UsedWater` _bpc_inventory))
          (set `/Game/Items/ItemBP/Water/BP_Water.WaterSupply` (`KismetMathLibrary.Clamp` (+ (`/Game/NewInventory/BPC_Inventory.UsedWater` (`/Game/Characters/PlayerCharacter/BP_PlayerCharacter.BPC_Inventory` (`self.Player Ref`))) (`/Game/Items/ItemBP/Water/BP_Water.WaterSupply` _asbp_water)) 0 100) _asbp_water)
          (`KismetArrayLibrary.Array_Set` (`/Game/NewInventory/BPC_Inventory.Items` (`/Game/Characters/PlayerCharacter/BP_PlayerCharacter.BPC_Inventory` (`self.Player Ref`))) (`local.CachedIndex`) (make `/Game/NewInventory/S_ItemData` _asbp_water _quantity))
          (set `self.WaterSupply` (- (`self.WaterSupply`) (`/Game/NewInventory/BPC_Inventory.UsedWater` (`/Game/Characters/PlayerCharacter/BP_PlayerCharacter.BPC_Inventory` (`self.Player Ref`)))))
          (`/Game/NewInventory/BPC_Inventory.OnInventoryChanged` (`/Game/Characters/PlayerCharacter/BP_PlayerCharacter.BPC_Inventory` (`self.Player Ref`)))
          (return)
          (else
            (`/Game/Characters/PlayerCharacter/HUD/WBP_ObjectInfo.SetText` (`self.ObjectInfoWidget`) (`KismetTextLibrary.Conv_StringToText` (`KismetStringLibrary.Concat_StrStr` (`self.NotEnoughWaterString`) (`KismetStringLibrary.Concat_StrStr` "(" (`KismetStringLibrary.Conv_IntToString` (`self.WaterSupply`)) "/" (`KismetStringLibrary.Conv_IntToString` (`self.MaxWaterSupply`)) ")"))))
            (`self.ShowMessage`)
            (return))))))
  (`/Game/Characters/PlayerCharacter/HUD/WBP_ObjectInfo.SetText` (`self.ObjectInfoWidget`) "You do not own a water bottle")
  (`self.ShowMessage`))