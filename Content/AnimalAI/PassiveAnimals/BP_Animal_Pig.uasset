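; BP_Animal_Pig is the pig variant of the passive animal AI, adding a pig-specific hit sound on top of its parent class.
; Its ReceiveDamage override passes damage to the parent, then, if the pig is still valid, plays Pig_hit at its location.
; The construction script only calls the parent, and the event graph holds only disabled placeholder events.
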(fn `ReceiveDamage`
  (params (DamagePoints :type "Float (double-precision)") (DamageCauser :type "Actor Object Reference"))
  (`parent.ReceiveDamage` DamagePoints DamageCauser)
  (`/Engine/EditorBlueprintResources/StandardMacros.IsValid` self
    (:`Is Valid`
      (`GameplayStatics.PlaySoundAtLocation` "/Game/3rdPartyAssets/Sounds/Sounds/pig_hit.pig_hit" (`self.K2_GetActorLocation`) (struct) 1.0 1.0 0.0 null null null null))))

(fn `UserConstructionScript`
  (`parent.UserConstructionScript`))