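; BP_Animal_Aggressive is an animal AI Blueprint that can attack players and passive animals and flag players as chased.
; AttackOtherActor sets the animal state, then applies AttackDamage through ReceiveDamage, passing itself as the damage causer only for passive animals.
; StartChasingActor and StopChasingActor toggle IsBeingChased on the player character and ignore other actors.
; Its event graph has no active logic, so these functions rely on outside callers.
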(event `self.ReceiveTick`
  (params (DeltaSeconds :type "Float (single-precision)")))

(fn `AttackOtherActor`
  (params (OtherActor :type "Actor Object Reference"))
  (`self.SetAnimalState` "NewEnumerator5")
  (bind _asbp_player_character (cast `/Game/PlayerCharacter/BP_PlayerCharacter` OtherActor)
    (:`then`
      (`/Game/PlayerCharacter/BP_PlayerCharacter.ReceiveDamage` _asbp_player_character (`self.AttackDamage`)))
    (:`CastFailed`
      (bind _asbp_animal_passive (cast `/Game/AnimalAI/PassiveAnimals/BP_Animal_Passive` OtherActor))
      (`self.ReceiveDamage` _asbp_animal_passive (`self.AttackDamage`) self))))

(fn `StartChasingActor`
  (params (ChasedActor :type "Actor Object Reference"))
  (bind _asbp_player_character (cast `/Game/PlayerCharacter/BP_PlayerCharacter` ChasedActor))
  (set `/Game/PlayerCharacter/BP_PlayerCharacter.IsBeingChased` true _asbp_player_character))

(fn `StopChasingActor`
  (params (ChasedActor :type "Actor Object Reference"))
  (bind _asbp_player_character (cast `/Game/PlayerCharacter/BP_PlayerCharacter` ChasedActor))
  (set `/Game/PlayerCharacter/BP_PlayerCharacter.IsBeingChased` false _asbp_player_character))

(fn `UserConstructionScript`
  (`parent.UserConstructionScript`))