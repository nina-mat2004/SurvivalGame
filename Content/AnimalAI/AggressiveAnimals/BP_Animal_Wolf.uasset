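; BP_Animal_Wolf is an aggressive AI animal that layers wolf animation and audio onto inherited chase and attack behavior.
; Its overrides call the parent first, then the attack plays a montage and an attenuated sound at the wolf's location.
; Starting a chase plays the AudioComponent and prints a debug string, and stopping the chase stops that audio.
; The event graph and construction script add no logic of their own.
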(fn `AttackOtherActor`
  (params (OtherActor :type "Actor Object Reference"))
  (`parent.AttackOtherActor` OtherActor)
  (`self.PlayAnimMontage` "/Game/AnimalAI/AggressiveAnimals/Animations/AM_WolfAttack.AM_WolfAttack")
  (`GameplayStatics.PlaySoundAtLocation` "/Game/Sounds/SoundCues/wolf_attack.wolf_attack" (`self.K2_GetActorLocation`) (struct) 1.0 1.0 0.0 "/Game/Sounds/WolfChasingAttenuation.WolfChasingAttenuation" null null null))

(fn `StartChasingPlayer`
  (params (ChasedActor :type "Actor Object Reference"))
  (`parent.StartChasingPlayer` ChasedActor)
  (`AudioComponent.Play` (`self.AudioComponent`) 0.0)
  (`KismetSystemLibrary.PrintString` "CHASING OTHER ACTOR"))

(fn `StopChasingPlayer`
  (params (ChasedActor :type "Actor Object Reference"))
  (`parent.StopChasingPlayer` ChasedActor)
  (`AudioComponent.Stop` (`self.AudioComponent`)))

(fn `UserConstructionScript`
  (`parent.UserConstructionScript`))