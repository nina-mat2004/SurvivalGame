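; BP_AnimalAIController is the AI controller for animal pawns derived from BP_AnimalBase.
; On possess it runs the behavior tree defined on the animal and records the spawn location as its home location.
; When AI perception senses an actor, it stores it as the threat actor and lets the animal update its state in response; lost-sight updates are ignored.
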(event `self.ReceivePossess`
  (params (PossessedPawn :type "Pawn Object Reference"))
  (bind _asbp_animal_base (cast `/Game/AnimalAI/Base/BP_AnimalBase` PossessedPawn))
  (`self.RunBehaviorTree` (`/Game/AnimalAI/Base/BP_AnimalBase.BehaviorTree` _asbp_animal_base))
  (`/Game/AnimalAI/AI/BFL_AIHelpers.SetHomeLocation` self (`self.K2_GetActorLocation` (`self.K2_GetPawn`))))

(event `self.AIPerception.OnTargetPerceptionUpdated`
  (params (Actor :type "Actor Object Reference") (Stimulus :type "AIStimulus Structure"))
  (if (`.bSuccessfullySensed` (break `AIStimulus` Stimulus))
    (`/Game/AnimalAI/AI/BFL_AIHelpers.SetThreatActor` self Actor)
    (bind _asbp_animal_base (cast `/Game/AnimalAI/Base/BP_AnimalBase` (`self.K2_GetPawn`)))
    (`/Game/AnimalAI/Base/BP_AnimalBase.SetAnimalStateAfterSeeingActor` _asbp_animal_base Actor)))

(fn `UserConstructionScript`)