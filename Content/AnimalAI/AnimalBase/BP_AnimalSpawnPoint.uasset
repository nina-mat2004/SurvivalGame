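; Spawn point actor that spawns one animal of a set class at its location and persists it through save games.
; On BeginPlay it restores its entry from the current save, matched by an ID defaulting to the object name, or spawns fresh without one.
; When the animal is destroyed, it retries spawning after a delay with a random chance, if respawning is allowed.
; Save data nests the spawned animal's own data.
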(event `self.ReceiveBeginPlay`
  (bind _asbp_game_instance (cast `/Game/Saving/BP_GameInstance` (`GameplayStatics.GetGameInstance`)))
  (bind _currentsave (`/Game/Saving/BP_GameInstance.CurrentSave` _asbp_game_instance))
  (`/Engine/EditorBlueprintResources/StandardMacros.IsValid` _currentsave
    (:`Is Valid`
      (for _array_element (`/Game/Saving/BP_SaveGame.AnimalSpawnpoints` _currentsave)
        (if (`KismetStringLibrary.EqualEqual_StrStr` (`self.ID`) (`.ID_7_D0EFB0DA48F375C1006B028E4A8C2924` (break `/Game/Saving/SavingStructures/S_AnimalSpawnpointData` _array_element)))
          (`self.ApplySaveData` _array_element)))
      (`self.StartRespawnTimer`))
    (:`Is Not Valid`
      (if (`KismetSystemLibrary.IsValidClass` (`self.AnimalClass`))
        (`self.TrySpawnAnimal`)))))

(event `StartRespawnTimer`
  (`KismetSystemLibrary.Delay` (`self.RespawnDelay`))
  (`self.AttemptRespawn`))

(fn `ApplySaveData`
  (params (SaveData :type "/Game/Saving/SavingStructures/S_AnimalSpawnpointData Structure"))
  (bind (_id _hasanimalspawned _animaldata) (break `/Game/Saving/SavingStructures/S_AnimalSpawnpointData` SaveData))
  (bind _spawnedanimal (`self.SpawnedAnimal`))
  (if _hasanimalspawned
    (`self.TrySpawnAnimal`)
    (`/Engine/EditorBlueprintResources/StandardMacros.IsValid` _spawnedanimal
      (:`Is Valid`
        (`/Game/AnimalAI/AnimalBase/BP_AnimalBase.ApplySaveData` _spawnedanimal _animaldata))
      (:`Is Not Valid`
        (`self.StartRespawnTimer` :!label _label)))
    (else
      (goto _label))))

(fn `AttemptRespawn`
  (`/Engine/EditorBlueprintResources/StandardMacros.IsValid` (`self.SpawnedAnimal`)
    (:`Is Not Valid`
      (if (<= (`KismetMathLibrary.RandomFloatInRange` 0.0 1.0) (`self.RespawnChance`))
        (`self.TrySpawnAnimal`)
        (else
          (`self.StartRespawnTimer`))))))

(fn `GetSaveData`
  (returns (SaveData :type "/Game/Saving/SavingStructures/S_AnimalSpawnpointData Structure"))
  (bind _spawnedanimal (`self.SpawnedAnimal`))
  (`/Engine/EditorBlueprintResources/StandardMacros.IsValid` _spawnedanimal
    (:`Is Valid`
      (return (make `/Game/Saving/SavingStructures/S_AnimalSpawnpointData` (`self.ID`) true (`/Game/AnimalAI/AnimalBase/BP_AnimalBase.GetSaveData` _spawnedanimal))))
    (:`Is Not Valid`
      (return (make `/Game/Saving/SavingStructures/S_AnimalSpawnpointData` (`self.ID`))))))

(fn `OnSpawnedAnimalDestroyed`
  (params (DestroyedActor :type "Actor Object Reference"))
  (set `self.SpawnedAnimal` null)
  (if (`self.CanRespawn`)
    (`self.StartRespawnTimer`)))

(fn `TrySpawnAnimal`
  (`/Engine/EditorBlueprintResources/StandardMacros.IsValid` (`self.SpawnedAnimal`)
    (:`Is Not Valid`
      (bind _returnvalue (`|SpawnActorFromClass` (`self.AnimalClass`) (`KismetMathLibrary.MakeTransform` (`self.K2_GetActorLocation`)) "Undefined" "MultiplyWithRoot" null null))
      (`/Engine/EditorBlueprintResources/StandardMacros.IsValid` _returnvalue
        (:`Is Valid`
          (bind _output_get (set `self.SpawnedAnimal` _returnvalue))
          (add `self.OnDestroyed` _output_get (`|CreateDelegate` :!event `OnSpawnedAnimalDestroyed`)))))))

(fn `UserConstructionScript`
  (if (`KismetStringLibrary.IsEmpty` (`self.ID`))
    (set `self.ID` (`KismetSystemLibrary.GetObjectName` self))))