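; Base animal actor for AI wildlife, handling health, behavior state, death, loot and save data.
; SetAnimalState switches walk or run speed and disables movement on death, while SetAnimalStateAfterSeeingActor is an empty hook.
; Damage passes the attacker to the AI controller as a threat or triggers death, which spawns physics pickups, notifies the player's QuestManager and destroys the actor after a delay.
; Save data restores fields directly, bypassing SetAnimalState.
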(event `self.ReceiveBeginPlay`
  (`self.InitializeAnimal`)
  (bind _returnvalue (`GameplayStatics.GetActorOfClass` "/Game/PlayerCharacter/BP_PlayerCharacter.BP_PlayerCharacter_C"))
  (set `self.PlayerRef` _returnvalue))

(event `Die`
  (set `self.IsDead` true)
  (`self.SetAnimalState` "NewEnumerator7")
  (`self.DropLoot`)
  (`/Game/Quests/BP_QuestManager.OnQuestCompleted` (`/Game/PlayerCharacter/BP_PlayerCharacter.QuestManager` (`self.PlayerRef`)) "KillAnimal")
  (`KismetSystemLibrary.Delay` 3.0)
  (`self.K2_DestroyActor`))

(fn `ApplySaveData`
  (params (SaveData :type "/Game/Saving/SavingStructures/S_AnimalData Structure"))
  (bind (_currentstate _animallocation _animalrotation _health _isdead _homelocation) (break `/Game/Saving/SavingStructures/S_AnimalData` SaveData))
  (set `self.CurrentState` _currentstate)
  (set `self.Health` _health)
  (set `self.IsDead` _isdead)
  (set `self.HomeLocation` _homelocation)
  (`self.K2_SetActorLocation` _animallocation))

(fn `CanDropLoot`
  (returns (CanDropLoot :type Boolean))
  (return (and (`self.DropLootOnDeath`) (`KismetSystemLibrary.IsValidClass` (`self.LootClass`)) (`self.IsDead`))))

(fn `DropLoot`
  (bind _lootclass (`self.LootClass`))
  (bind (_id _displayname _description _itemtype _stackable _stacksize _staticmesh _staticmeshtransform) (defaults `Object` _lootclass))
  (if (`self.CanDropLoot`)
    (for _ (range (`self.LootCountMin`) (+ (`KismetMathLibrary.RandomIntegerInRange` (`self.LootCountMin`) (`self.LootCountMax`)) 1))
      (bind _returnvalue (`|SpawnActorFromClass` "/Game/Items/BP_PickableItemActor.BP_PickableItemActor_C" (`KismetMathLibrary.MakeTransform` (+ (`self.K2_GetActorLocation`) (`KismetMathLibrary.MakeVector` 0.0 0.0 (`KismetMathLibrary.RandomFloatInRange` 20.0 50.0)))) "Undefined" "MultiplyWithRoot" null false null))
      (set `/Game/Items/BP_PickableItemActor.ItemObjectClass` _lootclass _returnvalue)
      (bind _staticmesh_2 (`/Game/Items/BP_PickableItemActor.StaticMesh` _returnvalue))
      (`StaticMeshComponent.SetStaticMesh` _staticmesh_2 _staticmesh)
      (`SceneComponent.K2_SetRelativeTransform` _staticmesh_2 _staticmeshtransform false false)
      (`PrimitiveComponent.SetSimulatePhysics` _staticmesh_2 true))))

(fn `GetSaveData`
  (returns (SaveData :type "/Game/Saving/SavingStructures/S_AnimalData Structure"))
  (return (make `/Game/Saving/SavingStructures/S_AnimalData` (`self.CurrentState`) (`self.K2_GetActorLocation`) (`self.K2_GetActorRotation`) (`self.Health`) (`self.IsDead`) (`self.HomeLocation`))))

(fn `InitializeAnimal`
  (set `self.Health` (`self.MaxHealth`))
  (set `self.HomeLocation` (`self.K2_GetActorLocation`))
  (set `CharacterMovementComponent.MaxWalkSpeed` (`self.WalkSpeed`) (`self.CharacterMovement`))
  (set `self.IsDead` false)
  (`self.SetAnimalState` "NewEnumerator1"))

(fn `IsAlive`
  (returns (IsAlive :type Boolean))
  (return (not (`self.IsDead`))))

(fn `ReceiveDamage`
  (params (DamagePoints :type "Float (double-precision)") (DamageCauser :type "Actor Object Reference"))
  (if (not (`self.IsDead`))
    (bind _output_get (set `self.Health` (- (`self.Health`) DamagePoints)))
    (`KismetSystemLibrary.PrintString` (`KismetStringLibrary.Conv_DoubleToString` _output_get))
    (if (<= _output_get 0.0)
      (`self.Die`)
      (else
        (bind _asbp_animal_aicontroller (cast `/Game/AnimalAI/AI/BP_AnimalAIController` (`self.GetController`)))
        (`/Game/AnimalAI/AI/BFL_AIHelpers.SetThreatActor` _asbp_animal_aicontroller DamageCauser)))))

(fn `SetAnimalState`
  (params (NewState :type "/Game/AnimalAI/AnimalBase/E_AnimalState Enum" :default "NewEnumerator0"))
  (bind _output_get (set `self.CurrentState` NewState))
  (switch `/Game/AnimalAI/AnimalBase/E_AnimalState` _output_get
    (:`NewEnumerator0`
      (set `CharacterMovementComponent.MaxWalkSpeed` (`self.WalkSpeed`) (`self.CharacterMovement`) :!label _label))
    (:`NewEnumerator1`
      (goto _label))
    (:`NewEnumerator3`
      (set `CharacterMovementComponent.MaxWalkSpeed` (`self.RunSpeed`) (`self.CharacterMovement`) :!label _label_2))
    (:`NewEnumerator4`
      (goto _label_2))
    (:`NewEnumerator5`
      (goto _label_2))
    (:`NewEnumerator7`
      (`CharacterMovementComponent.DisableMovement` (`self.CharacterMovement`)))))

(fn `SetAnimalStateAfterSeeingActor`
  (params (SeenActor :type "Actor Object Reference")))

(fn `UserConstructionScript`)