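; Spawn point actor that keeps a single animal of a configurable class at its location, with optional respawning.
; On BeginPlay it spawns the animal if the class is valid and binds to the animal's destroyed event.
; When respawning is allowed, destruction starts a delay followed by a random chance roll.
; A failed roll restarts the delay, and validity checks prevent a second animal while one is alive.
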(event `self.ReceiveBeginPlay`
  (if (`KismetSystemLibrary.IsValidClass` (`self.AnimalClass`))
    (`self.TrySpawnAnimal`)))

(event `StartRespawnTimer`
  (`KismetSystemLibrary.Delay` (`self.RespawnDelay`))
  (`self.AttemptRespawn`))

(fn `AttemptRespawn`
  (`/Engine/EditorBlueprintResources/StandardMacros.IsValid` (`self.SpawnedAnimal`)
    (:`Is Not Valid`
      (if (<= (`KismetMathLibrary.RandomFloatInRange` 0.0 1.0) (`self.RespawnChance`))
        (`self.TrySpawnAnimal`)
        (else
          (`self.StartRespawnTimer`))))))

(fn `OnSpawnedAnimalDestroyed`
  (params (DestroyedActor :type "Actor Object Reference"))
  (set `self.SpawnedAnimal` null)
  (if (`self.CanRespawn`)
    (`self.StartRespawnTimer`)))

(fn `TrySpawnAnimal`
  (`/Engine/EditorBlueprintResources/StandardMacros.IsValid` (`self.SpawnedAnimal`)
    (:`Is Not Valid`
      (bind _returnvalue (`|SpawnActorFromClass` (`self.AnimalClass`) (`KismetMathLibrary.MakeTransform` (`self.K2_GetActorLocation`)) "Undefined" "MultiplyWithRoot" null null))
      (`/Engine/EditorBlueprintResources/StandardMacros.IsValid` _returnvalue
        (:`Is Valid`
          (bind _output_get (set `self.SpawnedAnimal` _returnvalue))
          (add `self.OnDestroyed` _output_get (`|CreateDelegate` :!event `OnSpawnedAnimalDestroyed`)))))))

(fn `UserConstructionScript`
  (`parent.UserConstructionScript`))