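; Quest manager that runs a linear chain of hardcoded survival objectives, from gathering sticks to contacting people.
; BeginPlay builds the quest array, caches the player character and broadcasts the first quest through OnQuestUpdated after a short delay.
; CompleteQuest accepts only the current quest's ID, then StartNextQuest advances the index under a hardcoded bound and rebroadcasts.
; Each completion also briefly shows completed and new objective text on the player's in-game screen widget.
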(event `self.ReceiveBeginPlay`
  (set `self.Quests` (`|MakeArray` (make `/Game/Quests/S_QuestData` "GatherSticks" "Gather Sticks" "Find and pick up sticks from  \nthe ground") (make `/Game/Quests/S_QuestData` "CraftTool" "Craft a tool" "Use collected material to craft  \nany type of tool") (make `/Game/Quests/S_QuestData` "UseWaterCollector" "Use water collector" "Find or craft a water collector and  \nuse it to get drinkable water") (make `/Game/Quests/S_QuestData` "SleepInBed" "Sleep in a bed" "Craft or find a bed and sleep in it") (make `/Game/Quests/S_QuestData` "KillAnimal" "Kill an animal" "Kill any type of animal") (make `/Game/Quests/S_QuestData` "ContactPeople" "Contact people" "Craft a Walkie Talkie and try to  \ncontact someone \nHint: There are electronic devices \nnear camps that can be destroyed \nfor parts") (make `/Game/Quests/S_QuestData` "End" "" "All Objectives finished")))
  (bind _asbp_player_character (cast `/Game/PlayerCharacter/BP_PlayerCharacter` (`GameplayStatics.GetPlayerCharacter` 0)))
  (set `self.PlayerRef` _asbp_player_character)
  (bind _output_get (set `self.CurrentQuest` (`|GetArrayItem` (`self.Quests`))))
  (`KismetSystemLibrary.Delay` 0.2)
  (`self.OnQuestUpdated` _output_get))

(event `ShowNewObjectiveMessage`
  (bind _ingamescreenwidget (`/Game/PlayerCharacter/BP_PlayerCharacter.InGameScreenWidget` (`self.PlayerRef`)))
  (bind _newobjtext (`/Game/PlayerCharacter/GUI/WBP_InGameScreen.NewObjText` _ingamescreenwidget))
  (bind _objcompletedtext (`/Game/PlayerCharacter/GUI/WBP_InGameScreen.ObjCompletedText` _ingamescreenwidget))
  (`/Game/PlayerCharacter/GUI/WBP_InGameScreen.SetNewObjectiveText` _ingamescreenwidget (`.Title_9_D7D8E80D4ADAC91F90CBDF8B30F0219F` (break `/Game/Quests/S_QuestData` (`self.CurrentQuest`))))
  (set `Widget.Visibility` "Visible" _newobjtext)
  (set `Widget.Visibility` "Visible" _objcompletedtext)
  (`KismetSystemLibrary.Delay` 6.5)
  (set `Widget.Visibility` "Hidden" _newobjtext)
  (set `Widget.Visibility` "Hidden" _objcompletedtext))

(fn `CompleteQuest`
  (params (QuestID :type Name))
  (bind (_id _title _description) (break `/Game/Quests/S_QuestData` (`self.CurrentQuest`)))
  (if (== QuestID _id)
    (set `self.CurrentQuest` (make `/Game/Quests/S_QuestData` _id _title _description true))
    (`self.StartNextQuest`)
    (`self.ShowNewObjectiveMessage`)))

(fn `SendNewQuestMessage`)

(fn `StartNextQuest`
  (bind _result (`/Engine/EditorBlueprintResources/StandardMacros.IncrementInt` (`self.CurrentQuestIndex`))
    (:`  `
      (if (< _result 6)
        (bind _output_get (set `self.CurrentQuest` (`|GetArrayItem` (`self.Quests`) _result)))
        (`self.OnQuestUpdated` _output_get)))))

(fn `UserConstructionScript`)