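; Player survival attribute component that tracks health, hunger, water, energy, dirtiness and breath, raising low-stat warnings on the in-game widget.
; Self-recalling Delay events drive the stats at rates shaped by player state, while a looping timer updates breath and its widget.
; Depleted hunger, water or breath feeds the health drain, which ends in player death or hands off to conditional regeneration.
; Helper functions apply pickups, mining cost, damage and sleep effects.
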(event `self.ReceiveBeginPlay`
  (bind _returnvalue (`GameplayStatics.GetActorOfClass` "/Game/PlayerCharacter/BP_PlayerCharacter.BP_PlayerCharacter_C"))
  (set `self.PlayerRef` _returnvalue)
  (`KismetSystemLibrary.Delay` 1.0)
  (`self.StartAttributes`)
  (`self.UpdateWarnings`))

(event `DecreaseWater`
  ;[0.2162 0.6734 1] Water
  (if (< (`self.Water`) (`self.WarningThreshold`))
    (`self.AddToWarningMessages` "Water"))
  (bind _output_get (set `self.Water` (`self.SubtractNewPoints` (`self.Water`) 1.0)))
  (if (< _output_get 0.0)
    (`self.DecreaseHealth`)
    (else
      (`KismetSystemLibrary.Delay` 10.0)
      (`self.DecreaseWater`))))

(event `DecreaseHunger`
  ;[0.274 0.1182 0.03514] Hunger
  (if (< (`self.Hunger`) (`self.WarningThreshold`))
    (`self.AddToWarningMessages` "Hunger"))
  (bind _output_get (set `self.Hunger` (`self.SubtractNewPoints` (`self.Hunger`) 1.0)))
  (if (<= _output_get 0.0)
    (`self.DecreaseHealth`)
    (else
      (if (`/Game/PlayerCharacter/BP_PlayerCharacter.IsSprinting` (`self.PlayerRef`))
        (`KismetSystemLibrary.Delay` 5.0)
        (else
          (`KismetSystemLibrary.Delay` 10.0)))
      (`self.DecreaseHunger`))))

(event `DecreaseHealth`
  ;[1 0.1307 0.5254] Health
  (if (< (`self.Health`) 30.0)
    (`self.AddToWarningMessages` "Health"))
  (bind _output_get (set `self.Health` (`self.SubtractNewPoints` (`self.Health`) 1.0)))
  (if (<= _output_get 0.0)
    (`/Game/PlayerCharacter/BP_PlayerCharacter.PlayerDiedEvent` (`self.PlayerRef`))
    (elif (or (<= (`self.Hunger`) 0.0) (`/Game/PlayerCharacter/BP_PlayerCharacter.IsOutsidePlayArea` (`self.PlayerRef`)))
      (`KismetSystemLibrary.Delay` 0.5)
      (`self.DecreaseHealth`)
      (else
        (`self.IncreaseHealth`)))))

(event `IncreaseHealth`
  ;[1 0.1307 0.5254] Health
  (if (and (> (`self.Hunger`) 0.0) (< (`self.Dirtiness`) (`self.DirtinessWarningTreshold`)) (not (`/Game/PlayerCharacter/BP_PlayerCharacter.IsOutsidePlayArea` (`self.PlayerRef`))))
    (set `self.Health` (`self.AddNewPoints` (`self.Health`) 1.0))
    (`KismetSystemLibrary.Delay` 2.0)
    (`self.IncreaseHealth`)))

(event `DecreaseEnergy`
  (bind _playerref (`self.PlayerRef`))
  ;[0.6749 1 0.5301] Evergy
  (if (< (`self.Energy`) (`self.WarningThreshold`))
    (`self.AddToWarningMessages` "Energy"))
  (set `self.Energy` (`self.SubtractNewPoints` (`self.Energy`) 1.0))
  (if (or (`/Game/PlayerCharacter/BP_PlayerCharacter.IsSwimming` _playerref) (`/Game/PlayerCharacter/BP_PlayerCharacter.IsSprinting` _playerref))
    (`KismetSystemLibrary.Delay` 5.0)
    (`self.DecreaseEnergy`)))

(event `IncreaseEnergy`
  (bind _playerref (`self.PlayerRef`))
  ;[0.6749 1 0.5301] Evergy
  (if (and (not (`/Game/PlayerCharacter/BP_PlayerCharacter.IsSprinting` _playerref)) (not (`/Game/PlayerCharacter/BP_PlayerCharacter.IsSwimming` _playerref)))
    (if (>= (`self.Energy`) (`self.WarningThreshold`))
      (`self.DeleteFromWarningMessages` "Energy"))
    (set `self.Energy` (`self.AddNewPoints` (`self.Energy`) 1.0))
    (`KismetSystemLibrary.Delay` 5.0)
    (`self.IncreaseEnergy`)))

(event `IncreaseDirt`
  ;[0.408 0.3636 1] Dirtiness
  (if (not (`/Game/PlayerCharacter/BP_PlayerCharacter.IsSwimming` (`self.PlayerRef`)))
    (if (>= (`self.Dirtiness`) (`self.DirtinessWarningTreshold`))
      (`self.AddToWarningMessages` "Dirty"))
    (set `self.Dirtiness` (`self.AddNewPoints` (`self.Dirtiness`) 1.0))
    (`KismetSystemLibrary.Delay` 10.0)
    (`self.IncreaseDirt`)))

(event `CleaningInWater`
  ;[0.408 0.3636 1] Dirtiness
  (if (`/Game/PlayerCharacter/BP_PlayerCharacter.IsSwimming` (`self.PlayerRef`))
    (`KismetSystemLibrary.Delay` 5.0)
    (if (`/Game/PlayerCharacter/BP_PlayerCharacter.IsSwimming` (`self.PlayerRef`))
      (set `self.Dirtiness` 0.0)
      (`self.DeleteFromWarningMessages` "Dirtiness")
      (`self.IncreaseHealth`))))

(event `StartBreathTimer`
  (`KismetSystemLibrary.K2_SetTimer` null "UpdateBreathOverTime" 1.0 true))

(fn `AddDirtinessPoints`
  (params (PointsToAdd :type "Float (double-precision)"))
  (bind _output_get (set `self.Dirtiness` (`self.AddNewPoints` (`self.Dirtiness`) PointsToAdd)))
  (if (> _output_get 70.0)
    (`self.AddToWarningMessages` "None")))

(fn `AddEnergyPoints`
  (params (PointsToAdd :type "Float (double-precision)"))
  (bind _output_get (set `self.Energy` (`self.AddNewPoints` (`self.Energy`) PointsToAdd)))
  (if (>= _output_get 30.0)
    (`self.DeleteFromWarningMessages` "Energy")))

(fn `AddHealthPoints`
  (params (PointsToAdd :type "Float (double-precision)"))
  (bind _output_get (set `self.Health` (`self.AddNewPoints` (`self.Health`) PointsToAdd)))
  (if (>= _output_get 30.0)
    (`self.DeleteFromWarningMessages` "Health")))

(fn `AddHungerPoints`
  (params (PointsToAdd :type "Float (double-precision)"))
  (bind _output_get (set `self.Hunger` (`self.AddNewPoints` (`self.Hunger`) PointsToAdd)))
  (if (>= _output_get 30.0)
    (`self.DeleteFromWarningMessages` "Hunger")))

(fn `AddNewPoints`
  (params (Points :type "Float (double-precision)") (NewPoints :type "Float (double-precision)"))
  (returns (ReturnPoints :type "Float (double-precision)"))
  (return (`KismetMathLibrary.FClamp` (+ Points NewPoints) 0.0 (`self.MaxAttributeValue`))))

(fn `AddToWarningMessages`
  (params (AttributeName :type Name))
  (`/Game/PlayerCharacter/GUI/WBP_InGameScreen.AddToActiveWarnings` (`/Game/PlayerCharacter/BP_PlayerCharacter.InGameScreenWidget` (`self.PlayerRef`)) AttributeName))

(fn `AddWaterPoints`
  (params (PointsToAdd :type "Float (double-precision)"))
  (bind _output_get (set `self.Water` (`self.AddNewPoints` (`self.Water`) PointsToAdd)))
  (if (>= _output_get 30.0)
    (`self.DeleteFromWarningMessages` "Water")))

(fn `CanSprint`
  (returns (CanSprint :type Boolean))
  (return (and (> (`self.Hunger`) 30.0) (> (`self.Energy`) 30.0))))

(fn `DecreaseEnergyAfterMining`
  (params (EnegryDecrease :type "Float (double-precision)"))
  (bind _output_get (set `self.Energy` (`self.SubtractNewPoints` (`self.Energy`) EnegryDecrease)))
  (if (< _output_get 30.0)
    (`self.AddToWarningMessages` "Energy")))

(fn `DeleteFromWarningMessages`
  (params (AttributeName :type Name))
  (`/Game/PlayerCharacter/GUI/WBP_InGameScreen.DeleteFromActiveWarnings` (`/Game/PlayerCharacter/BP_PlayerCharacter.InGameScreenWidget` (`self.PlayerRef`)) AttributeName))

(fn `ReceiveDamage`
  (params (DamagePoints :type "Float (double-precision)"))
  (bind _output_get (set `self.Health` (- (`self.Health`) DamagePoints)))
  (if (< _output_get 30.0)
    (`self.AddToWarningMessages` "Health")
    (if (< _output_get 0.0)
      (`KismetSystemLibrary.PrintString` "DIED"))))

(fn `SetAttributesAfterSleeping`
  (set `self.Hunger` (`KismetMathLibrary.FClamp` (- (`self.Hunger`) 50.0) 20.0 (`self.MaxAttributeValue`)))
  (set `self.Water` (`KismetMathLibrary.FClamp` (- (`self.Water`) 50.0) 20.0 (`self.MaxAttributeValue`)))
  (set `self.Energy` (`self.MaxAttributeValue`))
  (`self.UpdateWarnings`))

(fn `StartAttributes`
  (`self.DecreaseHunger`)
  (`self.IncreaseHealth`)
  (`self.DecreaseWater`)
  (`self.IncreaseEnergy`)
  (`self.StartBreathTimer`))

(fn `SubtractNewPoints`
  (params (Points :type "Float (double-precision)") (NewPoints :type "Float (double-precision)"))
  (returns (ReturnPoints :type "Float (double-precision)"))
  (return (`KismetMathLibrary.FClamp` (- Points NewPoints) 0.0 (`self.MaxAttributeValue`))))

(fn `UpdateBreathOverTime`
  (locals (Delta :type "Float (double-precision)" :default 1.0) (DrainRate :type "Float (double-precision)" :default 1.0) (RegenRate :type "Float (double-precision)" :default 3.0))
  (bind _maxbreath (`self.MaxBreath`))
  (if (`/Game/PlayerCharacter/BP_PlayerCharacter.IsUnderWater` (`self.PlayerRef`))
    (bind _output_get (set `self.Breath` (`KismetMathLibrary.FClamp` (- (`self.Breath`) (* (`local.Delta`) (`local.DrainRate`))) 0.0 (`self.MaxBreath`))))
    (`/Game/PlayerCharacter/GUI/WBP_Breath.Update Breath` (`/Game/PlayerCharacter/BP_PlayerCharacter.BreathUnderWaterWidget` (`self.PlayerRef`)) _output_get (`self.MaxBreath`))
    (if (== _output_get 0.0)
      (`self.DecreaseHealth`))
    (else
      (bind _output_get_2 (set `self.Breath` (`KismetMathLibrary.FClamp` (+ (`self.Breath`) (* (`local.Delta`) (`local.RegenRate`))) 0.0 (`self.MaxBreath`))))
      (`/Game/PlayerCharacter/GUI/WBP_Breath.Update Breath` (`/Game/PlayerCharacter/BP_PlayerCharacter.BreathUnderWaterWidget` (`self.PlayerRef`)) _output_get_2 _maxbreath)
      (if (== _output_get_2 _maxbreath)
        (`/Game/PlayerCharacter/BP_PlayerCharacter.HideBreathWidget` (`self.PlayerRef`))))))

(fn `UpdateWarnings`
  (if (< (`self.Health`) (`self.WarningThreshold`))
    (`self.AddToWarningMessages` "Health")
    (else
      (`self.DeleteFromWarningMessages` "Health")))
  (if (< (`self.Hunger`) (`self.WarningThreshold`))
    (`self.AddToWarningMessages` "Hunger")
    (else
      (`self.DeleteFromWarningMessages` "Hunger")))
  (if (< (`self.Water`) (`self.WarningThreshold`))
    (`self.AddToWarningMessages` "Water")
    (else
      (`self.DeleteFromWarningMessages` "Water")))
  (if (< (`self.Energy`) (`self.WarningThreshold`))
    (`self.AddToWarningMessages` "Energy")
    (else
      (`self.DeleteFromWarningMessages` "Energy")))
  (if (>= (`self.Dirtiness`) (`self.DirtinessWarningTreshold`))
    (`self.AddToWarningMessages` "Dirtiness")
    (else
      (`self.DeleteFromWarningMessages` "Dirtiness"))))