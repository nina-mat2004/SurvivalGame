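; Harvestable resource actor that loses health when hit with its designated tool class and breaks into pickable loot.
; ApplyHitDamage checks the tool, plays its swing timeline and subtracts that tool class's default damage, calling OnDestroy at zero health.
; OnDestroy destroys the actor, then spawns a random number of physics-simulated pickups configured from LootItem's class defaults.
; The player, cached on BeginPlay, loses energy for each spawned pickup.
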(event `self.ReceiveBeginPlay`
  (bind _asbp_player_character (cast `/Game/PlayerCharacter/BP_PlayerCharacter` (`GameplayStatics.GetPlayerCharacter` 0)))
  (set `self.PlayerRef` _asbp_player_character))

(fn `ApplyHitDamage`
  (params (Tool :type "/Game/Items/ToolActors/BP_ToolActor Object Reference"))
  (bind _objectclass (`/Game/Items/ToolActors/BP_ToolActor.ObjectClass` Tool))
  (if (== _objectclass (`self.DamageTool`))
    (`TimelineComponent.PlayFromStart` (`/Game/Items/ToolActors/BP_ToolActor.TL_ToolSwing` Tool))
    (bind _asbp_tool_object (castclass `/Game/Items/ItemObjects/Tool/BP_ToolObject` _objectclass))
    (bind _returnvalue (- (`self.Health`) (`.Damage` (defaults `Object` _asbp_tool_object))))
    (if (<= _returnvalue 0.0)
      (`self.OnDestroy`)
      (else
        (set `self.Health` _returnvalue)))))

(fn `OnDestroy`
  (locals (LastLocation :type "Vector Structure"))
  (bind (_id _displayname _description _itemtype _stackable _stacksize _staticmesh _staticmeshtransform) (defaults `Object` (`self.LootItem`)))
  (set `local.LastLocation` (`self.K2_GetActorLocation`))
  (`self.K2_DestroyActor`)
  (for _ (range (+ (`KismetMathLibrary.RandomIntegerInRange` (`self.MinAmountOfDroppedItems`) (`self.MaxAmountOfDroppedItems`)) 1))
    (bind _returnvalue (`|SpawnActorFromClass` "/Game/Items/BP_PickableItemActor.BP_PickableItemActor_C" (`KismetMathLibrary.MakeTransform` (+ (`local.LastLocation`) (0.0 0.0 40.0))) "Undefined" "MultiplyWithRoot" null null))
    (bind _staticmesh_2 (`/Game/Items/BP_PickableItemActor.StaticMesh` _returnvalue))
    (`StaticMeshComponent.SetStaticMesh` _staticmesh_2 _staticmesh)
    (`SceneComponent.K2_SetRelativeTransform` _staticmesh_2 _staticmeshtransform false false)
    (`PrimitiveComponent.SetSimulatePhysics` _staticmesh_2 true)
    (set `/Game/Items/BP_PickableItemActor.ItemObjectClass` (`self.LootItem`) _returnvalue)
    (`/Game/Attributes/BPC_Attributes.DecreaseEnergyAfterMining` (`/Game/PlayerCharacter/BP_PlayerCharacter.BPC_Attributes` (`self.PlayerRef`)) 5.0)))

(fn `SpawnItems`)

(fn `UserConstructionScript`)