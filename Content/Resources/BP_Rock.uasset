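; BP_Rock is a mineable rock resource that breaks into small rock drops.
; ApplyHitDamage accepts only a BP_Pickaxe, subtracts damage from its item data, and prints the remaining Health.
; When a hit would deplete Health, OnDestroy caches the location, destroys the actor, then spawns BP_SmallRock drops slightly above that spot, with the count randomized between configurable minimum and maximum values.
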(fn `ApplyHitDamage`
  (params (Tool :type "/Game/Items/ItemBP/BP_Item Object Reference"))
  (bind _asbp_pickaxe (cast `/Game/Items/ItemBP/BP_Pickaxe` Tool))
  (bind _returnvalue (- (`self.Health`) (`/Game/NewInventory/BP_ItemDefinition.Damage` (`.ItemClass_24_5E96F30A488B4287D92F9A9E36D555D4` (break `/Game/NewInventory/S_ItemData` (`/Game/Items/ItemBP/BP_Item.ItemData` _asbp_pickaxe))))))
  (if (<= _returnvalue 0)
    (`self.OnDestroy`)
    (else
      (bind _output_get (set `self.Health` _returnvalue))
      (`KismetSystemLibrary.PrintString` (`KismetStringLibrary.Conv_IntToString` _output_get)))))

(fn `OnDestroy`
  (locals (CachedLocation :type "Vector Structure" :default (0.0 0.0 0.0)))
  (set `local.CachedLocation` (`self.K2_GetActorLocation`))
  (`self.K2_DestroyActor`)
  (for _ (range (+ (`KismetMathLibrary.RandomIntegerInRange` (`self.MinAmountOfDroppedItems`) (`self.MaxAmountOfDroppedItems`)) 1))
    (`|SpawnActorFromClass` "/Game/Items/ItemBP/BP_SmallRock.BP_SmallRock_C" (`KismetMathLibrary.MakeTransform` (+ (`local.CachedLocation`) (0.0 0.0 40.0))) "Undefined" "MultiplyWithRoot" null (struct) null)))

(fn `UserConstructionScript`
  (`parent.UserConstructionScript`))