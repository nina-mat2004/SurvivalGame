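; BP_PalmTree_Base is a harvestable palm tree that players chop with an axe to get sticks.
; ApplyHitDamage accepts only axe tool actors and subtracts the damage from the axe's tool class defaults from Health, calling OnDestroy at zero or below.
; OnDestroy removes the tree, spawns a random number of stick actors above its location and decreases player energy once per spawned stick.
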(fn `ApplyHitDamage`
  (params (Tool :type "/Game/Items/ItemActors/BP_ItemActor Object Reference"))
  (bind _asbp_tool_actor_axe (cast `/Game/Items/ItemActors/Tool/BP_ToolActor_Axe` Tool))
  (bind _asbp_tool_object (castclass `/Game/Items/ItemObjects/Tool/BP_ToolObject` (`/Game/Items/ItemActors/BP_ItemActor.ClassRef` _asbp_tool_actor_axe)))
  (bind _returnvalue (- (`self.Health`) (`.Damage` (defaults `Object` _asbp_tool_object))))
  (if (<= _returnvalue 0.0)
    (`self.OnDestroy`)
    (else
      (set `self.Health` _returnvalue))))

(fn `OnDestroy`
  (locals (LocalLocation :type "Vector Structure" :default (0.0 0.0 0.0)))
  (set `local.LocalLocation` (`self.K2_GetActorLocation`))
  (`self.K2_DestroyActor`)
  (for _ (range (+ (`KismetMathLibrary.RandomIntegerInRange` (`self.MinAmountOfDroppedItems`) (`self.MaxAmountOfDroppedItems`)) 1))
    (`|SpawnActorFromClass` "/Game/Items/ItemActors/Material/BP_MaterialActor_Stick.BP_MaterialActor_Stick_C" (`KismetMathLibrary.MakeTransform` (+ (`local.LocalLocation`) (0.0 0.0 40.0))) "Undefined" "MultiplyWithRoot" null null)
    (`/Game/PlayerCharacter/BP_PlayerCharacter.DecreaseEnergyAfterMining` (`self.PlayerRef`))))

(fn `UserConstructionScript`
  (`parent.UserConstructionScript`))