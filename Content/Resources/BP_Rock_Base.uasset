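; BP_Rock_Base is a base mineable rock resource that takes damage from pickaxes and drops rock material when destroyed.
; ApplyHitDamage ignores tools other than BP_Tool_Pickaxe, subtracts the pickaxe's damage from Health and calls OnDestroy when it runs out.
; OnDestroy removes the actor and spawns a random number of BP_Material_Rock pickups just above its location, decreasing player energy once per spawned item.
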(fn `ApplyHitDamage`
  (params (Tool :type "/Game/Items/ItemBP/BP_Item Object Reference"))
  (bind _asbp_tool_pickaxe (cast `/Game/Items/ItemBP/Tool/BP_Tool_Pickaxe` Tool))
  (bind _returnvalue (- (`self.Health`) (`/Game/Items/ItemBP/Tool/BP_Tool.Damage` _asbp_tool_pickaxe)))
  (if (<= _returnvalue 0)
    (`self.OnDestroy`)
    (else
      (set `self.Health` _returnvalue))))

(fn `OnDestroy`
  (locals (LocalLocation :type "Vector Structure" :default (0.0 0.0 0.0)))
  (set `local.LocalLocation` (`self.K2_GetActorLocation`))
  (`self.K2_DestroyActor`)
  (for _ (range (+ (`KismetMathLibrary.RandomIntegerInRange` (`self.MinAmountOfDroppedItems`) (`self.MaxAmountOfDroppedItems`)) 1))
    (`|SpawnActorFromClass` "/Game/Items/ItemBP/Material/BP_Material_Rock.BP_Material_Rock_C" (`KismetMathLibrary.MakeTransform` (+ (`local.LocalLocation`) (0.0 0.0 40.0))) "Undefined" "MultiplyWithRoot" null (struct) null)
    (`/Game/Characters/PlayerCharacter/BP_PlayerCharacter.DecreaseEnergyAfterMining` (`self.PlayerRef`))))

(fn `UserConstructionScript`
  (`parent.UserConstructionScript`))