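; Player character Blueprint that manages health, hunger and stamina, and creates the attributes widget on BeginPlay.
; Self-calling events with Delays act as timers: sprint functions set walk speed and start stamina drain or regeneration.
; Hunger falls faster while sprinting; health regenerates until hunger hits zero, then drains until death, which only prints a message.
; Hunger and health regeneration loops end at zero hunger, with nothing here restarting them.
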(event `self.ReceiveBeginPlay`
  (bind _returnvalue (`|CreateWidget` "/Game/Characters/MainCharacter/PlayerAtributes.PlayerAtributes_C"))
  (`UserWidget.AddToViewport` _returnvalue 0)
  (`self.DecreaseHunger`)
  (`self.IncreaseHealth`))

(event `DecreaseStamina`
  ;[0.05203 0.6079 1] Stamina
  (bind _output_get (set `self.Stamina` (`KismetMathLibrary.Clamp` (- (`self.Stamina`) 3) 0 (`self.MaxStamina`))))
  (if (== _output_get 0)
    (`self.StopSprinting`)
    (elif (`self.IsSprinting`)
      (`KismetSystemLibrary.Delay` 0.2)
      (`self.DecreaseStamina`))))

(event `IncreaseStamina`
  ;[0.05203 0.6079 1] Stamina
  (bind _output_get (set `self.Stamina` (`KismetMathLibrary.Clamp` (+ (`self.Stamina`) 1) 0 (`self.MaxStamina`))))
  (if (== _output_get (`self.MaxStamina`))
    _
    (elif (not (`self.IsSprinting`))
      (`KismetSystemLibrary.Delay` 0.2)
      (`self.IncreaseStamina`))))

(event `DecreaseHunger`
  ;[0.2323 0.1481 0.01906] Hunger Decrement
  (if true
    (bind _output_get (set `self.Hunger` (`KismetMathLibrary.Clamp` (- (`self.Hunger`) 1) 0 (`self.MaxHunger`))))
    (if (== _output_get 0)
      (`self.DecreaseHealth`)
      (elif (`self.IsSprinting`)
        (`KismetSystemLibrary.Delay` 1.0)
        (`self.DecreaseHunger`)
        (else
          (`KismetSystemLibrary.Delay` 3.0)
          (`self.DecreaseHunger`))))))

(event `DecreaseHealth`
  ;[1 0.2622 0.356] Health
  (bind _output_get (set `self.Health` (`KismetMathLibrary.Clamp` (- (`self.Health`) 1) 0 (`self.MaxHealth`))))
  (if (== _output_get 0)
    (`KismetSystemLibrary.PrintString` "Player died.")
    (elif (== (`self.Hunger`) 0)
      (`KismetSystemLibrary.Delay` 0.5)
      (`self.DecreaseHealth`))))

(event `IncreaseHealth`
  ;[1 0.2622 0.356] Health
  (if (> (`self.Hunger`) 0)
    (set `self.Health` (`KismetMathLibrary.Clamp` (+ (`self.Health`) 1) 0 (`self.MaxHealth`)))
    (`KismetSystemLibrary.Delay` 0.5)
    (`self.IncreaseHealth`)))

(fn `StartSprinting`
  (set `CharacterMovementComponent.MaxWalkSpeed` 600.0 (`self.CharacterMovement`))
  (set `self.IsSprinting` true)
  (`self.DecreaseStamina`))

(fn `StopSprinting`
  (set `CharacterMovementComponent.MaxWalkSpeed` 300.0 (`self.CharacterMovement`))
  (set `self.IsSprinting` false)
  (`self.IncreaseStamina`))

(fn `UserConstructionScript`)