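; Player character for a survival game, with hunger, water, energy and health, plus sprinting, swimming and HUD widgets.
; Stats change through self-calling Delay loops that raise low-level warnings and drain health when depleted.
; Camera line traces drive item prompts, harvesting hits and refilling water bottles at collectors.
; BPCInventory stores picked-up items and supplies hotbar items, which spawn attached to the right-hand socket.
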(event `self.ReceiveTick`
  (params (DeltaSeconds :type "Float (single-precision)"))
  (bind (_returnvalue_x _returnvalue_y _returnvalue_z) (`KismetMathLibrary.BreakVector` (`self.K2_GetActorLocation`)))
  (bind _inventoryfullwidget (`self.InventoryFullWidget`))
  (bind _camera (`self.Camera`))
  (bind _returnvalue (`SceneComponent.K2_GetComponentLocation` _camera))
  ;[1 1 1] Interaction
  (`KismetSystemLibrary.PrintString` (`KismetStringLibrary.Conv_DoubleToString` _returnvalue_z))
  (bind _outhit (`KismetSystemLibrary.LineTraceSingle` _returnvalue (+ _returnvalue (* (`KismetMathLibrary.GetForwardVector` (`SceneComponent.K2_GetComponentRotation` _camera)) (`self.TraceLength`))) "TraceTypeQuery1"))
  (bind _asbp_item (cast `/Game/Items/ItemBP/BP_Item` (`.HitActor` (`GameplayStatics.BreakHitResult` _outhit)))
    (:`then`
      (set `self.CurrentInractable` _asbp_item)
      (`Widget.SetVisibility` (`self.InteractWidget`) "Visible"))
    (:`CastFailed`
      (`Widget.SetVisibility` (`self.InteractWidget`) "Hidden")
      (if (`Widget.IsVisible` _inventoryfullwidget)
        (`Widget.SetVisibility` _inventoryfullwidget "Hidden")))))

(event `self.ReceiveBeginPlay`
  (`self.CreateInGameScreen`)
  (`self.CreateInteractionWidget`)
  (`self.Create Inventory Widget`))

(event `DecreaseWater`
  ;[0.2682 0.6538 1] Water Decrement
  (if (<= (`self.Water`) 30)
    (set `self.ShowThirstWarning` true)
    (`/Game/Characters/PlayerCharacter/HUD/WBP_InGameScreen.UpdateWarningMessages` (`self.InGameScreenWidget`)))
  (bind _output_get (set `self.Water` (`KismetMathLibrary.Clamp` (- (`self.Water`) 1) 0 (`self.MaxAtributeValue`))))
  (if (<= _output_get 0)
    (`self.DecreaseHealth`)
    (else
      (`KismetSystemLibrary.Delay` 10.0)
      (`self.DecreaseWater`))))

(event `DecreaseHunger`
  ;[0.2323 0.1481 0.01906] Hunger Decrement
  (if (<= (`self.Hunger`) 30)
    (set `self.ShowHungerWarning` true)
    (`/Game/Characters/PlayerCharacter/HUD/WBP_InGameScreen.UpdateWarningMessages` (`self.InGameScreenWidget`)))
  (bind _output_get (set `self.Hunger` (`KismetMathLibrary.Clamp` (- (`self.Hunger`) 1) 0 (`self.MaxAtributeValue`))))
  (if (<= _output_get 0)
    (`self.DecreaseHealth`)
    (elif (`self.IsSprinting`)
      (`KismetSystemLibrary.Delay` 5.0)
      (`self.DecreaseHunger`)
      (else
        (`KismetSystemLibrary.Delay` 10.0)
        (`self.DecreaseHunger`)))))

(event `DecreaseHealth`
  ;[1 0.2622 0.356] Health
  (bind _output_get (set `self.Health` (`KismetMathLibrary.Clamp` (- (`self.Health`) 1) 0 (`self.MaxAtributeValue`))))
  (if (== _output_get 0)
    (`KismetSystemLibrary.PrintString` "Player died.")
    (elif (== (`self.Hunger`) 0)
      (`KismetSystemLibrary.Delay` 0.5)
      (`self.DecreaseHealth`))))

(event `IncreaseHealth`
  ;[1 0.2622 0.356] Health
  (if (> (`self.Hunger`) 0)
    (set `self.Health` (`KismetMathLibrary.Clamp` (+ (`self.Health`) 1) 0 (`self.MaxAtributeValue`)))
    (`KismetSystemLibrary.Delay` 0.5)
    (`self.IncreaseHealth`)))

(event `DecreaseEnergy`
  ;[0.5554 1 0.4726] Energy
  (if (<= (`self.Energy`) 30)
    (set `self.ShowTiredWarning` true)
    (`/Game/Characters/PlayerCharacter/HUD/WBP_InGameScreen.UpdateWarningMessages` (`self.InGameScreenWidget`)))
  (bind _output_get (set `self.Energy` (`KismetMathLibrary.Clamp` (- (`self.Energy`) 1) 0 (`self.MaxAtributeValue`))))
  (if (<= _output_get 0)
    (`self.DecreaseHealth`)
    (elif (`self.IsSprinting`)
      (`KismetSystemLibrary.Delay` 3.0)
      (`self.DecreaseEnergy`))))

(event `IncreaseEnergy`
  ;[0.5554 1 0.4726] Energy
  (if (not (`self.IsSprinting`))
    (if (>= (`self.Energy`) 30)
      (set `self.ShowTiredWarning` false)
      (`/Game/Characters/PlayerCharacter/HUD/WBP_InGameScreen.UpdateWarningMessages` (`self.InGameScreenWidget`)))
    (set `self.Energy` (`KismetMathLibrary.Clamp` (+ (`self.Energy`) 1) 0 (`self.MaxAtributeValue`)))
    (`KismetSystemLibrary.Delay` 5.0)
    (`self.IncreaseEnergy`)))

(event `StartSwimming`
  ;[0.8736 0.8153 1] Swimming
  (`self.LaunchCharacter` (* (`KismetMathLibrary.GetUpVector` (`self.K2_GetActorRotation`)) 2.0))
  (set `PhysicsVolume.bWaterVolume` true (`MovementComponent.GetPhysicsVolume` (`self.CharacterMovement`)))
  (set `self.IsSwimming` true))

(event `StopSwimming`
  ;[0.8736 0.8153 1] Swimming
  (set `PhysicsVolume.bWaterVolume` false (`MovementComponent.GetPhysicsVolume` (`self.CharacterMovement`)))
  (set `self.IsSwimming` false))

(fn `Add Water Points`
  (params (WaterPoints :type Integer))
  (bind _output_get (set `self.Water` (`KismetMathLibrary.Clamp` (+ WaterPoints (`self.Water`)) 0 (`self.MaxAtributeValue`))))
  (if (> _output_get 30)
    (set `self.ShowThirstWarning` false)
    (`/Game/Characters/PlayerCharacter/HUD/WBP_InGameScreen.UpdateWarningMessages` (`self.InGameScreenWidget`))))

(fn `AddHungerPoints`
  (params (HungerPoints :type Integer))
  (bind _output_get (set `self.Hunger` (`KismetMathLibrary.Clamp` (+ HungerPoints (`self.Hunger`)) 0 (`self.MaxAtributeValue`))))
  (if (> _output_get 30)
    (set `self.ShowHungerWarning` false)
    (`/Game/Characters/PlayerCharacter/HUD/WBP_InGameScreen.UpdateWarningMessages` (`self.InGameScreenWidget`))))

(fn `Create Inventory Widget`
  (bind _returnvalue (`|CreateWidget` "/Game/NewInventory/WBP_Inventory.WBP_Inventory_C"))
  (set `/Game/NewInventory/WBP_Inventory.InventoryComponentRef` (`self.BPC_Inventory`) _returnvalue)
  (bind _output_get (set `self.InventoryWidget` _returnvalue))
  (`UserWidget.AddToViewport` _output_get 0)
  (`Widget.SetVisibility` _output_get "Hidden"))

(fn `CreateInGameScreen`
  (bind _returnvalue (`|CreateWidget` "/Game/Characters/PlayerCharacter/HUD/WBP_InGameScreen.WBP_InGameScreen_C"))
  (bind _output_get (set `self.InGameScreenWidget` _returnvalue))
  (`UserWidget.AddToViewport` _output_get 0)
  (`self.DecreaseHunger`)
  (`self.IncreaseHealth`)
  (`self.DecreaseWater`)
  (`self.IncreaseEnergy`))

(fn `CreateInteractionWidget`
  ;[1 1 1] Interact
  (bind _returnvalue (`|CreateWidget` "/Game/Characters/PlayerCharacter/HUD/WBP_InteractText.WBP_InteractText_C"))
  (bind _output_get (set `self.InteractWidget` _returnvalue))
  (`UserWidget.AddToViewport` _output_get 0)
  (`Widget.SetVisibility` _output_get "Hidden")
  ;[1 1 1] Inventory Full
  (bind _returnvalue_2 (`|CreateWidget` "/Game/Characters/PlayerCharacter/HUD/WBP_InventoryFullText.WBP_InventoryFullText_C"))
  (bind _output_get_2 (set `self.InventoryFullWidget` _returnvalue_2))
  (`UserWidget.AddToViewport` _output_get_2 0)
  (`Widget.SetVisibility` _output_get_2 "Hidden"))

(fn `DestroyEquippedItem`
  (`self.K2_DestroyActor` (`self.CurrentEquipedItem`))
  (set `self.CurrentHotbarIndex` -1))

(fn `Spawn and Attach Equipped Item`
  (params (ItemDefinition :type "/Game/NewInventory/BP_ItemDefinition Object Reference"))
  (bind _currentequipeditem (`self.CurrentEquipedItem`))
  (`/Engine/EditorBlueprintResources/StandardMacros.IsValid` _currentequipeditem
    (:`Is Valid`
      (`self.K2_DestroyActor` _currentequipeditem))
    (:`Is Not Valid`
      _))
  (bind _returnvalue (`|SpawnActorFromClass` (`/Game/NewInventory/BP_ItemDefinition.WorldActor` ItemDefinition) (`SceneComponent.GetSocketTransform` (`self.Mesh`) "RightHandSocket" "RTS_World") "Undefined" "MultiplyWithRoot" null (struct) null))
  (bind _output_get (set `self.CurrentEquipedItem` _returnvalue))
  (`self.K2_AttachToComponent` _output_get (`self.Mesh`) "RightHandSocket" "SnapToTarget" "SnapToTarget" "SnapToTarget" true))

(fn `StartSprinting`
  (if (> (`self.Hunger`) 30)
    (set `CharacterMovementComponent.MaxWalkSpeed` 600.0 (`self.CharacterMovement`))
    (set `self.IsSprinting` true)
    (`self.DecreaseEnergy`)))

(fn `StopSprinting`
  (set `CharacterMovementComponent.MaxWalkSpeed` 300.0 (`self.CharacterMovement`))
  (set `self.IsSprinting` false)
  (`self.IncreaseEnergy`))

(fn `TryHitObject`
  (bind _camera (`self.Camera`))
  (bind _returnvalue (`SceneComponent.K2_GetComponentLocation` _camera))
  (`/Engine/EditorBlueprintResources/StandardMacros.IsValid` (`self.CurrentEquipedItem`)
    (:`Is Valid`
      (bind _outhit (`KismetSystemLibrary.LineTraceSingle` :`Start` _returnvalue :`End` (+ _returnvalue (* (`KismetMathLibrary.GetForwardVector` (`SceneComponent.K2_GetComponentRotation` _camera)) (`self.TraceLength`))) :`TraceChannel` "TraceTypeQuery1" :`DrawDebugType` "ForDuration"))
      (bind _asbp_harvestable_resource (cast `/Game/Resources/BP_HarvestableResource` (`.HitActor` (`GameplayStatics.BreakHitResult` _outhit))))
      (`/Game/Resources/BP_HarvestableResource.ApplyHitDamage` _asbp_harvestable_resource (`self.CurrentEquipedItem`)))))

(fn `TryInteractWithObject`
  (bind _camera (`self.Camera`))
  (bind _returnvalue (`SceneComponent.K2_GetComponentLocation` _camera))
  (bind _outhit (`KismetSystemLibrary.LineTraceSingle` :`Start` _returnvalue :`End` (+ _returnvalue (* (`KismetMathLibrary.GetForwardVector` (`SceneComponent.K2_GetComponentRotation` _camera)) (`self.TraceLength`))) :`TraceChannel` "TraceTypeQuery1" :`DrawDebugType` "ForDuration"))
  (bind _asbp_placeable_object (cast `/Game/PlaceableObjects/BP_PlaceableObject` (`.HitActor` (`GameplayStatics.BreakHitResult` _outhit))))
  (bind _asbp_water_collector (cast `/Game/PlaceableObjects/BP_WaterCollector` _asbp_placeable_object))
  (`self.UseWaterCollector` _asbp_water_collector))

(fn `TryPickUpObject`
  (bind _currentinractable (`self.CurrentInractable`))
  (if (and (`KismetSystemLibrary.IsValid` _currentinractable) (not (`self.IsInventoryOpen`)))
    (bind _itemaddedsuccessfully (`/Game/NewInventory/BPC_Inventory.AddItemToInventory` (`self.BPC_Inventory`) (`/Game/Items/ItemBP/BP_Item.ItemData` _currentinractable)))
    (if _itemaddedsuccessfully
      (`/Game/NewInventory/WBP_Inventory.UpdateInventoryWidget` (`self.InventoryWidget`))
      (`/Game/Items/ItemBP/BP_Item.DestroyItem` (`self.CurrentInractable`))
      (else
        (`Widget.SetVisibility` (`self.InventoryFullWidget`) "Visible")))))

(fn `UpdateEquippedItem`
  (params (Index :type Integer))
  (bind _itemclass (break `/Game/NewInventory/S_ItemData` (`|GetArrayItem` (`/Game/NewInventory/BPC_Inventory.HotbarItems` (`self.BPC_Inventory`)) Index)))
  (if (!= Index (`self.CurrentHotbarIndex`))
    (`/Engine/EditorBlueprintResources/StandardMacros.IsValid` _itemclass
      (:`Is Valid`
        (bind _output_get (set `self.EquippedItemDef` _itemclass))
        (`self.Spawn and Attach Equipped Item` _output_get)
        (set `self.CurrentHotbarIndex` Index))
      (:`Is Not Valid`
        (set `self.CurrentHotbarIndex` -1)))
    (else
      (`KismetSystemLibrary.PrintString` "Hello"))))

(fn `UseItem`)

(fn `UserConstructionScript`)

(fn `UseWaterCollector`
  (params (WaterCollector :type "/Game/PlaceableObjects/BP_WaterCollector Object Reference"))
  (bind _bpc_inventory (`self.BPC_Inventory`))
  (bind _watersupply (`/Game/PlaceableObjects/BP_WaterCollector.WaterSupply` WaterCollector))
  (bind _usedwater (`/Game/NewInventory/BPC_Inventory.UsedWater` _bpc_inventory))
  (for (_array_element _array_index) (`/Game/NewInventory/BPC_Inventory.Items` _bpc_inventory)
    (bind (_itemclass _quantity _isequiped _watersupply_2) (break `/Game/NewInventory/S_ItemData` _array_element))
    (`/Engine/EditorBlueprintResources/StandardMacros.IsValid` _itemclass
      (:`Is Valid`
        (if (== (`/Game/NewInventory/BP_ItemDefinition.WorldActor` _itemclass) "/Game/Items/ItemBP/BP_WaterBottle.BP_WaterBottle_C")
          (if (> _watersupply _usedwater)
            (`KismetArrayLibrary.Array_Set` (`/Game/NewInventory/BPC_Inventory.Items` (`self.BPC_Inventory`)) _array_index (make `/Game/NewInventory/S_ItemData` _itemclass _quantity _isequiped (`KismetMathLibrary.Clamp` (+ _watersupply_2 _usedwater) 0 100)))
            (set `/Game/PlaceableObjects/BP_WaterCollector.WaterSupply` (- _watersupply _usedwater) WaterCollector)
            (`/Game/NewInventory/BPC_Inventory.OnInventoryChanged` (`self.BPC_Inventory`))
            (return)
            (else
              (`KismetSystemLibrary.PrintString` "Not enough water in the collector")
              (return)))))))
  (`KismetSystemLibrary.PrintString` "You do not own water bottle"))